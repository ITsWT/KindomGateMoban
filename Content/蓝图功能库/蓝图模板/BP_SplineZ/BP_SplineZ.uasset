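; BP_SplineZ is a spline actor template that lays repeated spline meshes along an editable, optionally closed path.
; Its construction script can resample the spline into evenly spaced points as a one-shot toggle, also exposed as an event, then builds the meshes.
; Each rebuild destroys old segments and spawns new ones by length, gap and fill percentage, scaling tangents for clipped segments and applying material overrides.
; Tick optionally rebuilds the meshes every frame.
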(event Custom|CE_优化样条线
  (bind _优化后点位 (CallFunction|F优化线条))
  (CallFunction|F重设路径 _优化后点位 (Variables|默认|优化|GetType)))

(event EventBeginPlay)

(event Collision|EventActorBeginOverlap
  (params (OtherActor :type Actor%20Object%20Reference)))

(event EventTick
  (params (DeltaSeconds :type Float%20%28single-precision%29))
  (if (and (Variables|默认|样条网格体|Get实时更新样条网格体) (Variables|默认|样条网格体|Get启用样条网格体))
    (CallFunction|F更新样条网格体)))

(fn ConstructionScript
  (Spline|SetClosedLoop (Variables|Default|GetSplineZ) (Variables|默认|Get闭合样条线) true)
  (Utilities|FlowControl|Sequence
    (:then_0
      (if (Variables|默认|优化|Get优化)
        (Variables|默认|优化|Set优化 false)
        (bind _优化后点位 (CallFunction|F优化线条))
        (CallFunction|F重设路径 _优化后点位 "Linear")))
    (:then_1
      (if (Variables|默认|样条网格体|Get启用样条网格体)
        (CallFunction|F更新样条网格体)))))

(fn F优化线条
  (Utilities|Array|Add (LocalVariables|Get输出点位_lp) (Spline|GetLocationatSplinePoint (Variables|Default|GetSplineZ) 0 "World"))
  (bind _output_get (LocalVariables|Set个数_lp (Math|Float|Truncate (/ (Spline|GetSplineLength (Variables|Default|GetSplineZ)) (Variables|默认|优化|Get优化点间距)))))
  (LocalVariables|Set间距_lp (/ (Spline|GetSplineLength (Variables|Default|GetSplineZ)) (Math|Conversions|ToFloat(Integer) _output_get)))
  (for _index (range 1 _output_get)
    (bind _output_get_2 (LocalVariables|Set位置_lp (Spline|GetLocationatDistanceAlongSpline (Variables|Default|GetSplineZ) (* _index (LocalVariables|Get间距_lp)) "World")))
    (Utilities|Array|Add (LocalVariables|Get输出点位_lp) _output_get_2))
  (return (LocalVariables|Get输出点位_lp)))

(fn F重设路径
  (params (路径点 :type Array%20of%20Vectors) (Type :type ESplinePointType%20Enum :default "Linear"))
  (LocalVariables|Set路径点_lp 路径点)
  (Spline|ClearSplinePoints (Variables|Default|GetSplineZ) true)
  (for (_array_element _array_index) (LocalVariables|Get路径点_lp)
    (Class|SplineComponent|AddPoint (Variables|Default|GetSplineZ) (Utilities|Struct|MakeSplinePoint (Math|Conversions|ToFloat(Integer) _array_index) (Math|Transform|InverseTransformLocation (Transformation|GetActorTransform) _array_element) Type) true)))

(fn F更新样条网格体
  (bind (_起始位置 _起始切线 _结束位置 _结束切线) (CallFunction|F样条网格体的起始和结束))
  (bind _splinez (Variables|Default|GetSplineZ))
  (bind _样条网格体长度 (Variables|默认|样条网格体|Get样条网格体长度))
  (bind _样条网格体间距 (Variables|默认|样条网格体|Get样条网格体间距))
  (bind _returnvalue (Class|SplineComponent|FindScaleClosesttoWorldLocation _splinez _起始位置))
  (bind _returnvalue_2 (+ _样条网格体长度 _样条网格体间距))
  (CallFunction|F清理已生成的样条网格体)
  (Variables|默认|样条网格体|SetDistance (* (+ (Variables|默认|样条网格体|Get样条网格体长度) (Variables|默认|样条网格体|Get样条网格体间距)) -1.0))
  (for _index (range 0 (Math|Float|Floor (/ (* (Spline|GetSplineLength (Variables|Default|GetSplineZ)) (Variables|默认|样条网格体|Get生成百分比)) _returnvalue_2)))
    (Variables|默认|样条网格体|SetDistance (+ (Variables|默认|样条网格体|GetDistance) _returnvalue_2))
    (bind _returnvalue_3 (AddComponent|AddSplineMeshComponent false))
    (Transformation|SetAbsolute _returnvalue_3 true true true)
    (Components|StaticMesh|SetStaticMesh _returnvalue_3 (Variables|默认|样条网格体|Get网格体模型))
    (SplineMesh|SetStartandEnd _returnvalue_3 _起始位置 _起始切线 _结束位置 _结束切线 true :!class /Script/Engine.SplineMeshComponent)
    (SplineMesh|SetForwardAxis _returnvalue_3 (Variables|默认|样条网格体|Get模型向前轴) true)
    (SplineMesh|SetStartScale _returnvalue_3 (* (Variables|默认|样条网格体|Get网格体起始缩放) (.y _returnvalue)) true :!class /Script/Engine.SplineMeshComponent)
    (SplineMesh|SetEndScale _returnvalue_3 (* (Variables|默认|样条网格体|Get网格体结束缩放) (.y _returnvalue)) true :!class /Script/Engine.SplineMeshComponent)
    (Utilities|Array|Add (Variables|默认|样条网格体|Get生成的样条网格体) _returnvalue_3)
    (CallFunction|F样条网格体覆盖材质 _returnvalue_3)))

(fn F样条网格体的起始和结束
  (bind _distance (Variables|默认|样条网格体|GetDistance))
  (bind _样条网格体长度 (Variables|默认|样条网格体|Get样条网格体长度))
  (bind _splinez (Variables|Default|GetSplineZ))
  (bind _网格体切线缩放 (Variables|默认|样条网格体|Get网格体切线缩放))
  (bind _生成百分比 (Variables|默认|样条网格体|Get生成百分比))
  (bind _distance_2 (Variables|默认|样条网格体|GetDistance))
  (bind _样条网格体长度_2 (Variables|默认|样条网格体|Get样条网格体长度))
  (bind _splinez_2 (Variables|Default|GetSplineZ))
  (bind _returnvalue (Spline|GetSplineLength _splinez_2))
  (bind _returnvalue_2 (+ _distance_2 _样条网格体长度))
  (bind _returnvalue_3 (Math|Float|Clamp(Float) _distance 0.0 _returnvalue))
  (bind _returnvalue_4 (* _returnvalue _生成百分比))
  (bind _returnvalue_5 (Math|Float|Clamp(Float) _returnvalue_2 0.0 _returnvalue_4))
  (bind _returnvalue_6 (- _returnvalue_3 _returnvalue_5))
  (bind _returnvalue_7 (Math|Float|Absolute(Float) _returnvalue_6))
  (bind _returnvalue_8 (/ _returnvalue_7 _样条网格体长度_2))
  (bind _returnvalue_9 (* _网格体切线缩放 _returnvalue_8))
  (return (Spline|GetLocationatDistanceAlongSpline _splinez _returnvalue_3 "World") (* (Spline|GetTangentatDistanceAlongSpline _splinez _returnvalue_3 "World") _returnvalue_9) (Spline|GetLocationatDistanceAlongSpline _splinez _returnvalue_5 "World") (* (Spline|GetTangentatDistanceAlongSpline _splinez _returnvalue_5 "World") _returnvalue_9)))

(fn F样条网格体覆盖材质
  (params (网格体组件 :type Primitive%20Component%20Object%20Reference))
  (if (Utilities|Array|IsValidIndex (Variables|默认|样条网格体|Get更换网格体材质))
    (for (_array_element _array_index) (Variables|默认|样条网格体|Get更换网格体材质)
      (Rendering|Material|SetMaterial 网格体组件 _array_index _array_element))))

(fn F清理已生成的样条网格体
  (bind _生成的样条网格体 (Variables|默认|样条网格体|Get生成的样条网格体))
  (for _array_element _生成的样条网格体
    (Utilities|IsValid _array_element
      (:Is%20Valid
        (Components|DestroyComponent _array_element))))
  (Utilities|Array|Clear _生成的样条网格体)
  (return))