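; Base trigger actor with a box or sphere volume that broadcasts trigger and leave dispatchers, likely for child Blueprints to extend.
; Overlaps and hits pass an enabled check and seeded probability roll before broadcasting; end overlaps broadcast directly.
; Tick watches the enabled flag and briefly pulses the selected shape's collision when it turns on.
; Helpers toggle collision, animate a one-shot scale-up, and destroy the actor at a trigger-count limit.
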(event OnComponentEndOverlap(Box_触发范围)
  (params (OverlappedComponent :type Primitive%20Component%20Object%20Reference) (OtherActor :type Actor%20Object%20Reference) (OtherComp :type Primitive%20Component%20Object%20Reference) (OtherBodyIndex :type Integer))
  ;[0.9219 0 1 0.8] 离开时
  (CallFunction|CE-离开时 OverlappedComponent OtherActor OtherComp OtherBodyIndex))

(event OnComponentHit(Sphere_触发范围)
  (params (HitComponent :type Primitive%20Component%20Object%20Reference) (OtherActor :type Actor%20Object%20Reference) (OtherComp :type Primitive%20Component%20Object%20Reference) (NormalImpulse :type Vector :default "0, 0, 0") (Hit :type Hit%20Result%20Structure%20%28by%20ref%29))
  ;[0 1 0.25] 触发
  (Utilities|能否触发命中
    (:触发
      (CallFunction|CE-触发时 HitComponent OtherActor OtherComp 0 false Hit))))

(event OnComponentBeginOverlap(Box_触发范围)
  (params (OverlappedComponent :type Primitive%20Component%20Object%20Reference) (OtherActor :type Actor%20Object%20Reference) (OtherComp :type Primitive%20Component%20Object%20Reference) (OtherBodyIndex :type Integer) (bFromSweep :type Boolean) (SweepResult :type Hit%20Result%20Structure%20%28by%20ref%29))
  ;[0 1 0.25] 触发
  (Utilities|能否触发命中
    (:触发
      (CallFunction|CE-触发时 OverlappedComponent OtherActor OtherComp OtherBodyIndex bFromSweep SweepResult))))

(event OnComponentHit(Box_触发范围)
  (params (HitComponent :type Primitive%20Component%20Object%20Reference) (OtherActor :type Actor%20Object%20Reference) (OtherComp :type Primitive%20Component%20Object%20Reference) (NormalImpulse :type Vector :default "0, 0, 0") (Hit :type Hit%20Result%20Structure%20%28by%20ref%29))
  ;[0 1 0.25] 触发
  (Utilities|能否触发命中
    (:触发
      (CallFunction|CE-触发时 HitComponent OtherActor OtherComp 0 false Hit))))

(event OnComponentBeginOverlap(Sphere_触发范围)
  (params (OverlappedComponent :type Primitive%20Component%20Object%20Reference) (OtherActor :type Actor%20Object%20Reference) (OtherComp :type Primitive%20Component%20Object%20Reference) (OtherBodyIndex :type Integer) (bFromSweep :type Boolean) (SweepResult :type Hit%20Result%20Structure%20%28by%20ref%29))
  ;[0 1 0.25] 触发
  (Utilities|能否触发命中
    (:触发
      (CallFunction|CE-触发时 OverlappedComponent OtherActor OtherComp OtherBodyIndex bFromSweep SweepResult))))

(event OnComponentEndOverlap(Sphere_触发范围)
  (params (OverlappedComponent :type Primitive%20Component%20Object%20Reference) (OtherActor :type Actor%20Object%20Reference) (OtherComp :type Primitive%20Component%20Object%20Reference) (OtherBodyIndex :type Integer))
  ;[0.9219 0 1 0.8] 离开时
  (CallFunction|CE-离开时 OverlappedComponent OtherActor OtherComp OtherBodyIndex))

(event Custom|CE-切换激活
  (params (激活 :type Boolean))
  ;[0 0.3203 1] 状态
  (Collision|SetCollisionEnabled (Variables|Default|GetBox_触发范围) (select 激活 "QueryOnly" "NoCollision")))

(event Custom|CE-离开时
  (params (OverlappedComponent :type Primitive%20Component%20Object%20Reference) (OtherActor :type Actor%20Object%20Reference) (OtherComp :type Primitive%20Component%20Object%20Reference) (OtherBodyIndex :type Integer))
  ;[0.9219 0 1 0.8] 离开时
  (Default|CallED-离开时 OtherActor))

(event Custom|CE-缩放一次
  (params (动画时长 :type Float%20%28double-precision%29) (完成后销毁 :type Boolean))
  (Transformation|SetRelativeScale3D (Variables|Default|GetRoot) "0.010000,0.010000,0.010000")
  (CallFunction|CE-切换激活 true)
  (Components|Timeline|SetPlayRate (Variables|Default|GetTL_缩放一次) (/ 1.0 动画时长))
  (bind _f (Timeline|TL_缩放一次 PlayFromStart)
    (:Update
      (Transformation|SetRelativeScale3D (Variables|Default|GetRoot) (Math|Conversions|ToVector(Float) (Math|Float|Lerp 0.01 1.0 _f))))
    (:Finished
      (if 完成后销毁
        (Actor|DestroyActor)))))

(event Custom|CE_触发一次
  ;[0 0.3203 1] 状态
  (Collision|SetCollisionEnabled (CallFunction|F获取触发组件) "QueryOnly")
  (Utilities|FlowControl|Delay 0.0)
  (Collision|SetCollisionEnabled (CallFunction|F获取触发组件) "NoCollision"))

(event Custom|CE-延迟触发
  (params (Duration :type Float%20%28double-precision%29) (OverlappedComponent :type Primitive%20Component%20Object%20Reference) (OtherActor :type Actor%20Object%20Reference) (OtherComp :type Primitive%20Component%20Object%20Reference) (OtherBodyIndex :type Integer) (bFromSweep :type Boolean) (SweepResult :type Hit%20Result%20Structure%20%28by%20ref%29))
  ;[0 1 0.25] 触发
  (Utilities|DelayNotZero Duration
    (:false
      (CallFunction|CE-触发时 OverlappedComponent OtherActor OtherComp OtherBodyIndex bFromSweep SweepResult))))

(event Custom|CE-触发时
  (params (OverlappedComponent :type Primitive%20Component%20Object%20Reference) (OtherActor :type Actor%20Object%20Reference) (OtherComp :type Primitive%20Component%20Object%20Reference) (OtherBodyIndex :type Integer) (bFromSweep :type Boolean) (SweepResult :type Hit%20Result%20Structure%20%28by%20ref%29))
  ;[0 1 0.25] 触发
  (Default|CallED-触发时 OtherActor OtherComp SweepResult))

(event EventBeginPlay
  ;[0 1 0.2969] 初始化
  (Utilities|FlowControl|Sequence
    (:then_0
      (bind _aspawn (Utilities|Casting|CastToPawn (Actor|GetAttachParentActor)))
      (Variables|Actor|SetInstigator _aspawn))
    (:then_1
      (if (Variables|默认|触发器设置|Get初始激活)
        (Utilities|FlowControl|Delay 0.2)
        (CallFunction|CE-切换激活 false)
        (CallFunction|CE-切换激活 true)))
    (:then_2
      (EventDispatchers|BindEventtoED-触发成功时 (EventDispatchers|CreateEvent :!event FED-检查触发次数))
      (Variables|调试状态|Set启用_Last (Variables|默认|触发器设置|Get启用)))))

(event EventTick
  (params (DeltaSeconds :type Float%20%28single-precision%29))
  (CallFunction|F监测启用状态))

(fn ConstructionScript
  ;[0.05469 0 1] 切换组件
  (Rendering|SetVisibility (Variables|Default|GetBox_触发范围) (not (Variables|默认|触发器设置|Get球体/盒体)) false)
  (Rendering|SetVisibility (Variables|Default|GetSphere_触发范围) (Variables|默认|触发器设置|Get球体/盒体) false)
  ;[0.5234 0 1 0.8] 游戏中隐藏
  (Development|SetHiddeninGame (Variables|Default|GetBox_触发范围) (Variables|默认|触发器设置|Get游戏中隐藏) false))

(fn F获取触发组件
  (return (select (Variables|默认|触发器设置|Get球体/盒体) (Variables|Default|GetSphere_触发范围) (Variables|Default|GetBox_触发范围))))

(fn FED-检查触发次数
  (params (触发器 :type BP%20SH触发器%20Base%20Object%20Reference) (最后触发角色 :type BP%20SH角色%20Base%20Object%20Reference) (最后触发Actor :type Actor%20Object%20Reference))
  (if (> (Variables|默认|触发器设置|Get最大触发次数) 0)
    (bind _result (Math|Integer|IncrementInt (Variables|调试状态|Get已触发次数))
      (:%20%20
        (if (>= _result (Variables|默认|触发器设置|Get最大触发次数))
          (Actor|DestroyActor))))))

(fn F监测启用状态
  ;[0.4062 1 0] 检测启用状态
  (if (!= (Variables|默认|触发器设置|Get启用) (Variables|调试状态|Get启用_Last))
    (bind _output_get (Variables|调试状态|Set启用_Last (Variables|默认|触发器设置|Get启用)))
    (if _output_get
      (CallFunction|CE触发一次))))