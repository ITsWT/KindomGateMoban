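; Child Blueprint of a standalone tire prop (独立轮胎) that overrides how the tire visually breaks.
; F轮胎破碎动画 plays the explosion break animation once on the tire skeletal mesh, or hides that mesh in game if no animation is set.
; The override replaces the parent's break logic without calling it; construction defers to the parent and the event graph holds only disabled stubs.
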(event EventBeginPlay
  (|CallParentFunction) ; This node is disabled and will not be called.\nDrag off pins to build functionality.
)

(event Collision|EventActorBeginOverlap
  (params (OtherActor :type Actor%20Object%20Reference)))

(event EventTick
  (params (DeltaSeconds :type Float%20%28single-precision%29))
  (|CallParentFunction DeltaSeconds) ; This node is disabled and will not be called.\nDrag off pins to build functionality.
)

(fn ConstructionScript
  (|CallParentFunction))

(fn F轮胎破碎动画
  (bind _爆炸_使用破碎动画 (Variables|Default|Get爆炸_使用破碎动画))
  (bind _skm_轮胎 (Variables|Default|GetSKM_轮胎))
  (Utilities|IsValid _爆炸_使用破碎动画
    (:Is%20Valid
      (Components|Animation|PlayAnimation _skm_轮胎 _爆炸_使用破碎动画 false))
    (:Is%20Not%20Valid
      (Development|SetHiddeninGame _skm_轮胎 true false))))