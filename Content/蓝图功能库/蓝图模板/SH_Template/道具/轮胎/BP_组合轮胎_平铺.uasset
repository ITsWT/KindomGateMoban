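; Combined tire obstacle: a flat row of BP_独立轮胎 child actors sharing one health pool, shown on a widget number.
; The construction script spawns the centered row and routes each tire's damage into that pool.
; As health crosses per-tire thresholds, a tire explodes and a timeline re-centers the rest; other hits play reactions.
; A Sequencer-keyed health value (K帧生命值) above -1 overrides damage, polled on Tick.
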(event Custom|CEED-受到伤害
  (params (DamagedActor :type Actor%20Object%20Reference) (Damage :type Float%20%28single-precision%29) (DamageType :type Damage%20Type%20Object%20Reference) (InstigatedBy :type Controller%20Object%20Reference) (DamageCauser :type Actor%20Object%20Reference))
  ;[0.1484 1 0] 事件 受到伤害时
  ;;[0.9922 1 0] 储存一下是哪个轮胎受到了伤害
  (bind _asbp_独立轮胎 (Utilities|Casting|CastToBP_独立轮胎 DamagedActor))
  (Variables|调试|Set被击中的轮胎 _asbp_独立轮胎)
  ;;[0 1 0.2734] 判断是否要用定序器去K，不用定序器K的话才能修改生命值，否则以K帧的数值为准
  (if (<= (Variables|调试|GetK帧生命值) -1.0)
    (Variables|参数|Set生命值_当前 (- (Variables|参数|Get生命值_当前) Damage))
    (Default|CallED-生命值变化时 (Variables|参数|Get生命值_当前))
    (CallFunction|CE-轮胎受击反馈)
    ;[0.15 0 0.02348 0.5] 使用BP_音效控制蓝图播放音效
    (Default|CE子弹击中 (Variables|Default|GetBP_音效控制) "NewEnumerator3")))

(event Custom|CE-UMG缩放
  ;[1 0.8672 0 0.8] UMG缩放动画
  (Utilities|FlowControl|Sequence
    (:then_0
      (Utilities|FlowControl|DoOnce false :!label _label
        (:Completed
          (Default|CallED-UMG缩放时)
          (Components|Timeline|SetPlayRate (Variables|Default|Gettl_scale) (/ 1.0 (Variables|参数|GetUMG_受击缩放耗时)))
          (bind _f (Timeline|TL_Scale PlayFromStart)
            (:Update
              (Transformation|SetRelativeScale3D (Variables|Default|GetRoot_UMG_Scale) (Math|Conversions|ToVector(Float) (Math|Float|Lerp 1.0 (Variables|参数|GetUMG_受击缩放程度) _f))))))))
    (:then_1
      (Utilities|FlowControl|Delay (Variables|参数|GetUMG_受击缩放间隔时间))
      (goto _label Reset))))

(event Custom|CE-轮胎受击反馈
  (bind _生成的轮胎 (Variables|Debug|Get生成的轮胎))
  ;[0.5469 1 0 0.8] 轮胎受击反馈
  (Utilities|IsValid (Variables|调试|Get被击中的轮胎) ; 检查一下真的有轮胎被击中吗？
    (:Is%20Valid
      (if (Utilities|Array|ContainsItem (Variables|Debug|Get生成的轮胎) (Variables|调试|Get被击中的轮胎))
        _
        (else
          (Variables|调试|Set被击中的轮胎 (.OutItem (Utilities|Array|Random (Variables|Debug|Get生成的轮胎))) :!label _label))))
    (:Is%20Not%20Valid
      (goto _label)))
  ;;[1 0 0.9844] 判断应该剩下多少轮胎
  (Variables|调试|Set应当剩余的轮胎数量 (+ (.ReturnValue (Math|Float|Division(WholeandRemainder) (Variables|参数|Get生命值_当前) (Variables|Debug|Get每个轮胎生命值))) 1))
  (CallFunction|CE-UMG缩放)
  (CallFunction|F更新UMG数字) ; 更新数字
  ;;[0 0.5078 1] 还有剩的轮胎吗？
  (if (Utilities|Array|IsNotEmpty (Variables|Debug|Get生成的轮胎))
    ;;[1 0.4453 0] 是否应该炸轮胎
    (if (or (< (Variables|调试|Get应当剩余的轮胎数量) (Utilities|Array|Length (Variables|Debug|Get生成的轮胎))) (<= (Variables|参数|Get生命值_当前) 0.0))
      ;;[1 0.04688 0] 轮胎爆炸
      (Utilities|Array|RemoveItem (Variables|Debug|Get生成的轮胎) (Variables|调试|Get被击中的轮胎))
      (Default|CE爆炸 (Variables|调试|Get被击中的轮胎))
      (Default|CallED-轮胎爆炸时 (Variables|调试|Get被击中的轮胎))
      ;;[0 1 0.4844] 还有剩余的轮胎吗
      (if (Utilities|Array|IsNotEmpty (Variables|Debug|Get生成的轮胎))
        ;;[1 0 0.6328] 更新轮胎位置
        (bind _f (Timeline|时间轴 PlayFromStart)
          (:Update
            (for (_array_element _array_index) _生成的轮胎
              (Utilities|IsValid _array_element
                (:Is%20Valid
                  (if (Variables|/Game/蓝图功能库/蓝图模板/SH_Template/道具/轮胎/BP_独立轮胎.BP_独立轮胎_C|Get已爆炸 _array_element)
                    (Utilities|Array|Add (Variables|调试|Get已爆炸的轮胎) _array_element :!label _label_2)
                    (else
                      (bind _相对位置_y (私有函数|F计算轮胎位置 _array_index (Utilities|Array|LastIndex _生成的轮胎)))
                      (Transformation|SetActorLocation _array_element (Math|Vector|Lerp(Vector) (Transformation|GetActorLocation _array_element) (CallFunction|向量合并XYZ轴 (+ (Transformation|GetActorLocation) (* (Transformation|GetActorRightVector) _相对位置_y)) (Transformation|GetActorLocation _array_element)) _f) false false)
                      (if (Variables|参数|Get轮胎_对齐到地面？)
                        (Default|CE对齐到地面 _array_element)))))
                (:Is%20Not%20Valid
                  (goto _label_2))))
            (for _array_element_2 (Variables|调试|Get已爆炸的轮胎)
              (Utilities|Array|RemoveItem (Variables|Debug|Get生成的轮胎) _array_element_2))))
        (else
          (Default|CallED-所有轮胎都爆炸时)))
      (else
        ;;[0.07812 1 0] 不需要爆炸，所以调用轮胎受击效果
        (bind _被击中的轮胎 (Variables|调试|Get被击中的轮胎)
          (:then
            (Default|CE受击 _被击中的轮胎))
          (:else))))))

(event Custom|CE-持续追击目标
  ;[0.3557 0.6094 0.1142 0.5] 添加障碍物移动
  (CallFunction|F追击目标))

(event EventBeginPlay
  (bind _k帧生命值 (Variables|调试|GetK帧生命值))
  ;[0.5469 1 0] 初始化
  (|CallParentFunction)
  (Utilities|FlowControl|Sequence
    (:then_0
      ;;[1 0.4688 0] 储存UMG变量
      (bind _asumg_文本 (Utilities|Casting|CastToUMG_文本 (UserInterface|GetWidget (Variables|Default|GetUMG_轮胎数字))))
      (Variables|调试|SetAs%20UMG%20文本 _asumg_文本)
      (Rendering|SetCastShadow (Variables|Default|GetUMG_轮胎数字) false))
    (:then_1
      ;;[0.125 0 1 0.8] 启用UMG
      (Utilities|FlowControl|Delay 0.033333) ; 延迟一下，兼容定序器
      (bind _output_get (Variables|调试|Set生命值_最大 (select (> _k帧生命值 -1.0) _k帧生命值 (Variables|参数|Get生命值_当前))))
      (Variables|Debug|Set每个轮胎生命值 (/ _output_get (Variables|参数|Get轮胎_数量))) ; 平均每个轮胎应该有多少血量
      (CallFunction|F更新UMG数字) ; 刷新数字
      (Actor|Tick|SetActorTickEnabled true))
    (:then_2
      ;;[0.125 0 1] 启用轮胎碰撞
      (for _array_element (Variables|Debug|Get生成的轮胎)
        (Utilities|IsValid _array_element
          (:Is%20Valid
            (Collision|SetCollisionEnabled (Variables|/Game/蓝图功能库/蓝图模板/SH_Template/道具/轮胎/BP_独立轮胎.BP_独立轮胎_C|GetBox _array_element) "QueryOnly")
            (Variables|/Script/Engine.PrimitiveComponent|SetbGenerateOverlapEvents (Variables|/Game/蓝图功能库/蓝图模板/SH_Template/道具/轮胎/BP_独立轮胎.BP_独立轮胎_C|GetBox _array_element) true)))))
    (:then_3
      (Variables|/Game/蓝图功能库/通用组件/BPAC_Actor持续位移.BPAC_Actor持续位移_C|Set位移速度 (Variables|Default|GetBPAC_Actor持续位移) (Variables|Default|Get普通位移速度)))
    (:then_4
      (bind _returnvalue (Actor|GetActorOfClass "/Game/蓝图功能库/蓝图模板/SH_Template/角色/玩家控制器/BP_音效控制.BP_音效控制_C"))
      (Variables|Default|SetBP_音效控制 _returnvalue))))

(event EventTick
  (params (DeltaSeconds :type Float%20%28single-precision%29))
  ;[0.1484 1 0] 事件 受到伤害时
  ;;[1 0.7031 0] Tick覆盖生命值
  (|CallParentFunction DeltaSeconds)
  (CallFunction|F文本面向相机)
  ;;;[0 0.5312 1] 大于-1说明这个值被定序器K了，所以要用定序器K的值去覆盖当前生命值参与计算
  (if (> (Variables|调试|GetK帧生命值) -1.0)
    (bind _output_get (Variables|参数|Set生命值_当前 (Variables|调试|GetK帧生命值)))
    ;;;[0.8516 1 0] 判断是否和上一帧一致，也就是K帧的值是否正在变化
    (if (!= _output_get (Variables|调试|GetK帧生命值_LastFrame))
      (Variables|调试|SetK帧生命值_LastFrame (Variables|调试|GetK帧生命值))
      (CallFunction|F更新UMG数字) ; 更新数字
      (Default|CallED-生命值变化时 (Variables|参数|Get生命值_当前))
      (CallFunction|CE-轮胎受击反馈)
      ;[0.15 0 0.02348 0.5] 使用BP_音效控制蓝图播放音效
      (Default|CE子弹击中 (Variables|Default|GetBP_音效控制) "NewEnumerator3"))))

(fn ConstructionScript
  (bind _轮胎_数量 (Variables|参数|Get轮胎_数量))
  (bind _returnvalue (- _轮胎_数量 1))
  ;[1 0 0.8906] 避免重复构造
  (私有函数|F销毁全部轮胎)
  ;[1 0 0.2812] 循环生成 BP_独立轮胎
  (for _index (range 0 _returnvalue)
    (bind _相对位置_y (私有函数|F计算轮胎位置 _index _returnvalue)) ; 计算每个轮胎的偏移位置
    ;;[0.8047 0 1] 生成child actor component并且提出child actor转换为BP_独立轮胎
    (bind _returnvalue_2 (AddComponent|AddChildActorComponent false (Math|Transform|MakeTransform (Math|Vector|MakeVector 0.0 _相对位置_y 0.0) "0, 0, 0" "1.000000,1.000000,1.000000")))
    (Utilities|IsValid _returnvalue_2
      (:Is%20Valid
        (bind _asbp_独立轮胎 (Utilities|Casting|CastToBP_独立轮胎 (Variables|/Script/Engine.ChildActorComponent|GetChildActor _returnvalue_2)))
        (LocalVariables|SetAs_BP_独立轮胎 _asbp_独立轮胎)
        ;;[0 1 0.3672] 绑定一个事件到轮胎受到伤害的时候（这个轮胎受到伤害时就会直接调用我们绑定的事件）多个轮胎受伤时会多次调用这个事件（看不懂的话去学一下事件分发器）
        (EventDispatchers|BindEventtoOnTakeAnyDamage (LocalVariables|GetAs_BP_独立轮胎) (EventDispatchers|CreateEvent :!event Custom|CEED-受到伤害))
        ;;[0.4531 0 1] 调用独立轮胎蓝图里的事件 让它放到地面上
        (if (Variables|参数|Get轮胎_对齐到地面？)
          (Default|CE对齐到地面 (LocalVariables|GetAs_BP_独立轮胎)))
        ;;[1 0.375 0] 生成的轮胎存到数组里，便于统一计算位置（轮胎爆炸后一起位移到新位置）
        (Utilities|Array|Add (Variables|Debug|Get生成的轮胎) (LocalVariables|GetAs_BP_独立轮胎))
        ;[1 0 0.4687] 传递数值
        (Variables|/Game/蓝图功能库/蓝图模板/SH_Template/道具/轮胎/BP_独立轮胎.BP_独立轮胎_C|Set轮胎之间的间距 (LocalVariables|GetAs_BP_独立轮胎) (Variables|参数|Get轮胎_间距))
        (Variables|/Game/蓝图功能库/蓝图模板/SH_Template/道具/轮胎/BP_独立轮胎.BP_独立轮胎_C|Set伤害百分比 (LocalVariables|GetAs_BP_独立轮胎) (Variables|参数|Get受击_伤害百分比))
        (Variables|/Game/蓝图功能库/蓝图模板/SH_Template/道具/轮胎/BP_独立轮胎.BP_独立轮胎_C|Set爆炸时震屏 (LocalVariables|GetAs_BP_独立轮胎) (Variables|状态|移动|追击|Get爆炸时震屏)))
      (:Is%20Not%20Valid
        (Development|PrintString "生成轮胎失败了")))))

(fn F销毁全部轮胎
  (bind _生成的轮胎 (Variables|Debug|Get生成的轮胎))
  (for _array_element _生成的轮胎
    (Utilities|IsValid _array_element
      (:Is%20Valid
        (Actor|DestroyActor _array_element))))
  (Utilities|Array|Clear _生成的轮胎))

(fn F更新UMG数字
  (Default|F修改文本内容Float (Variables|调试|GetAs%20UMG%20文本) (Variables|参数|Get生命值_当前) "ToPositiveInfinity" false false false 0 true)
  (if (<= (Variables|参数|Get生命值_当前) 0.0)
    (Development|SetHiddeninGame (Variables|Default|GetUMG_轮胎数字) true false)))

(fn F计算轮胎位置
  (params (Index :type Integer) (LastIndex :type Integer))
  (bind _轮胎_间距 (Variables|参数|Get轮胎_间距))
  (return (- (* _轮胎_间距 Index) (* LastIndex _轮胎_间距 0.5))))

(fn F获取最近的轮胎
  (params (Origin :type Vector))
  (return (.AsBP%20独立轮胎 (Utilities|Casting|CastToBP_独立轮胎 (.ReturnValue (Actor|FindNearestActor Origin (Variables|Debug|Get生成的轮胎)))))))

(fn F文本面向相机
  (if (Variables|参数|GetUMG面向相机)
    (CallFunction|将F组件朝向相机(正对) (Variables|Default|GetUMG_轮胎数字))))

(fn F追击目标
  (params (TargetActor :type Actor%20Object%20Reference))
  (bind _returnvalue (Transformation|GetActorLocation))
  (bind _追击衰减距离 (Variables|状态|移动|追击|Get追击衰减距离))
  (bind _追击衰减强度 (Variables|状态|移动|追击|Get追击衰减强度))
  (bind (_x _y) (Math|Vector2D|BreakVector2D _追击衰减距离))
  (bind (_x_2 _y_2) (Math|Vector2D|BreakVector2D _追击衰减强度))
  (Utilities|IsValid TargetActor
    (:Is%20Valid
      (Variables|状态|移动|追击|Set追击_目标最后位置 (Transformation|GetActorLocation TargetActor)))
    (:Is%20Not%20Valid
      _))
  (Transformation|AddActorWorldOffset (* (Math|Float|MapRangeClamped (Math|Vector|Distance2D(Vector) (Variables|状态|移动|追击|Get追击_目标最后位置) _returnvalue) _x _y _x_2 _y_2) (Math|Vector|Lerp(Vector) (Variables|状态|移动|追击|Get追击_之前移动方向) (CallFunction|单元方向2D _returnvalue (Variables|状态|移动|追击|Get追击_目标最后位置)) (Variables|状态|移动|追击|Get追击_当前Alpha)) (Variables|状态|移动|追击|Get移动速度))))