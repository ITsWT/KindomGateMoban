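; BP_独立轮胎 is a rolling tire obstacle that damages and knocks back overlapping actors of faction 1.
; Hits play a rate-limited scale punch and material flash, while damage interface calls forward scaled damage to ApplyDamage.
; Exploding disables collision, shakes the camera and breaks the tire by randomized physics impulses, animation or hiding before it expires.
; The explosion's scale timeline can line-trace sideways, pushing neighboring tires apart through their per-source offset maps.
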(event OnComponentBeginOverlap(Box)
  (params (OverlappedComponent :type Primitive%20Component%20Object%20Reference) (OtherActor :type Actor%20Object%20Reference) (OtherComp :type Primitive%20Component%20Object%20Reference) (OtherBodyIndex :type Integer) (bFromSweep :type Boolean) (SweepResult :type Hit%20Result%20Structure%20%28by%20ref%29))
  ;[1 0 0.7031 0.8] 轮胎撞击伤害
  (if (> (Variables|参数|Get撞击_伤害值) 0.0)
    (bind _阵营 (Class|BPISH交互接口|BPI-获取所属阵营(Message) OtherActor))
    (if (== _阵营 1)
      (Class|BPISH交互接口|BPI-应用伤害-SH(Message) OtherActor (Variables|参数|Get撞击_伤害值) (Variables|Actor|GetInstigator) self "轮胎撞击" (+ (* (Transformation|GetActorForwardVector) (CallFunction|范围内随机浮点2D (Variables|参数|Get撞击_水平冲击力))) (Math|Vector|MakeVector 0.0 0.0 (CallFunction|范围内随机浮点2D (Variables|参数|Get撞击_垂直冲击力)))) SweepResult)
      (Utilities|冷却 0.2
        (:Completed
          (CallFunction|震屏 "/Game/蓝图功能库/相机振动/CS_获得奖励.CS_获得奖励_C")
          ;[0.00265 0.15 0 0.5] 此处单独播放死亡音效，以至明显被撞死
          (Audio|PlaySound2D "/Game/DoormdayTrain/Audios/男人死亡.男人死亡" 1.0 1.0 0.0 0 0))))))

(event Custom|CE_受击
  (bind _box (Variables|Default|GetBox))
  (bind _returnvalue (Transformation|GetWorldLocation _box))
  ;[0 0.8828 1] 受击缩放和闪烁
  (Utilities|FlowControl|Sequence
    (:then_0
      (Utilities|FlowControl|DoOnce false :!label _label
        (:Completed
          ;;[0 1 0.6484] 缩放动画
          (bind _新建轨道_0 (Timeline|TL_缩放 PlayFromStart)
            (:Update
              (bind _output_get (Variables|调试|Set缩放alpha _新建轨道_0))
              (Transformation|SetRelativeScale3D (Variables|Default|Get轮胎Root) (Math|Vector|Lerp(Vector) "1.000000,1.000000,1.000000" (Math|Conversions|ToVector(Float) (Variables|参数|Get受击_缩放大小)) _output_get))
              ;[0.007812 1 0] 爆炸了才能推开
              (if (Variables|调试|Get已爆炸)
                ;[0 0.7187 1] 推开左右的轮胎
                (if (Variables|参数|Get爆炸_推开左右轮胎？)
                  (for _index (range -1 1)
                    (if (!= _index 0)
                      (bind (_outhits _returnvalue_2) (Class|KismetSystemLibrary|LineTraceMultiforObjects _returnvalue (+ _returnvalue (* (Transformation|GetActorRightVector) 2e+03 _index)) (Utilities|Array|MakeArray "ObjectTypeQuery2") false 0 "None" true))
                      (if _returnvalue_2
                        (for _array_element _outhits
                          (bind _asbp_独立轮胎 (Utilities|Casting|CastToBP_独立轮胎 (.HitActor (Collision|BreakHitResult _array_element))))
                          (Utilities|Map|Add (Variables|BP_独立轮胎_C|Get受到的额外偏移 _asbp_独立轮胎) _asbp_独立轮胎 (* (Variables|Debug|Get轮胎之间的间距) (Variables|调试|Get缩放alpha) (- (Variables|参数|Get受击_缩放大小) 1.0) _index 1.0))
                          (CallFunction|CE更新额外偏移 _asbp_独立轮胎))))))))))))
    (:then_1
      (Utilities|FlowControl|Delay (Variables|参数|Get受击_频率间隔时间))
      (goto _label Reset))
    (:then_2
      ;;[0.1016 1 0] 闪烁动画
      (Components|Timeline|SetPlayRate (Variables|Default|GetTL_闪烁) (Variables|参数|Get受击_闪烁动画速率))
      (bind _网格体组件 (CallFunction|F获取所有网格体组件 self true true false))
      (bind _变色time (Timeline|TL_闪烁 PlayFromStart)
        (:Update
          (Rendering|Material|SetScalarParameterValueonMaterials _网格体组件 "SH_闪烁Alpha" _变色time))))))

(event Custom|CE_对齐到地面
  ;[0.1484 1 0] 对齐到地面
  (bind (_是否命中 _命中结果) (CallFunction|向下的对象的线条检测 (Transformation|GetActorLocation) 1e+02 2e+03 (Utilities|Array|MakeArray "ObjectTypeQuery1") false "None" 1.0))
  (if _是否命中
    (Transformation|SetActorLocation (CallFunction|向量合并XYZ轴 (Transformation|GetActorLocation) (.Location (Collision|BreakHitResult _命中结果))) false false)))

(event Custom|CE_爆炸
  (bind _tl_缩放 (Variables|Default|GetTL_缩放))
  ;[0.4531 1 0] 爆炸
  (Components|Activation|Activate (Variables|Default|GetP_爆炸) true)
  (Collision|SetCollisionEnabled (Variables|Default|GetBox) "NoCollision")
  (Actor|SetLifeSpan 0.4)
  (Variables|调试|Set已爆炸 true)
  (Components|Timeline|PlayfromStart _tl_缩放)
  (Components|Timeline|SetPlayRate _tl_缩放 1.25)
  (CallFunction|F轮胎破碎动画)
  (CallFunction|CE播放TL闪烁)
  (CallFunction|震屏 (Variables|Default|Get爆炸时震屏))
  (Default|CE木桶碎裂 (Variables|Default|GetBP_音效控制)))

(event Custom|CE_更新额外偏移
  (bind _受到的额外偏移 (Variables|Debug|Get受到的额外偏移))
  ;[1 0.9141 0] 被其他轮胎推开
  (bind _keys (Utilities|Map|Keys _受到的额外偏移))
  (for _array_element _keys
    (Transformation|SetRelativeLocation (Variables|Default|Get轮胎Root) (Math|Vector|MakeVector 0.0 (+ (.Value (Utilities|Map|Find _受到的额外偏移 _array_element)) (Variables|调试|Get相对位置%20Y_初始)) 0.0) false false)))

(event Custom|CE_播放TL闪烁
  ;[0 0.8828 1] 受击缩放和闪烁
  ;;[0.1016 1 0] 闪烁动画
  (Components|Timeline|SetPlayRate (Variables|Default|GetTL_闪烁) (Variables|参数|Get受击_闪烁动画速率))
  (bind _网格体组件 (CallFunction|F获取所有网格体组件 self true true false))
  (bind _变色time (Timeline|TL_闪烁 PlayFromStart)
    (:Update
      (Rendering|Material|SetScalarParameterValueonMaterials _网格体组件 "SH_闪烁Alpha" _变色time))))

(event Custom|CE-模拟物理
  (bind _爆炸_物理水平角速度 (Variables|参数|Get爆炸_物理水平角速度))
  ;[1 0 0.3047 0.8] 物理爆炸
  (if (Variables|参数|Get爆炸_模拟物理)
    (CallFunction|一键模拟物理 (Variables|Default|GetSKM_轮胎) "PhysicsOnly" "ECC_PhysicsBody" true)
    (for _array_element (Transformation|GetAllSocketNames (Variables|Default|GetSKM_轮胎))
      (Physics|SetPhysicsLinearVelocity (Variables|Default|GetSKM_轮胎) (+ (* (Math|Vector|RotateVector (Math|Vector|NegateVector (Transformation|GetActorForwardVector)) (Math|Rotator|MakeRotator 0.0 0.0 (CallFunction|范围内随机浮点2D (Variables|参数|Get爆炸_物理水平旋转角度)))) (CallFunction|范围内随机浮点2D (Variables|参数|Get爆炸_物理水平冲击力))) (Math|Vector|MakeVector 0.0 0.0 (CallFunction|范围内随机浮点2D (Variables|参数|Get爆炸_物理垂直冲击力)))) false _array_element)
      (Class|PrimitiveComponent|SetPhysicsAngularVelocityinDegrees (Variables|Default|GetSKM_轮胎) (* (Math|Random|RandomUnitVectorinConeinDegrees (Math|Vector|NegateVector (Transformation|GetActorForwardVector)) (Variables|参数|Get爆炸_物理水平角角度)) (Math|Vector|MakeVector (CallFunction|范围内随机浮点2D _爆炸_物理水平角速度) (CallFunction|范围内随机浮点2D _爆炸_物理水平角速度) (CallFunction|范围内随机浮点2D _爆炸_物理水平角速度))) false "None"))
    (Collision|SetCollisionResponsetoAllChannels (Variables|Default|GetSKM_轮胎) "ECR_Ignore")
    (Actor|SetLifeSpan 0.7)))

(event EventBeginPlay
  ;[1 0.9141 0] 被其他轮胎推开
  (Variables|调试|Set相对位置%20Y_初始 (.y (Variables|/Script/Engine.SceneComponent|GetRelativeLocation (Variables|Default|Get轮胎Root))))
  (Transformation|AddLocalRotation (Variables|Default|Get轮胎Root) (Math|Rotator|MakeRotator 0.0 (CallFunction|绝对值范围内随机浮点 (Variables|Default|Get滚动速度)) 0.0) false false)
  (bind _returnvalue (Actor|GetActorOfClass "/Game/蓝图功能库/蓝图模板/SH_Template/角色/玩家控制器/BP_音效控制.BP_音效控制_C"))
  (Variables|Default|SetBP_音效控制 _returnvalue))

(event EventTick
  (params (DeltaSeconds :type Float%20%28single-precision%29))
  (bind _滚动速度 (Variables|Default|Get滚动速度))
  ;[0 0.1328 1 0.8] 滚动
  (if (!= _滚动速度 0.0)
    (Transformation|AddLocalRotation (Variables|Default|Get轮胎Root) (Math|Rotator|MakeRotator 0.0 (* DeltaSeconds _滚动速度) 0.0) false false)))

(fn ConstructionScript)

(fn F轮胎破碎动画
  (bind _skm_轮胎 (Variables|Default|GetSKM_轮胎))
  (if (Variables|参数|Get爆炸_模拟物理)
    (CallFunction|CE-模拟物理)
    (else
      (Utilities|IsValid (Variables|参数|Get爆炸_使用破碎动画)
        (:Is%20Valid
          (Components|Animation|PlayAnimation _skm_轮胎 "/Game/蓝图功能库/蓝图模板/SH_Template/道具/轮胎/滚木/test_Anim1.test_Anim1" false))
        (:Is%20Not%20Valid
          (Development|SetHiddeninGame _skm_轮胎 true false))))))

(fn BPI-发起交互
  (params (发起者 :type Actor%20Object%20Reference) (交互类型 :type String))
  (return false ""))

(fn BPI-应用伤害-SH
  (params (伤害值 :type Float%20%28double-precision%29) (Instigator :type Pawn%20Object%20Reference) (DamageCauser :type Actor%20Object%20Reference) (伤害类型 :type String) (物理冲击 :type Vector :default "0, 0, 0") (命中结果 :type Hit%20Result%20Structure))
  (bind _returnvalue (Game|Damage|ApplyDamage self (* 伤害值 (Variables|调试|Get伤害百分比)) 0 DamageCauser))
  (return true _returnvalue))

(fn BPI-获取当前速度
  (return false "0, 0, 0"))

(fn BPI-获取所属阵营
  (return -1))

(fn BPI-获取是否死亡
  (return (Variables|调试|Get已爆炸) 0))