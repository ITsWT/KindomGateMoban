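; BP_组合轮胎_堆叠 is a damageable tire-stack obstacle with a floating health number that damages and knocks back overlapping other-faction actors.
; The construction script spawns seeded, jittered BP_独立轮胎 child actors sharing one health pool.
; Hits always target the bottom tire, exploding it when health crosses a per-tire share, then a timeline lowers the stack and label.
; A keyframe health value lets Sequencer influence starting health and damage results.
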(event OnComponentBeginOverlap(Box_Damage)
  (params (OverlappedComponent :type Primitive%20Component%20Object%20Reference) (OtherActor :type Actor%20Object%20Reference) (OtherComp :type Primitive%20Component%20Object%20Reference) (OtherBodyIndex :type Integer) (bFromSweep :type Boolean) (SweepResult :type Hit%20Result%20Structure%20%28by%20ref%29))
  ;[0 1 0.2969] 轮胎杀人
  (bind _阵营 (Class|BPISH交互接口|BPI-获取所属阵营(Message) OtherActor))
  (if (!= _阵营 (Variables|Default|Get阵营))
    (Class|BPISH交互接口|BPI-应用伤害-SH(Message) OtherActor 1e+02 (Variables|Actor|GetInstigator) (Components|GetOwner) "轮胎碰撞" (CallFunction|流送中范围内复合冲量 "0, 0, 0" (Transformation|GetActorForwardVector) (Variables|Default|Get水平力度范围) (Variables|Default|Get垂直力度范围) 0.0 (Variables|Default|GetSeed_组合轮胎)))))

(event Custom|CEED-受到伤害
  (params (DamagedActor :type Actor%20Object%20Reference) (Damage :type Float%20%28single-precision%29) (DamageType :type Damage%20Type%20Object%20Reference) (InstigatedBy :type Controller%20Object%20Reference) (DamageCauser :type Actor%20Object%20Reference))
  (bind _生成的轮胎 (Variables|Debug|Get生成的轮胎))
  ;[0.1484 1 0] 事件 受到伤害时
  ;;[0.9922 1 0] 储存一下是哪个轮胎受到了伤害
  (Utilities|Casting|CastToBP_独立轮胎 DamagedActor)
  (Variables|调试|Set被击中的轮胎 (Utilities|Array|Get(acopy) (Variables|Debug|Get生成的轮胎)))
  ;;[0 0.2266 1] 生命值变化
  (bind _output_get (Variables|Default|Set生命值_当前 (select (> (Variables|调试|GetK帧生命值) -1.0) (CallFunction|浮点关键帧插值 (- (Variables|Default|Get生命值_当前) Damage) (Variables|调试|GetK帧生命值) (Variables|调试|Get生命值_最大)) (- (Variables|Default|Get生命值_当前) Damage))))
  (Default|CallED-生命值变化时 _output_get)
  (Utilities|IsValid (Variables|调试|Get被击中的轮胎) ; 检查一下真的有轮胎被击中吗？
    (:Is%20Valid
      (Default|CallED-成功受击时)
      ;;[1 0 0.9844] 判断应该剩下多少轮胎
      (Variables|调试|Set应当剩余的轮胎数量 (+ (select (!= (.Remainder (Math|Float|Division(WholeandRemainder) (Variables|Default|Get生命值_当前) (Variables|Debug|Get每个轮胎生命值))) 0.0) 1 0) (.ReturnValue (Math|Float|Division(WholeandRemainder) (Variables|Default|Get生命值_当前) (Variables|Debug|Get每个轮胎生命值)))))
      (CallFunction|F更新UMG数字) ; 更新数字
      ;;[0 0.5078 1] 还有剩的轮胎吗？
      (if (Utilities|Array|IsNotEmpty (Variables|Debug|Get生成的轮胎))
        ;;[1 0.4453 0] 是否应该炸轮胎
        (if (or (< (Variables|调试|Get应当剩余的轮胎数量) (Utilities|Array|Length (Variables|Debug|Get生成的轮胎))) (<= (Variables|Default|Get生命值_当前) 0.0))
          ;;[1 0.04688 0] 轮胎爆炸
          (Utilities|Array|RemoveItem (Variables|Debug|Get生成的轮胎) (Variables|调试|Get被击中的轮胎))
          (Default|CE爆炸 (Variables|调试|Get被击中的轮胎))
          (Default|CallED-轮胎爆炸时 (Variables|调试|Get被击中的轮胎))
          ;;[0 1 0.4844] 还有剩余的轮胎吗
          (if (Utilities|Array|IsNotEmpty (Variables|Debug|Get生成的轮胎))
            (Collision|SetCollisionEnabled (Variables|/Game/蓝图功能库/蓝图模板/SH_Template/道具/轮胎/BP_独立轮胎.BP_独立轮胎_C|GetBox (Utilities|Array|Get(acopy) (Variables|Debug|Get生成的轮胎))) "QueryOnly" :!pinned true) ; PP启用新轮胎碰撞
            ;;[1 0 0.6328] 更新轮胎位置
            (bind _f (Timeline|TL_轮胎位置 PlayFromStart)
              (:Update
                (Default|CallED-更新轮胎位置时 _f)
                (for (_array_element _array_index) _生成的轮胎
                  (Utilities|IsValid _array_element
                    (:Is%20Valid
                      (if (Variables|/Game/蓝图功能库/蓝图模板/SH_Template/道具/轮胎/BP_独立轮胎.BP_独立轮胎_C|Get已爆炸 _array_element)
                        (Utilities|Array|Add (Variables|调试|Get已爆炸的轮胎) _array_element :!label _label)
                        (else
                          (bind _相对位置 (私有函数|F计算轮胎位置 _array_index (Utilities|Array|LastIndex _生成的轮胎)))
                          (Transformation|SetActorLocation _array_element (Math|Vector|Lerp(Vector) (Transformation|GetActorLocation _array_element) (CallFunction|向量合并XYZ轴 (Transformation|GetActorLocation _array_element) (+ (Transformation|GetActorLocation) (Math|Vector|MakeVector 0.0 0.0 (* _相对位置 (.z (Transformation|GetActorScale3D)))))) _f) false false))))
                    (:Is%20Not%20Valid
                      (goto _label))))
                ;;;[1 0 0.8203] 移动完成后移除无效的轮胎
                (for _array_element_2 (Variables|调试|Get已爆炸的轮胎)
                  (Utilities|Array|RemoveItem (Variables|Debug|Get生成的轮胎) _array_element_2))
                (if (Variables|Default|Getb更新UMG位置)
                  (CallFunction|F更新UMG位置 _f true))))
            (else
              ;[0 0.0625 1] 没有剩余的轮胎了，说明全炸了，如果要加入道具之类的话可以在这个时候处理掉
              (Collision|SetCollisionEnabled (Variables|Default|GetBox_Damage) "NoCollision")
              (Default|CallED-所有轮胎都爆炸时)))
          (else
            ;;[0.07812 1 0] 不需要爆炸，所以调用轮胎受击效果
            (Default|CE受击 (Variables|调试|Get被击中的轮胎))
            (CallFunction|CE数字缩放)))))))

(event Custom|CE_数字缩放
  ;[0.1484 1 0] 事件 受到伤害时
  ;;[0 0.6719 1] 数字缩放
  (Utilities|FlowControl|Sequence
    (:then_0
      (Utilities|FlowControl|DoOnce false :!label _label
        (:Completed
          (Components|Timeline|SetPlayRate (Variables|Default|GetTL_数字缩放) (Variables|默认|文本设置|Get受击时数字缩放速率))
          (bind _v (Timeline|TL_数字缩放 PlayFromStart)
            (:Update
              (Default|CallED-数字缩放时 _v)
              (Transformation|SetRelativeScale3D (Variables|Default|GetRoot_UMG变换) (Math|Conversions|ToVector(Float) (Math|Float|Lerp 1.0 (Variables|默认|文本设置|Get受击时数字缩放程度) (.X (Math|Vector|BreakVector _v))))))))))
    (:then_1
      (Utilities|FlowControl|Delay (Variables|/Game/蓝图功能库/蓝图模板/SH_Template/道具/轮胎/BP_独立轮胎.BP_独立轮胎_C|Get受击_频率间隔时间 (Variables|调试|Get被击中的轮胎)))
      (goto _label Reset))))

(event Custom|CE_全部爆炸
  ;[1 0.5156 0] 强制全部爆炸
  (for _array_element (Variables|Debug|Get生成的轮胎)
    (Default|CE爆炸 _array_element)
    (Development|SetHiddeninGame (Variables|Default|GetUMG_文本) false false))
  (Transformation|DetachFromActor "KeepWorld" "KeepWorld" "KeepWorld")
  (Collision|SetCollisionEnabled (Variables|Default|GetBox_Damage) "NoCollision")
  (Default|CallED-所有轮胎都爆炸时))

(event EventBeginPlay
  (bind _k帧生命值 (Variables|调试|GetK帧生命值))
  ;[0.5469 1 0] 初始化
  ;;[1 1 1] 结束预览
  (Components|DestroyComponent (Variables|Default|GetTEXT_预览))
  (Rendering|SetVisibility (Variables|Default|GetUMG_文本) true false)
  ;;[1 0.4688 0] 储存UMG变量
  (bind _asumg_文本 (Utilities|Casting|CastToUMG_文本 (UserInterface|GetWidget (Variables|Default|GetUMG_文本))))
  (bind _output_get (Variables|调试|SetAs%20UMG%20文本 _asumg_文本))
  (Default|F修改文本描边 _output_get (Variables|默认|文本设置|Get文本_描边宽度) (Variables|默认|文本设置|Get文本_描边颜色) true)
  (CallFunction|F更新UMG位置 1.0 false)
  (Utilities|FlowControl|Delay 0.033333) ; 延迟一下，兼容定序器
  (bind _output_get_2 (Variables|Default|Set生命值_当前 (select (> _k帧生命值 -1.0) _k帧生命值 (Variables|Default|Get生命值_当前))))
  (bind _output_get_3 (Variables|调试|Set生命值_最大 _output_get_2))
  (Variables|Debug|Set每个轮胎生命值 (/ _output_get_3 (Variables|Default|Get轮胎生成数量))) ; 平均每个轮胎应该有多少血量
  (CallFunction|F更新UMG数字) ; 刷新数字
  (Rendering|SetCastShadow (Variables|Default|GetUMG_文本) (Variables|默认|文本设置|Get文本_启用阴影)))

(event Game|Damage|EventAnyDamage
  (params (Damage :type Float%20%28single-precision%29) (DamageType :type Damage%20Type%20Object%20Reference) (InstigatedBy :type Controller%20Object%20Reference) (DamageCauser :type Actor%20Object%20Reference))
  ;[0.1484 1 0] 事件 受到伤害时
  ;;[0.9219 1 0] 备用方案，删了都行
  (CallFunction|CEED-受到伤害 self Damage DamageType InstigatedBy DamageCauser))

(event EventTick
  (params (DeltaSeconds :type Float%20%28single-precision%29))
  ;[0.1484 1 0] 事件 受到伤害时
  ;;[1 0.7031 0] Tick覆盖生命值
  (|CallParentFunction DeltaSeconds))

(fn ConstructionScript
  (bind _轮胎生成数量 (Variables|Default|Get轮胎生成数量))
  (bind _seed_组合轮胎 (Variables|Default|GetSeed_组合轮胎))
  (bind _轮胎xy偏移范围 (Variables|Default|Get轮胎XY偏移范围))
  (bind _returnvalue (- _轮胎生成数量 1))
  ;[1 0 0.8906] 避免重复构造
  (私有函数|F销毁全部轮胎)
  ;[1 0 0.2812] 循环生成 BP_独立轮胎
  (for _index (range 0 _returnvalue)
    (bind _相对位置 (私有函数|F计算轮胎位置 _index _returnvalue)) ; 计算每个轮胎的偏移位置
    ;;[0.8047 0 1] 生成child actor component并且提出child actor转换为BP_独立轮胎
    (bind _returnvalue_2 (AddComponent|AddChildActorComponent false (Math|Transform|MakeTransform (Math|Vector|MakeVector (CallFunction|流送中绝对值范围内随机浮点 (.x _轮胎xy偏移范围) _seed_组合轮胎) (CallFunction|流送中绝对值范围内随机浮点 (.y _轮胎xy偏移范围) _seed_组合轮胎) _相对位置) (Math|Rotator|MakeRotator 0.0 0.0 0.0) "1.000000,1.000000,1.000000")))
    (Utilities|IsValid _returnvalue_2
      (:Is%20Valid
        (bind _asbp_独立轮胎 (Utilities|Casting|CastToBP_独立轮胎 (Variables|/Script/Engine.ChildActorComponent|GetChildActor _returnvalue_2)))
        (Utilities|Array|Add (Variables|Debug|Get生成的轮胎) _asbp_独立轮胎)
        ;;[1 0.375 0] 生成的轮胎存到数组里，便于统一计算位置（轮胎爆炸后一起位移到新位置）
        (Variables|/Game/蓝图功能库/蓝图模板/SH_Template/道具/轮胎/BP_独立轮胎.BP_独立轮胎_C|Set轮胎之间的间距 _asbp_独立轮胎 (Variables|Default|Get轮胎间距))
        ;;[1 0 0.4687] 传递数值
        (Variables|/Game/蓝图功能库/蓝图模板/SH_Template/道具/轮胎/BP_独立轮胎.BP_独立轮胎_C|Set伤害百分比 _asbp_独立轮胎 (Variables|Default|Get受到伤害百分比)))
      (:Is%20Not%20Valid
        (Development|PrintString "生成轮胎失败了"))))
  (CallFunction|F更新UMG位置 1.0 false)
  ;;[1 1 1] 预览
  (Rendering|Components|TextRender|SetText (Variables|Default|GetTEXT_预览) (Utilities|Text|ToText(Float) (Variables|Default|Get生命值_当前) "ToPositiveInfinity" false true 1 324 0 0)))

(fn F销毁全部轮胎
  (bind _生成的轮胎 (Variables|Debug|Get生成的轮胎))
  (for _array_element _生成的轮胎
    (Actor|DestroyActor _array_element))
  (Utilities|Array|Clear _生成的轮胎))

(fn F更新UMG数字
  (bind _as_umg_文本 (Variables|调试|GetAs%20UMG%20文本))
  (Utilities|IsValid _as_umg_文本
    (:Is%20Valid
      (Default|F修改文本内容Float _as_umg_文本 (Variables|Default|Get生命值_当前) "ToPositiveInfinity" false false false 0 true)
      (if (<= (Variables|Default|Get生命值_当前) 0.0)
        (Development|SetHiddeninGame (Variables|Default|GetUMG_文本) true false)))))

(fn F计算轮胎位置
  (params (Index :type Integer) (LastIndex :type Integer))
  (return (* (Variables|Default|Get轮胎间距) Index)))

(fn F获取最近的轮胎
  (params (Origin :type Vector))
  (return (.AsBP%20独立轮胎 (Utilities|Casting|CastToBP_独立轮胎 (.ReturnValue (Actor|FindNearestActor Origin (Variables|Debug|Get生成的轮胎)))))))

(fn F更新UMG位置
  (params (Alpha :type Float%20%28double-precision%29) (只降不升 :type Boolean))
  (bind _root_umg变换 (Variables|Default|GetRoot_UMG变换))
  (bind _returnvalue (Transformation|GetWorldLocation _root_umg变换))
  (bind (_center _boxextent) (Collision|GetActorArrayBounds (Variables|Debug|Get生成的轮胎)))
  (bind _output_get (LocalVariables|Setlp平均位置 _center))
  (LocalVariables|Setlp_新位置 (Math|Vector|Lerp(Vector) _returnvalue (CallFunction|向量合并XYZ轴 _returnvalue (+ _output_get (Math|Vector|MakeVector 0.0 0.0 (* (Variables|Default|GetUMG高度百分比) (.Z (Math|Vector|BreakVector _boxextent)))))) (Math|Float|Min(Float) (* Alpha 2.0) 1.0)))
  (if 只降不升
    ;[1 0 0.6328] 新位置Z轴需要低于旧位置Z轴
    (if (< (.z (LocalVariables|Getlp_新位置)) (.z (Transformation|GetWorldLocation (Variables|Default|GetRoot_UMG变换))))
      (Transformation|SetWorldLocation (Variables|Default|GetRoot_UMG变换) (LocalVariables|Getlp_新位置) false false :!label _label))
    (else
      (goto _label))))

(fn BPI-发起交互
  (params (发起者 :type Actor%20Object%20Reference) (交互类型 :type String))
  (return false ""))

(fn BPI-应用伤害-SH
  (params (伤害值 :type Float%20%28double-precision%29) (Instigator :type Pawn%20Object%20Reference) (DamageCauser :type Actor%20Object%20Reference) (伤害类型 :type String) (物理冲击 :type Vector :default "0, 0, 0") (命中结果 :type Hit%20Result%20Structure))
  (bind _受到伤害百分比 (Variables|Default|Get受到伤害百分比))
  (bind _生成的轮胎 (Variables|Debug|Get生成的轮胎))
  (bind _returnvalue (* 伤害值 _受到伤害百分比))
  (if (Utilities|Array|IsValidIndex _生成的轮胎)
    (CallFunction|CEED-受到伤害 (Utilities|Array|Get(acopy) _生成的轮胎) _returnvalue)
    (return true _returnvalue)
    (else
      (return false 0.0))))

(fn BPI-获取当前速度
  (return false "0, 0, 0"))

(fn BPI-获取所属阵营
  (return 0))

(fn BPI-获取是否死亡
  (return false 0))