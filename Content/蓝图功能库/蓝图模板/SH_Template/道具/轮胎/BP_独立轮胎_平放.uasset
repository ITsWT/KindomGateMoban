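; BP_独立轮胎_平放 is a flat-lying standalone tire prop that shatters when its CE爆炸 event fires.
; The event shakes the screen, plays VFX and a flash, disables box collision, and swaps the tire for an animated debris mesh with random yaw.
; After a short delay, a timeline sinks the actor and destroys it.
; An alternative per-socket physics burst is unwired, and Tick's extra gravity force is set to zero.
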(event EventBeginPlay
  (|CallParentFunction) ; 此节点被禁用，将不会被调用。\n从引脚连出引线来编译功能。
)

(event Collision|EventActorBeginOverlap
  (params (OtherActor :type Actor%20Object%20Reference)))

(event EventTick
  (params (DeltaSeconds :type Float%20%28single-precision%29))
  (|CallParentFunction DeltaSeconds)
  (if (Class|SceneComponent|IsAnySimulatingPhysics (Variables|Default|GetSKM_轮胎))
    (CallFunction|F物理重力 0.0)))

(event EventCE爆炸
  (bind _skm_细碎轮胎 (Variables|Default|GetSKM_细碎轮胎))
  (CallFunction|震屏 "/Game/蓝图功能库/相机振动/CS_轮胎破碎.CS_轮胎破碎_C")
  (Components|Activation|Activate (Variables|Default|GetVFX_轮胎爆炸) true)
  (Collision|SetCollisionEnabled (Variables|Default|GetBox) "NoCollision")
  (Variables|Default|Set已爆炸 true)
  (CallFunction|CE播放TL闪烁)
  (Audio|Components|Audio|Play _skm_细碎轮胎 false)
  (Transformation|AddRelativeRotation _skm_细碎轮胎 (Math|Rotator|MakeRotator 0.0 0.0 (Math|Random|RandomFloatinRange -45.0 45.0)) false false)
  (Rendering|SetVisibility _skm_细碎轮胎 true false)
  (Development|SetHiddeninGame (Variables|Default|GetSKM_轮胎) true false)
  (Utilities|FlowControl|Delay 0.4)
  (Collision|SetCollisionResponsetoAllChannels (Variables|Default|GetSKM_轮胎) "ECR_Ignore")
  (Timeline|TL_退场 PlayFromStart
    (:Update
      (Transformation|AddActorLocalOffset (Math|Vector|MakeVector 0.0 0.0 (* (Utilities|Time|GetWorldDeltaSeconds) -4e+02)) false false))
    (:Finished
      (Actor|DestroyActor))))

(fn ConstructionScript
  (|CallParentFunction))

(fn F物理炸开
  (bind _skm_轮胎 (Variables|Default|GetSKM_轮胎))
  (CallFunction|一键模拟物理 _skm_轮胎 "PhysicsOnly" "ECC_PhysicsBody" true)
  (bind _output_get (LocalVariables|Setsockets (Transformation|GetAllSocketNames _skm_轮胎)))
  (for _array_element _output_get
    (Physics|SetPhysicsLinearVelocity (Variables|Default|GetSKM_轮胎) (CallFunction|流送中范围内复合冲量 "0, 0, 0" (Math|Random|RandomUnitVectorinConeinDegrees (Math|Vector|NegateVector (Transformation|GetActorForwardVector (Actor|GetAttachParentActor))) 1.8e+02) "(X=500.000000,Y=1000.000000)" "(X=500.000000,Y=1000.000000)" 0.0 (CallFunction|随机流送)) false _array_element)))

(fn F物理重力
  (params (额外重力 :type Float%20%28double-precision%29))
  (bind _output_get (LocalVariables|Setsockets (Transformation|GetAllSocketNames (Variables|Default|GetSKM_轮胎))))
  (for _array_element _output_get
    (Physics|AddForce (Variables|Default|GetSKM_轮胎) (Math|Vector|MakeVector 0.0 0.0 额外重力) _array_element false)))