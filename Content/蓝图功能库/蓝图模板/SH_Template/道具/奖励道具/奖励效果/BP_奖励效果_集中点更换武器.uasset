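; Reward effect that swaps the weapon of every unit in a rally point (集中点) and calls its group level change.
; CE-获得奖励 passes through a delay check, validates the rally point, then calls its group-wide functions for the swap and level change.
; Feedback follows: optional curve scaling and color flash, per-unit particles, upgrade sound, camera shake.
; The first two configured particles also spawn as larger overall effects attached to the rally point's core sphere.
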(event EventBeginPlay)

(event Collision|EventActorBeginOverlap
  (params (OtherActor :type Actor%20Object%20Reference)))

(event EventTick
  (params (DeltaSeconds :type Float%20%28single-precision%29)))

(event EventCE-获得奖励
  (bind _触发特效_粒子 (Variables|默认|外观效果|Get触发特效_粒子))
  (bind _触发特效_粒子_2 (Variables|默认|外观效果|Get触发特效_粒子))
  (bind _output (Utilities|Array|Get(acopy) _触发特效_粒子_2 1))
  (bind _output_2 (Utilities|Array|Get(acopy) _触发特效_粒子))
  (Utilities|DelayNotZero (Variables|Default|Get奖励执行延迟时间)
    (:false
      (bind _集中点 (Variables|Default|Get集中点)
        (:then
          (Default|F全体更换武器 _集中点 (Variables|Default|Get新武器))
          (Default|F全体修改等级 _集中点)
          (Utilities|FlowControl|Sequence
            (:then_0
              (bind _触发缩放_曲线 (Variables|默认|外观效果|Get触发缩放_曲线)
                (:then
                  (Default|F全体缩放 (Variables|Default|Get集中点) (Variables|默认|外观效果|Get缩放耗时) _触发缩放_曲线))
                (:else)))
            (:then_1
              (if (> (.a (Variables|默认|外观效果|Get触发闪烁_颜色)) 0.0)
                (Default|F全体闪烁 (Variables|Default|Get集中点) (Variables|默认|外观效果|Get触发闪烁_颜色) -1.0)))
            (:then_2
              ;[0.15 0.15 0.15 0.5] 触发每个单独特效
              (for _array_element (Variables|默认|外观效果|Get触发特效_粒子)
                (bind _valid (CallFunction|F特效有效 _array_element))
                (if _valid
                  (Default|F全体特效 _集中点 _array_element (Variables|默认|外观效果|Get触发特效_偏移) true (Variables|默认|外观效果|Get触发特效_缩放)))))
            (:then_3
              (Audio|PlaySound2D "/Game/Runnning/Audios/获得+升级音效.获得+升级音效" 1.0 1.0 0.0 0 0))
            (:then_4
              ;[0.00696 0.15 0 0.5] 震屏
              (CallFunction|震屏 "/Game/蓝图功能库/相机振动/CS_获得奖励.CS_获得奖励_C"))
            (:then_5
              ;[0.15 0.15 0.15 0.5] 在目标点触发总体特效
              (CallFunction|F生成粒子特效 (Math|Transform|MakeTransform (+ (Transformation|GetWorldLocation (Variables|/Script/Engine.Actor|GetRootComponent (Variables|Default|Get集中点))) "") "0, 0, 0" "1.500000,1.500000,1.500000") (Utilities|Struct|MakeF粒子特效 (.niagara _output_2) (.cascade _output_2)) (Variables|/Game/蓝图功能库/蓝图模板/SH_Template/角色/集中点/BP_集中点.BP_集中点_C|GetSphere_核心 (Variables|Default|Get集中点)) "None" "KeepWorldPosition" true true false)
              (CallFunction|F生成粒子特效 (Math|Transform|MakeTransform (+ (Transformation|GetWorldLocation (Variables|/Script/Engine.Actor|GetRootComponent (Variables|Default|Get集中点))) "0.000000,0.000000,-120.000000") "0, 0, 0" "1.500000,1.500000,1.500000") (Utilities|Struct|MakeF粒子特效 (.niagara _output) (.cascade _output)) (Variables|/Game/蓝图功能库/蓝图模板/SH_Template/角色/集中点/BP_集中点.BP_集中点_C|GetSphere_核心 (Variables|Default|Get集中点)) "None" "KeepWorldPosition" true true false))))
        (:else)))))

(fn ConstructionScript
  (|CallParentFunction))