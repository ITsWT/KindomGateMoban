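; Reward item variant that binds to the tiled combined-tire obstacle (BP_组合轮胎_平铺) it is attached to.
; F绑定附加障碍物 casts the attach parent to that obstacle, stores it, and subscribes to its UMG-scale, all-tires-exploded and health-change dispatchers.
; These bindings serve shake syncing, reward timing and health monitoring.
; BeginPlay and construction only call the parent class.
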(event EventBeginPlay
  (|CallParentFunction))

(fn ConstructionScript
  (|CallParentFunction))

(fn F绑定附加障碍物
  (bind _asbp_组合轮胎_平铺 (Utilities|Casting|CastToBP_组合轮胎_平铺 (Actor|GetAttachParentActor)))
  (LocalVariables|Set平铺轮胎 _asbp_组合轮胎_平铺)
  ;[1 0 0.4687 0.8] 同步抖动
  (EventDispatchers|BindEventtoED-UMG缩放时 (LocalVariables|Get平铺轮胎) (EventDispatchers|CreateEvent :!event CE播放上下抖动))
  ;[0.8281 1 0 0.8] 什么时候获取奖励
  (EventDispatchers|BindEventtoED-所有轮胎都爆炸时 (LocalVariables|Get平铺轮胎) (EventDispatchers|CreateEvent :!event CE获得))
  ;[0.8516 0 1 0.8] 监测生命值
  (EventDispatchers|BindEventtoED-生命值变化时 (LocalVariables|Get平铺轮胎) (EventDispatchers|CreateEvent :!event CEED-绑定生命值变化时)))