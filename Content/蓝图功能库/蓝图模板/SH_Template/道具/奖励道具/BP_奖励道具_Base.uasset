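; Base reward pickup that, when obtained, flashes, flies along a timeline-driven arc to its target with scale and effect changes, then grants its rewards.
; Rewards come from attached BP_奖励效果_Base actors, plus an optional "CE" console event; without a valid target it switches to physics simulation.
; It also provides bobbing, material-parameter flashing across attached meshes, and health-driven jump/hit animation flags.
; Subclasses override F绑定附加障碍物 to bind obstacles.
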(event Custom|CE_闪烁
  (bind _高亮参数 (Variables|默认|高亮设置|Get高亮参数))
  (bind (_变化耗时 _参数名称 _起始值 _结束值) (Utilities|Struct|BreakS_材质变化 _高亮参数))
  ;[1 1 1] 闪烁
  (for _array_element (Actor|GetAttachedActors true false)
    (bind _网格体组件 (CallFunction|F获取所有网格体组件 _array_element true true false))
    (Utilities|Array|AppendArray (Variables|调试状态|Get有效网格体组件) _网格体组件))
  (Rendering|Material|SetVectorParameterValueonMaterials (Variables|调试状态|Get有效网格体组件) "SH_闪烁Color" (Math|Conversions|ToVector(LinearColor) (Variables|默认|高亮设置|Get高亮颜色)))
  (Components|Timeline|SetPlayRate (Variables|Default|GetTL_闪烁) (/ 1.0 _变化耗时))
  (bind _f (Timeline|TL_闪烁 PlayFromStart)
    (:Update
      (Rendering|Material|SetScalarParameterValueonMaterials (Variables|调试状态|Get有效网格体组件) _参数名称 (Math|Float|Lerp _起始值 _结束值 _f)))))

(event Custom|CE_播放上下抖动
  (bind _root_道具 (Variables|Default|GetRoot_道具))
  (bind _常亮特效_初始相对缩放 (Variables|调试状态|Get常亮特效_初始相对缩放))
  (bind _root道具_初始相对缩放 (Variables|调试状态|GetRoot道具_初始相对缩放))
  ;[1 0 0.8672] 抖动动画
  (if (and (not (Variables|调试状态|Get已被获得)) (or (!= (Variables|默认|抖动设置|Get道具抖动强度_上下) 0.0) (!= (Variables|默认|抖动设置|Get特效抖动强度_上下) 0.0)))
    (Components|Timeline|SetPlayRate (Variables|Default|GetTL_上下抖动) (/ 1.0 (Variables|默认|抖动设置|Get抖动一次耗时)))
    (bind _f (Timeline|TL_上下抖动 Play)
      (:Update
        (Utilities|FlowControl|Sequence
          (:then_0
            ;;[0 0.01562 1 0.8] 道具抖动
            (if (!= (Variables|默认|抖动设置|Get道具抖动强度_上下) 0.0)
              (Transformation|SetRelativeLocation _root_道具 (+ (Variables|调试状态|GetRoot道具_初始相对位置) (Math|Vector|MakeVector 0.0 0.0 (Math|Float|Lerp 0.0 (Variables|默认|抖动设置|Get道具抖动强度_上下) _f))) false false)
              (Transformation|SetRelativeScale3D _root_道具 (Math|Vector|Lerp(Vector) _root道具_初始相对缩放 (* _root道具_初始相对缩放 (Variables|默认|抖动设置|Get道具抖动强度_缩放)) _f))))
          (:then_1
            ;;[1 0.9609 0 0.8] 特效抖动
            (if (!= (Variables|默认|抖动设置|Get特效抖动强度_上下) 0.0)
              (Transformation|SetRelativeLocation (Variables|Default|GetRoot_特效) (+ (Variables|调试状态|GetRoot特效%20初始相对位置) (Math|Vector|MakeVector 0.0 0.0 (Math|Float|Lerp 0.0 (Variables|默认|抖动设置|Get特效抖动强度_上下) _f))) false false)
              (Transformation|SetRelativeScale3D (Variables|Default|Get常亮特效_P) (Math|Vector|Lerp(Vector) _常亮特效_初始相对缩放 (* _常亮特效_初始相对缩放 (Variables|默认|抖动设置|Get特效抖动强度_缩放)) _f))))))
      (:Finished
        ;;[0.5234 1 0 0.8] 重置
        (Utilities|FlowControl|Delay 0.0)
        (Timeline|TL_上下抖动 SetNewTime)))))

(event Custom|CEED-绑定生命值变化时
  (params (当前生命值 :type Float%20%28double-precision%29))
  ;[0.07812 1 0 0.8] CEED-绑定生命值变化时
  (Variables|调试状态|Set绑定生命值 当前生命值)
  (Utilities|FlowControl|Sequence
    (:then_0
      (Utilities|IsValid (Variables|默认|骨骼模型设置|Get跳跃动画)
        (:Is%20Valid
          (bind _output_get (Variables|调试状态|Set已起跳 (<= (Variables|调试状态|Get绑定生命值) (Variables|默认|骨骼模型设置|Get提前起跳值))))
          (if _output_get
            (Utilities|FlowControl|DoOnce false
              (:Completed
                (bind _起跳前音效 (Variables|默认|骨骼模型设置|Get起跳前音效)
                  (:then
                    (Audio|PlaySound2D _起跳前音效 0.7 1.0 0.0 0 0))
                  (:else))))))))
    (:then_1
      (Utilities|IsValid (Variables|默认|骨骼模型设置|Get受击动画)
        (:Is%20Valid
          (Variables|调试状态|Set正在受击 true)
          (Utilities|FlowControl|RetriggerableDelay 0.5)
          (Variables|调试状态|Set正在受击 false))))))

(event Custom|CE_获得
  ;[1 0 0.4453 0.8] CE_获得    飞向获取者并执行效果
  (CallFunction|CE闪烁)
  (Utilities|IsValid (Variables|默认|飞行设置|Get飞行目标)
    (:Is%20Valid
      (Utilities|FlowControl|DoOnce false
        (:Completed
          (Variables|调试状态|Set已被获得 true)
          (Transformation|DetachFromActor "KeepWorld" "KeepWorld" "KeepWorld")
          ;;[0 0.8828 1] 飞行起点
          (Variables|调试状态|SetActor_初始位置 (Transformation|GetActorLocation))
          ;;[0 1 1] 特效控制
          (Components|Activation|Activate (Variables|Default|Get激活特效_P) true)
          (Development|SetHiddeninGame (Variables|Default|Get常亮特效_P) (Variables|默认|飞行设置|Get起飞时隐藏常亮特效) false)
          (Components|Timeline|SetPlayRate (Variables|Default|Get道具飞时间轴) (Variables|默认|飞行设置|Get飞行速率))
          ;;[0 0.4141 1] 飞向目标
          (bind _复合轨道 (Timeline|道具飞时间轴 PlayFromStart)
            (:Update
              (bind _output_get (Variables|调试状态|Set复合轨道AlphaV _复合轨道))
              (Transformation|SetActorLocation (+ (Math|Vector|MakeVector 0.0 0.0 (* (.z _output_get) (Variables|默认|飞行设置|Get飞行高度))) (Math|Vector|Lerp(Vector) (Variables|调试状态|GetActor_初始位置) (Transformation|GetActorLocation (Variables|默认|飞行设置|Get飞行目标)) (.x _output_get))) false false)
              (Transformation|SetRelativeScale3D (Variables|Default|GetRoot_道具) (Math|Conversions|ToVector(Float) (.y _output_get)))
              (Transformation|SetRelativeScale3D (Variables|Default|Get常亮特效_P) (* (Variables|调试状态|Get常亮特效_初始相对缩放) (.y _output_get))))
            (:Finished
              ;;[1 0.8672 0] 落地后
              (CallFunction|F执行奖励效果)
              (Development|SetHiddeninGame (Variables|Default|Get道具模型) true true)
              (Components|Activation|Activate (Variables|Default|Get完成时特效_P) true)
              (Actor|SetLifeSpan 3.0)
              (Utilities|FlowControl|Sequence
                (:then_0
                  (if (Variables|默认|飞行设置|Get落地时隐藏激活特效)
                    (Development|SetHiddeninGame (Variables|Default|Get激活特效_P) true false)))
                (:then_1
                  (if (Variables|默认|飞行设置|Get落地后附加到飞行目标)
                    (Transformation|AttachActorToActor (Variables|默认|飞行设置|Get飞行目标) "None" "KeepWorld" "KeepWorld" "KeepWorld" true)))))))))
    (:Is%20Not%20Valid
      (CallFunction|一键模拟物理 (Variables|Default|GetRoot_Box) "PhysicsOnly" "ECC_PhysicsBody" true))))

(event EventBeginPlay
  ;[0.2891 0 1] 初始化
  (CallFunction|F初始绑定奖励效果)
  (Variables|调试状态|SetRoot道具_初始相对位置 (Variables|/Script/Engine.SceneComponent|GetRelativeLocation (Variables|Default|GetRoot_道具)))
  (Variables|调试状态|SetRoot特效%20初始相对位置 (Variables|/Script/Engine.SceneComponent|GetRelativeLocation (Variables|Default|GetRoot_特效)))
  (Variables|调试状态|SetActor_初始位置 (Transformation|GetActorLocation))
  (Variables|调试状态|Set常亮特效_初始相对缩放 (Variables|/Script/Engine.SceneComponent|GetRelativeScale3D (Variables|Default|Get常亮特效_P)))
  (Variables|调试状态|SetRoot道具_初始相对缩放 (Variables|/Script/Engine.SceneComponent|GetRelativeScale3D (Variables|Default|GetRoot_道具)))
  (bind _网格体组件 (CallFunction|F获取所有网格体组件 self true true false))
  (Variables|调试状态|Set有效网格体组件 _网格体组件)
  (CallFunction|F绑定附加障碍物))

(fn ConstructionScript)

(fn F执行奖励效果
  (Utilities|FlowControl|Sequence
    (:then_0
      (if (Utilities|Enum|NotEqual(Enum) (Variables|默认|飞行设置|Get完成时Event) "")
        (Development|ExecuteConsoleCommand (Utilities|String|Append "CE " (Variables|默认|飞行设置|Get完成时Event)) 0)))
    (:then_1
      (if (Utilities|Array|IsNotEmpty (Variables|调试状态|Get奖励效果))
        (for _array_element (Variables|调试状态|Get奖励效果)
          (Utilities|IsValid _array_element
            (:Is%20Valid
              (Default|CE-获得奖励 _array_element))))))))

(fn F初始绑定奖励效果
  (bind _output_get (LocalVariables|Set附加的actors (Actor|GetAttachedActors true false)))
  (for _array_element _output_get
    (bind _asbp_奖励效果_base (Utilities|Casting|CastToBP_奖励效果_Base _array_element))
    (Utilities|Array|Add (Variables|调试状态|Get奖励效果) _asbp_奖励效果_base)))

(fn F绑定附加障碍物)