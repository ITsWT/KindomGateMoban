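; Light gate obstacle that turns hits into red or blue soldiers.
; Damage lowers signed health, updating the number and materials; the sign, optionally inverted, picks the colour.
; Accumulated damage past a threshold spawns a soldier at a seeded random point in the HitBox and launches it forward; health or spawn limits kill the gate.
; The construction script fits frame, curtain and HitBox to the gate width.
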(event EventBeginPlay
  (|CallParentFunction)
  (更新材质|F更新光门材质)
  (更新属性|F显隐WidgetC false)
  (bind _returnvalue (Actor|GetActorOfClass "/Game/蓝图功能库/蓝图模板/SH_Template/角色/玩家控制器/BP_音效控制.BP_音效控制_C"))
  (Variables|Default|SetBP_音效控制 _returnvalue))

(event EventTick
  (params (DeltaSeconds :type Float%20%28single-precision%29))
  (|CallParentFunction DeltaSeconds) ; 此节点被禁用，将不会被调用。\n从引脚连出引线来编译功能。
)

(event EventCE障碍物受击
  (params (伤害值 :type Float%20%28double-precision%29))
  (bind _每次出兵要求数量 (Variables|默认|生成士兵|Get每次出兵要求数量))
  (if (Variables|Default|Get能够受伤？)
    ;[0.8281 0 1] 计算扣多少
    (bind _output_get (Variables|状态|Set最后受到的伤害值 (select (!= (select (> (Variables|Default|Get障碍物生命值_Cur) 0.0) (Variables|Default|Get每次受到伤害值) (Variables|默认|生命值|Get每次受到伤害值_负)) 0.0) (select (> (Variables|Default|Get障碍物生命值_Cur) 0.0) (Variables|Default|Get每次受到伤害值) (Variables|默认|生命值|Get每次受到伤害值_负)) (* 伤害值 (Variables|Default|Get受到伤害百分比)))))
    ;[0 1 0.7891 0.8] 设置生命值
    (Variables|Default|Set障碍物生命值_Cur (- (Variables|Default|Get障碍物生命值_Cur) _output_get))
    ;[0.4531 0 1 0.8] 记录累计伤害
    (Variables|状态|Set累计出兵伤害值 (+ (Variables|状态|Get累计出兵伤害值) (Math|Float|Absolute(Float) (Variables|状态|Get最后受到的伤害值))))
    (Utilities|FlowControl|Sequence
      (:then_0
        ;[1 0 0.2578 0.8] 播放受击反馈
        (CallFunction|CE播放受击反馈)
        ;[0.15 0 0.02348 0.5] 使用BP_音效控制蓝图播放音效
        (Default|CE子弹击中 (Variables|Default|GetBP_音效控制) "NewEnumerator1"))
      (:then_1
        ;[0.4766 1 0 0.8] 更新文本和材质
        (CallFunction|F修改UMG文本数字 (Variables|Default|GetAs%20UMG%20文本) (Variables|Default|Get障碍物生命值_Cur) (Variables|Default|Get反转红蓝))
        (更新材质|F更新光门材质))
      (:then_2
        ;[0.5 0 1 0.8] 判断生成士兵
        (if (>= (Variables|状态|Get累计出兵伤害值) (select (<= (Variables|Default|Get障碍物生命值_Cur) 0.0) (.y _每次出兵要求数量) (.x _每次出兵要求数量)))
          (Variables|状态|Set累计出兵伤害值 (- (Variables|状态|Get累计出兵伤害值) (select (<= (Variables|Default|Get障碍物生命值_Cur) 0.0) (.y _每次出兵要求数量) (.x _每次出兵要求数量))))
          (默认|F生成士兵 (数值计算|F检查反转红蓝 (< (Variables|Default|Get障碍物生命值_Cur) 0.0)))))
      (:then_3
        ;[0.4062 1 0] 判断死亡
        (if (or (and (<= (Variables|Default|Get障碍物生命值_Cur) 0.0) (Variables|Default|Get生命值低于零时死亡)) (> (Math|Float|Absolute(Float) (Variables|Default|Get障碍物生命值_Cur)) (Variables|Default|Get最大生命值上限_Abs)))
          (CallFunction|CE死亡 0 "生命值达到死亡标准"))))
    (else
      ;[1 0 0.2578 0.8] 播放受击反馈
      (CallFunction|CE播放受击反馈))))

(fn ConstructionScript
  (|CallParentFunction)
  (更新材质|F更新光门材质)
  (初始化|F初始化光门宽度C))

(fn F障碍物受击缩放
  (bind _受击时光门缩放程度 (Variables|默认|反馈动画|Get受击时光门缩放程度))
  (bind _受击alphav (Variables|Default|Get受击alphaV))
  (bind _returnvalue (* (.z _受击alphav) _受击时光门缩放程度))
  (Transformation|SetRelativeScale3D (Variables|Default|GetRoot_障碍物模型) (Math|Vector|MakeVector _returnvalue _returnvalue _returnvalue))
  (Transformation|SetRelativeScale3D (Variables|Default|GetRoot_widget) (Math|Vector|MakeVector _returnvalue _returnvalue _returnvalue)))

(fn F更新光门材质
  (更新材质|F修改光幕材质C)
  (更新材质|F修改门框材质C))

(fn F修改光幕材质C
  (Rendering|Material|SetMaterial (Variables|Default|GetSM_光幕) 0 (select (数值计算|F检查反转红蓝 (< (Variables|Default|Get障碍物生命值_Cur) 0.0)) "/Game/场景道具/光门/细版/Mat/MI_半透明纯色_红色.MI_半透明纯色_红色" "/Game/场景道具/光门/细版/Mat/MI_半透明纯色_蓝色.MI_半透明纯色_蓝色")))

(fn F修改门框材质C
  (bind _sm_门框_r (Variables|Default|GetSM_门框_R))
  (bind _障碍物生命值_cur (Variables|Default|Get障碍物生命值_Cur))
  (bind _returnvalue (< _障碍物生命值_cur 0.0))
  (bind _检测反转颜色 (数值计算|F检查反转红蓝 _returnvalue))
  (bind _returnvalue_2 (select _检测反转颜色 "/Game/场景道具/光门/细版/Mat/MI_BasicPBR_红色.MI_BasicPBR_红色" "/Game/场景道具/光门/细版/Mat/MI_BasicPBR_蓝色.MI_BasicPBR_蓝色"))
  (Rendering|Material|SetMaterial _sm_门框_r 0 _returnvalue_2)
  (Rendering|Material|SetMaterial _sm_门框_r 1 _returnvalue_2)
  (Rendering|Material|SetMaterial _sm_门框_r 2 _returnvalue_2))

(fn F生成士兵
  (params (红兵 :type Boolean))
  (bind _returnvalue (Transformation|GetActorRotation))
  (bind _hitbox (Variables|Default|GetHitBox))
  (bind _障碍物seed (Variables|Default|Get障碍物Seed))
  (bind _root_小兵生成高度 (Variables|Default|GetRoot_小兵生成高度))
  (bind _蓝兵_class (Variables|默认|生成士兵|Get蓝兵_Class))
  (bind _红兵_class (Variables|默认|生成士兵|Get红兵_Class))
  (bind _障碍物seed_2 (Variables|Default|Get障碍物Seed))
  (bind _returnvalue_2 (Components|Box|GetScaledBoxExtent _hitbox))
  (bind _随机流送 (CallFunction|流送中的随机流送 _障碍物seed_2))
  (bind _returnvalue_3 (Transformation|GetWorldLocation _root_小兵生成高度))
  (bind _returnvalue_4 (Transformation|GetWorldLocation _hitbox))
  (bind _returnvalue_5 (select 红兵 _红兵_class _蓝兵_class))
  (bind _returnvalue_6 (CallFunction|流送中边界框中随机点 _returnvalue_4 _returnvalue_2 _障碍物seed "0, 0, 0"))
  (bind _角色所属阵营 (Utilities|GetClassDefaults _returnvalue_5))
  (bind _xyz (CallFunction|向量合并XYZ轴 _returnvalue_6 _returnvalue_3))
  (if (Variables|默认|生成士兵|Get能够生成士兵?)
    (if 红兵
      (bind _returnvalue_7 (Game|SpawnActorfromClass _红兵_class (Math|Transform|MakeTransform _xyz _returnvalue "1.000000,1.000000,1.000000") "Undefined" "MultiplyWithRoot" 0 _随机流送 _角色所属阵营 0 -1.0 0))
      ;[1 0 0.1641] 弹出红兵
      (Utilities|IsValid _returnvalue_7
        (:Is%20Valid
          (Utilities|IsValid (Variables|/Game/蓝图功能库/蓝图模板/SH_Template/角色/BP_SH角色_Base.BP_SH角色_Base_C|GetRef物理移动 _returnvalue_7)
            (:Is%20Valid
              (Default|F弹射物理移动 (Variables|/Game/蓝图功能库/蓝图模板/SH_Template/角色/BP_SH角色_Base.BP_SH角色_Base_C|GetRef物理移动 _returnvalue_7) (Math|Vector|RotateVector (* (Transformation|GetActorForwardVector) (.x (Variables|默认|生成士兵|Get红兵/蓝兵弹出速度))) (Math|Rotator|MakeRotator 0.0 0.0 (CallFunction|流送中绝对值范围内随机浮点 (.x (Variables|默认|生成士兵|Get红兵/蓝兵弹出角度)) (Variables|Default|Get障碍物Seed)))) false)
              ;[0.9688 1 0] 红兵数量达到一定程度后 光门死亡
              (bind _result (Math|Integer|IncrementInt (.y (Variables|状态|Get已生成士兵数量)))
                (:%20%20
                  (if (>= _result (.y (Variables|默认|生成士兵|Get生成士兵数量限制)))
                    (Variables|默认|生成士兵|Set能够生成士兵? false)
                    (CallFunction|CE死亡))))))))
      (else
        (bind _returnvalue_8 (Game|SpawnActorfromClass _蓝兵_class (Math|Transform|MakeTransform _xyz _returnvalue "1.000000,1.000000,1.000000") "Undefined" "MultiplyWithRoot" 0 _随机流送 _角色所属阵营 0 -1.0 0))
        ;[1 0.7969 0] 弹出蓝兵
        (Utilities|IsValid _returnvalue_8
          (:Is%20Valid
            (Utilities|IsValid (Variables|/Game/蓝图功能库/蓝图模板/SH_Template/角色/BP_SH角色_Base.BP_SH角色_Base_C|GetRef物理移动 _returnvalue_8)
              (:Is%20Valid
                (Default|F弹射物理移动 (Variables|/Game/蓝图功能库/蓝图模板/SH_Template/角色/BP_SH角色_Base.BP_SH角色_Base_C|GetRef物理移动 _returnvalue_8) (Math|Vector|RotateVector (* (Transformation|GetActorForwardVector) (.y (Variables|默认|生成士兵|Get红兵/蓝兵弹出速度))) (Math|Rotator|MakeRotator 0.0 0.0 (CallFunction|流送中绝对值范围内随机浮点 (.y (Variables|默认|生成士兵|Get红兵/蓝兵弹出角度)) (Variables|Default|Get障碍物Seed)))) false)
                ;[0.9688 1 0] 蓝兵数量达到一定程度后 光门死亡
                (bind _result_2 (Math|Integer|IncrementInt (.x (Variables|状态|Get已生成士兵数量)))
                  (:%20%20
                    (if (>= _result_2 (.x (Variables|默认|生成士兵|Get生成士兵数量限制)))
                      (Variables|默认|生成士兵|Set能够生成士兵? false)
                      (CallFunction|CE死亡 0 "生成士兵过多"))))))))))))

(fn F修改UMG文本数字
  (params (As%20UMG%20文本 :type UMG%20文本%20Object%20Reference) (Number :type Float%20%28double-precision%29) (反转符号 :type Boolean))
  (Default|F修改文本内容Float As%20UMG%20文本 Number (select (>= (Math|Float|Sign(Float) Number) 0.0) "ToPositiveInfinity" "ToNegativeInfinity") true 反转符号 false 0 true))

(fn F检查反转红蓝
  (params (当前颜色 :type Boolean))
  (return (select (Variables|Default|Get反转红蓝) (not 当前颜色) 当前颜色)))

(fn F初始化光门宽度C
  (bind _sm_门框_r (Variables|Default|GetSM_门框_R))
  (bind _门的宽度 (Variables|Default|Get门的宽度))
  (bind _sm_光幕 (Variables|Default|GetSM_光幕))
  (bind _sm_门框_l (Variables|Default|GetSM_门框_L))
  (bind _relativelocation (Variables|/Script/Engine.SceneComponent|GetRelativeLocation _sm_门框_r))
  (bind _relativelocation_2 (Variables|/Script/Engine.SceneComponent|GetRelativeLocation _sm_门框_l))
  (bind _relativescale3d (Variables|/Script/Engine.SceneComponent|GetRelativeScale3D _sm_光幕))
  (Transformation|SetRelativeLocation _sm_门框_l (Math|Vector|MakeVector (.x _relativelocation_2) _门的宽度 (.z _relativelocation_2)) false false)
  (Transformation|SetRelativeLocation _sm_门框_r (Math|Vector|MakeVector (.x _relativelocation) (* _门的宽度 -1.0) (.z _relativelocation)) false false)
  (Components|Box|SetBoxExtent (Variables|Default|GetHitBox) (Math|Vector|MakeVector 2e+01 (Variables|Default|Get门的宽度) 8e+01) true)
  (Transformation|SetRelativeScale3D _sm_光幕 (Math|Vector|MakeVector (+ (* (Variables|Default|Get门的宽度) 2.0 0.01) 0.1) (.y _relativescale3d) (.z _relativescale3d))))

(fn F显隐WidgetC
  (params (隐藏 :type Boolean))
  ;[0 1 0.3203 0.8] 建议子类覆写
  (Development|SetHiddeninGame (Variables|Default|GetWidget_文本) 隐藏 false))