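; Light gate array (光门阵列) actor that places a single row of gate actors as obstacles.
; The construction script previews the row with HISM instances from a formation helper.
; BeginPlay spawns a gate at each instance transform, attaches and stores it, then hides the preview; Tick repeats spawning on a cooldown when the interval is non-negative.
; An optional downward trace snaps the array to ground during construction and every Tick.
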(event Custom|CE-生成一次
  (Variables|Default|Get光门_Class
    (:then
      (bind _transform_array (CallFunction|F获取实例变换))
      (for _array_element _transform_array
        (bind _returnvalue (Game|SpawnActorfromClass (Variables|Default|Get光门_Class) (CallFunction|变换相加 _array_element (Variables|Default|Get光门变换调整)) "AlwaysSpawn" "MultiplyWithRoot" self true (Variables|Default|Get受击反馈时间) (Variables|Default|Get生成的人物类型) 0))
        (Utilities|IsValid _returnvalue
          (:Is%20Valid
            (CallFunction|F生成光门后 _returnvalue))))
      (Development|SetHiddeninGame (Variables|Default|GetHierarchicalInstancedStaticMesh) true false))
    (:else)))

(event Custom|CE_对齐到地面
  ;[0.1484 1 0] 对齐到地面
  (bind (_是否命中 _命中结果) (CallFunction|向下的对象的线条检测 (Transformation|GetActorLocation) 1e+02 2e+03 (Utilities|Array|MakeArray "ObjectTypeQuery1") false "None" 1.0))
  (if _是否命中
    (Transformation|SetActorLocation (CallFunction|向量合并XYZ轴 (Transformation|GetActorLocation) (.Location (Collision|BreakHitResult _命中结果))) false false)))

(event EventBeginPlay
  (CallFunction|CE-生成一次))

(event EventTick
  (params (DeltaSeconds :type Float%20%28single-precision%29))
  (|CallParentFunction DeltaSeconds)
  (Utilities|FlowControl|Sequence
    (:then_0
      (if (>= (Variables|默认|持续生成|Get持续生成间隔时间) 0.0)
        (Utilities|冷却 (Variables|默认|持续生成|Get持续生成间隔时间)
          (:Completed
            (CallFunction|CE-生成一次)))))
    (:then_1
      (if (Variables|Default|Get轮胎_对齐到地面？)
        (CallFunction|CE对齐到地面)))))

(fn ConstructionScript
  (Components|StaticMesh|SetStaticMesh (Variables|Default|GetHierarchicalInstancedStaticMesh) (Variables|Default|Get预览网格体))
  (bind _位置 (CallFunction|Formation实心矩形 1 (Variables|Default|Get生成数量) (Variables|Default|Get行间距) -1e+02 false false "1.000000,0,0" "0,1.000000,0"))
  (for _array_element _位置
    (Components|InstancedStaticMesh|AddInstance (Variables|Default|GetHierarchicalInstancedStaticMesh) (CallFunction|变换相加 (Math|Transform|MakeTransform _array_element "0, 0, 0" "1.000000,1.000000,1.000000") (Variables|Default|Get光门变换调整)) false))
  (if (Variables|Default|Get轮胎_对齐到地面？)
    (CallFunction|CE对齐到地面)))

(fn F获取实例变换
  (bind _hierarchicalinstancedstaticmesh (Variables|Default|GetHierarchicalInstancedStaticMesh))
  (for _index (range 0 (- (Components|InstancedStaticMesh|GetInstanceCount _hierarchicalinstancedstaticmesh) 1))
    (Utilities|Array|Add (LocalVariables|GetTransform) (.OutInstanceTransform (Components|InstancedStaticMesh|GetInstanceTransform _hierarchicalinstancedstaticmesh _index true))))
  (return (LocalVariables|GetTransform)))

(fn F生成光门后
  (params (New光门 :type BP%20障碍物%20光门%20Object%20Reference%20%28by%20ref%29))
  (Utilities|Array|Add (Variables|Default|Get生成的光门_array) New光门)
  (Transformation|AttachActorToActor New光门 self "None" "KeepWorld" "KeepWorld" "KeepWorld" true)
  (Default|CallED绑定到父类时 New光门))

(fn F光门功能开关
  (params (开关 :type Boolean))
  (for _array_element (Variables|Default|Get生成的光门_array)
    (Variables|/Game/蓝图功能库/蓝图模板/SH_Template/道具/障碍物/BP_障碍物_Base.BP_障碍物_Base_C|Set障碍物已启用 _array_element 开关)))