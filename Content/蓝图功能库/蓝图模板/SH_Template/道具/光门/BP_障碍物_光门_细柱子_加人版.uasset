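; Thin-pillar light gate obstacle, add-troops variant, that grows or shrinks a faction-1 squad on overlap.
; Its value comes from the parent gate array when bound, and hits raise it by one per cooldown.
; Actor scale follows the absolute value, with a one-time particle burst at the red-to-blue crossing.
; On contact it kills units if negative, otherwise spawns soldiers with optional radial launch, then broadcasts broken and destroys itself.
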(event OnComponentBeginOverlap(HitBox)
  (params (OverlappedComponent :type Primitive%20Component%20Object%20Reference) (OtherActor :type Actor%20Object%20Reference) (OtherComp :type Primitive%20Component%20Object%20Reference) (OtherBodyIndex :type Integer) (bFromSweep :type Boolean) (SweepResult :type Hit%20Result%20Structure%20%28by%20ref%29))
  (if (Variables|Default|Get障碍物已启用)
    (bind _asbp_sh角色_base (Utilities|Casting|CastToBP_SH角色_Base OtherActor))
    (Variables|Default|SetRef集中点 (Variables|/Game/蓝图功能库/蓝图模板/SH_Template/角色/BP_SH角色_Base.BP_SH角色_Base_C|GetRef集中点 _asbp_sh角色_base))
    (if (== (Variables|/Game/蓝图功能库/蓝图模板/SH_Template/角色/BP_SH角色_Base.BP_SH角色_Base_C|Get角色所属阵营 _asbp_sh角色_base) 1)
      (Utilities|IsValid (Variables|Default|GetRef集中点)
        (:Is%20Valid
          (Utilities|FlowControl|DoOnce false
            (:Completed
              ;[0.02276 0.15 0 0.5] 震屏
              (CallFunction|震屏 "/Game/蓝图功能库/相机振动/CS_获得奖励.CS_获得奖励_C")
              ;[0.0202 0.15 0.007367 0.5] 在目标点触发总体特效
              (CallFunction|F生成粒子特效 (Math|Transform|MakeTransform (+ (Transformation|GetActorLocation (Variables|Default|GetRef集中点)) "0.000000,0.000000,-120.000000") "0, 0, 0" "1.500000,1.500000,1.500000") (Utilities|Struct|MakeF粒子特效 0 "/Game/分类/升级/放置升级黄色.放置升级黄色") (Variables|/Game/蓝图功能库/蓝图模板/SH_Template/角色/集中点/BP_集中点.BP_集中点_C|GetSphere_核心 (Variables|Default|GetRef集中点)) "None" "KeepWorldPosition" true true false)
              (CallFunction|F生成粒子特效 (Math|Transform|MakeTransform (Transformation|GetWorldLocation (Variables|/Script/Engine.Actor|GetRootComponent (Variables|Default|GetRef集中点))) "0, 0, 0" "1.500000,1.500000,1.500000") (Utilities|Struct|MakeF粒子特效 0 "/Game/分类/升级/士兵升级5.士兵升级5") (Variables|/Script/Engine.Actor|GetRootComponent (Variables|Default|GetRef集中点)) "None" "KeepWorldPosition" true true false)
              ;[1 0.5469 0.5469] 根据数值判断当前是加还是减
              (if (< (Variables|Default|Get障碍物生命值_Cur) 0.0)
                ;[0.2575 1 0 0.5] 减少一部分
                (Default|F杀死一批 (Variables|Default|GetRef集中点) (Math|Float|Truncate (Math|Float|Absolute(Float) (Variables|Default|Get障碍物生命值_Cur))) "(X=1500.000000,Y=2000.000000)" "(X=750.000000,Y=1500.000000)")
                (Default|CallED-障碍物被打破时 self)
                (Actor|DestroyActor)
                (else
                  (Audio|PlaySoundatLocation "/Game/DoormdayTrain/Audios/shengji.shengji" (Transformation|GetActorLocation) "0, 0, 0" 2.0 1.0 0.0 0 0 0 0)
                  ;[0 1 0.5078 0.8] 中心加人
                  (bind _生成角色 (Default|F增加人数-外围 (Variables|Default|GetRef集中点) (Math|Float|Truncate (Variables|Default|Get障碍物生命值_Cur)) 6e+01 0.0 "/Game/蓝图功能库/蓝图模板/SH_Template/角色/跑酷角色/BP_SH角色_士兵_帽子男.BP_SH角色_士兵_帽子男_C" "1.000000,1.000000,1.000000"))
                  (for (_array_element _array_index) _生成角色
                    (Default|CE播放网格体缩放 _array_element 0.35 "/Game/蓝图功能库/函数库/Curve/缩放动画/CV_SA_先细后大_p150.CV_SA_先细后大_p150" 0.0)
                    (Default|CE-播放闪烁 _array_element true "(R=100.000000,G=24.710846,B=0.000000,A=1.000000)" -1.0 true 0.3)
                    (CallFunction|F生成粒子特效 (Math|Transform|MakeTransform (Transformation|GetWorldLocation (Variables|/Script/Engine.Character|GetMesh _array_element)) "0, 0, 0" "0.500000,0.500000,0.500000") (Utilities|Struct|MakeF粒子特效 0 "/Game/分类/升级/放置升级黄色.放置升级黄色") (Variables|/Script/Engine.Actor|GetRootComponent _array_element) "None" "KeepWorldPosition" true true false)
                    (CallFunction|F生成粒子特效 (Math|Transform|MakeTransform (Transformation|GetWorldLocation (Variables|/Script/Engine.Character|GetMesh _array_element)) "0, 0, 0" "1.000000,1.000000,1.000000") (Utilities|Struct|MakeF粒子特效 0 "/Game/分类/升级/士兵升级6.士兵升级6") (Variables|/Script/Engine.Actor|GetRootComponent _array_element) "None" "KeepWorldPosition" true true false)
                    (if (Variables|Default|Get开启物理移动)
                      (Utilities|IsValid (Variables|/Game/蓝图功能库/蓝图模板/SH_Template/角色/BP_SH角色_Base.BP_SH角色_Base_C|GetRef物理移动 _array_element)
                        (:Is%20Valid
                          (Default|F弹射物理移动 (Variables|/Game/蓝图功能库/蓝图模板/SH_Template/角色/BP_SH角色_Base.BP_SH角色_Base_C|GetRef物理移动 _array_element) (* (Math|Vector|RotateVector (Transformation|GetActorForwardVector (Variables|Default|GetRef集中点)) (Math|Rotator|MakeRotator 0.0 0.0 (* _array_index (/ 3.6e+02 (Variables|Default|Get障碍物生命值_Cur))))) (Math|Float|Clamp(Float) (* (Utilities|Array|Length (Variables|/Game/蓝图功能库/蓝图模板/SH_Template/角色/集中点/BP_集中点.BP_集中点_C|Get集中的角色数组 (Variables|Default|GetRef集中点))) 200) (.x (Variables|/Game/蓝图功能库/蓝图模板/SH_Template/角色/集中点/BP_物理移动.BP_物理移动_C|Get生成力范围 (Variables|/Game/蓝图功能库/蓝图模板/SH_Template/角色/BP_SH角色_Base.BP_SH角色_Base_C|GetRef物理移动 _array_element))) (.y (Variables|/Game/蓝图功能库/蓝图模板/SH_Template/角色/集中点/BP_物理移动.BP_物理移动_C|Get生成力范围 (Variables|/Game/蓝图功能库/蓝图模板/SH_Template/角色/BP_SH角色_Base.BP_SH角色_Base_C|GetRef物理移动 _array_element))))) false)))))
                  (Default|CallED-障碍物被打破时 self)
                  (Actor|DestroyActor))))))))))

(event Custom|CE_受击改变缩放和数值
  (bind _root_光门 (Variables|Default|GetRoot_光门))
  (bind _returnvalue (Transformation|GetWorldTransform _root_光门))
  ;[0.0639 0.15 0.02282 0.5] CE_受击改变缩放和数值
  (Variables|Default|Set上一个缩放 (Variables|Default|Get初始缩放))
  (Variables|Default|Set初始缩放 (CallFunction|F计算缩放与数值比例))
  (Utilities|FlowControl|Sequence
    (:then_0
      (Components|Timeline|SetPlayRate (Variables|Default|GetTimeline) (/ 0.3 (Variables|Default|Get受击反馈间隔时间)))
      (bind _newtrack_0 (Timeline|Timeline PlayFromStart)
        (:Update
          (Transformation|SetActorScale3D (Math|Conversions|ToVector(Float) (Math|Float|Lerp (Variables|Default|Get上一个缩放) (Variables|Default|Get初始缩放) _newtrack_0))))))
    (:then_1
      ;[0 0.15 0.004569 0.5] 当从红变蓝时播放一次范围特效
      (if (== (Class|KismetMathLibrary|FFloor64 (Variables|Default|Get障碍物生命值_Cur)) 0)
        (Utilities|FlowControl|DoOnce false
          (:Completed
            (CallFunction|F生成粒子特效 (Math|Transform|MakeTransform (.location _returnvalue) "0, 0, 0" (* (.scale _returnvalue) "0.100000,1.000000,0.500000")) (Variables|Default|Get门切换颜色粒子) (Variables|Default|GetRoot_光门) "None" "KeepWorldPosition" true true false)))))))

(event Custom|ED_绑定到父类时_Event
  ;[0.08684 0.15 0.02965 0.5] 当蓝图生成并绑定到父对象时调用该函数修改数值（实现直接设置数值）|在父类的 “F生成光门后” 函数内调用
  (CallFunction|F获取并设置当前显示数值)
  (CallFunction|F初始化文本)
  (CallFunction|F更新光门材质)
  (CallFunction|F显隐WidgetC false)
  (CallFunction|F受击改变缩放和数值))

(event EventBeginPlay
  (|CallParentFunction)
  ;[0.08684 0.15 0.02965 0.5] 当蓝图生成并绑定到父对象时调用该函数修改数值（实现直接设置数值）|在父类的 “F生成光门后” 函数内调用
  (EventDispatchers|BindEventtoED绑定到父类时 (delegate Custom|ED_绑定到父类时_Event)))

(event Collision|EventActorBeginOverlap
  (params (OtherActor :type Actor%20Object%20Reference))
  (|CallParentFunction OtherActor) ; 此节点被禁用，将不会被调用。\n从引脚连出引线来编译功能。
)

(event EventTick
  (params (DeltaSeconds :type Float%20%28single-precision%29))
  (|CallParentFunction DeltaSeconds) ; 此节点被禁用，将不会被调用。\n从引脚连出引线来编译功能。
)

(event EventCE播放受击反馈
  ;[1 0 0 0.5] 父类带有整体缩放，此处不需要
  (|CallParentFunction)
  ;[0.5103 0.849 0.4156 0.5] 子类派生添加收集修改数值
  (Utilities|FlowControl|DoOnce false :!label _label
    (:Completed
      (Variables|Default|Set障碍物生命值_Cur (+ (Variables|Default|Get障碍物生命值_Cur) 1.0))
      (CallFunction|CE受击改变缩放和数值)
      ;;[0.15 0.15 0.15 0.5] 设置攻击后变化冷却时间
      (Utilities|FlowControl|Delay 0.3)
      (goto _label Reset))))

(fn ConstructionScript
  (|CallParentFunction))

(fn F受击改变缩放和数值
  (bind _output_get (Variables|Default|Set初始缩放 (CallFunction|F计算缩放与数值比例)))
  (Transformation|SetActorScale3D (Math|Conversions|ToVector(Float) _output_get)))

(fn F计算缩放与数值比例
  (return (Math|Float|Clamp(Float) (Math|Float|Lerp 0.5 1.3 (/ (Math|Float|Absolute(Float) (Variables|Default|Get障碍物生命值_Cur)) 8.0)) 0.5 1.3)))

(fn F获取并设置当前显示数值
  (bind _returnvalue (Actor|GetAttachParentActor))
  (Utilities|IsValid _returnvalue
    (:Is%20Valid
      (bind _asbp_光门阵列_细柱子加人版 (Utilities|Casting|CastToBP_光门阵列_细柱子加人版 _returnvalue)
        (:then
          (Variables|Default|Set障碍物生命值_Cur (Variables|/Game/蓝图功能库/蓝图模板/SH_Template/道具/光门/BP_光门阵列.BP_光门阵列_C|Get生成的门生命值 _asbp_光门阵列_细柱子加人版)))
        (:CastFailed
          (Variables|Default|Set障碍物生命值_Cur 2.0))))))