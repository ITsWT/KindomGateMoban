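; Light-gate array variant (thin pillar, add-people) that continuously spawns gates and moves them along SplineZ, killing each at the spline's end.
; A SpawnColdDown timeline paces spawning, its play rate set from the interval; each new gate gets a BPAC沿线移动 component.
; Add-people events boost gate speed and switch the spawn interval until a 0.35s retriggerable delay lapses.
; Without a spline, they boost the array's own BPAC沿线移动 instead.
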(event Custom|CEED-加人之后
  (params (障碍物 :type BP%20障碍物%20Base%20Object%20Reference) (死因 :type String))
  (switch string 死因
    (:Default
      (Variables|Default|GetSplineZ
        (:then
          (Utilities|FlowControl|Sequence
            (:then_0
              (Variables|Default|Set加速 true)
              (Utilities|FlowControl|DoOnce false :!label _label
                (:Completed
                  (bind _output_get (Variables|Default|Set持续生成间隔时间 (Variables|默认|持续生成|Get持续生成间隔时间_加人后)))
                  (CallFunction|F修改生成耗时 _output_get)
                  (CallFunction|F沿线速度修改 (Variables|Default|Get加速位移速度)))))
            (:then_1
              (Utilities|FlowControl|RetriggerableDelay 0.35)
              (Variables|Default|Set加速 false)
              (CallFunction|F沿线速度修改 (Variables|Default|Get沿线位移速度))
              (bind _output_get_2 (Variables|Default|Set持续生成间隔时间 (Variables|默认|持续生成|Get持续生成间隔时间_加人前)))
              (CallFunction|F修改生成耗时 _output_get_2)
              (goto _label Reset))))
        (:else
          (Variables|/Game/蓝图功能库/通用组件/BPAC_沿线移动.BPAC_沿线移动_C|Set位移速度 (Variables|Default|GetBPAC_沿线移动) (Variables|Default|Get加速位移速度))
          (Utilities|FlowControl|RetriggerableDelay 0.35)
          (Variables|/Game/蓝图功能库/通用组件/BPAC_沿线移动.BPAC_沿线移动_C|Set位移速度 (Variables|Default|GetBPAC_沿线移动) (Variables|Default|Get普通位移速度)))))))

(event EventBeginPlay
  (|CallParentFunction)
  (Variables|/Game/蓝图功能库/通用组件/BPAC_沿线移动.BPAC_沿线移动_C|Set位移速度 (Variables|Default|GetBPAC_沿线移动) (Variables|Default|Get普通位移速度))
  (bind _output_get (Variables|默认|持续生成|Set持续生成间隔时间_加人前 (Variables|Default|Get持续生成间隔时间)))
  (CallFunction|F修改生成耗时 _output_get))

(event EventTick
  (params (DeltaSeconds :type Float%20%28single-precision%29))
  (if (>= (Variables|Default|Get持续生成间隔时间) 0.0)
    (if (not (Variables|Default|Get生成colddown))
      (Variables|Default|Set生成colddown true)
      (CallFunction|CE-生成一次)
      (Variables|Default|SetLastGameTime (Utilities|Time|GetGameTimeinSeconds))
      (Timeline|SpawnColdDown PlayFromStart
        (:Finished
          (Variables|Default|Set生成colddown false)
          (Timeline|SpawnColdDown SetNewTime))))))

(fn ConstructionScript
  (|CallParentFunction))

(fn F生成光门后
  (params (New光门 :type BP%20障碍物%20光门%20Object%20Reference%20%28by%20ref%29))
  (|CallParentFunction New光门)
  (EventDispatchers|BindEventtoED-障碍物被打破时 New光门 (EventDispatchers|CreateEvent :!event Custom|CEED-加人之后))
  (Utilities|FlowControl|Sequence
    (:then_0
      (bind _splinez (Variables|Default|GetSplineZ)
        (:then
          (bind _returnvalue (AddComponent|AddBPAC沿线移动 New光门 0.0))
          (EventDispatchers|BindEventtoED-抵达终点时 _returnvalue (EventDispatchers|CreateEvent :!event FED-沿线抵达终点时))
          (Variables|/Game/蓝图功能库/通用组件/BPAC_沿线移动.BPAC_沿线移动_C|Set位移速度 _returnvalue (select (Variables|Default|Get加速) (Variables|Default|Get加速位移速度) (Variables|Default|Get沿线位移速度)))
          (Variables|/Game/蓝图功能库/通用组件/BPAC_沿线移动.BPAC_沿线移动_C|SetSplineComp _returnvalue (Variables|/Game/蓝图功能库/蓝图模板/BP_SplineZ/BP_SplineZ.BP_SplineZ_C|GetSplineZ _splinez))
          (Default|CE-Init _returnvalue)
          (Utilities|Map|Add (Variables|/Game/蓝图功能库/通用组件/BPAC_沿线移动.BPAC_沿线移动_C|Get同步旋转 _returnvalue) "NewEnumerator1" true))
        (:else)))
    (:then_1
      (return))))

(fn FED-沿线抵达终点时
  (params (拥有者 :type Actor%20Object%20Reference) (组件 :type BPAC%20沿线移动%20Object%20Reference))
  (bind _asbp_障碍物_光门 (Utilities|Casting|CastToBP_障碍物_光门 拥有者))
  (Default|CE死亡 _asbp_障碍物_光门 _asbp_障碍物_光门 "抵达终点"))

(fn F沿线速度修改
  (params (位移速度 :type Float%20%28double-precision%29))
  (for _array_element (Variables|Default|Get生成的光门_array)
    (Utilities|IsValid _array_element
      (:Is%20Valid
        (Variables|/Game/蓝图功能库/通用组件/BPAC_沿线移动.BPAC_沿线移动_C|Set位移速度 (Actor|GetComponentbyClass _array_element "/Game/蓝图功能库/通用组件/BPAC_沿线移动.BPAC_沿线移动_C") 位移速度)))))

(fn F修改生成耗时
  (params (Time :type Float%20%28double-precision%29))
  (Components|Timeline|SetPlayRate (Variables|Default|GetSpawnColdDown) (/ 1.0 Time)))