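; Base destructible obstacle that shows its health on a widget, takes damage through an interface and breaks at its death threshold.
; Damage is either a fixed amount or a percentage of incoming damage, then updates the number text.
; Rate-limited hit feedback drives timelines for model and widget scale, with optional curve override, plus a material-parameter flash.
; Death fires a dispatcher, detaches, activates VFX, disables collision, fades text, shrinks the model and sets a lifespan.
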(event Custom|CE_障碍物受击
  (params (伤害值 :type Float%20%28double-precision%29))
  (if (Variables|状态|Get障碍物已启用)
    (if (Variables|默认|生命值|Get能够受伤？)
      (bind _output_get (Variables|默认|生命值|Set障碍物生命值_Cur (数值计算|F伤害计算 伤害值)))
      (Default|CallED-生命值变化时 _output_get)
      (Utilities|FlowControl|Sequence
        (:then_0
          (Utilities|FlowControl|DoOnce false :!label _label
            (:Completed
              (CallFunction|CE播放受击反馈))))
        (:then_1
          (Utilities|FlowControl|Delay (Variables|默认|反馈动画|Get受击反馈间隔时间))
          (goto _label Reset))
        (:then_2
          (更新属性|F修改UMG文本数字 (Variables|状态|GetAs%20UMG%20文本) (Variables|默认|生命值|Get障碍物生命值_Cur) false)
          ;[0.1016 0 1] 判断死亡
          (if (or (and (<= (Variables|默认|生命值|Get障碍物生命值_Cur) 0.0) (Variables|默认|生命值|Get生命值低于零时死亡)) (> (Math|Float|Absolute(Float) (Variables|默认|生命值|Get障碍物生命值_Cur)) (Variables|默认|生命值|Get最大生命值上限_Abs)))
            (CallFunction|CE死亡 self "生命值达到死亡标准")))))))

(event Custom|CE_播放受击反馈
  (Utilities|FlowControl|Sequence
    (:then_0
      (Utilities|FlowControl|DoOnce false :!label _label
        (:Completed
          (Default|CallED-受击反馈开始时)
          (Utilities|FlowControl|Sequence
            (:then_0
              (Components|Timeline|SetPlayRate (Variables|Default|GetTL_缩放) (Variables|默认|反馈动画|Get受击反馈动画速率))
              (bind _覆盖缩放曲线 (Variables|默认|反馈动画|Get覆盖缩放曲线)
                (:then
                  (Class|TimelineComponent|SetVectorCurve (Variables|Default|GetTL_缩放) _覆盖缩放曲线 "V")
                  ;[0.05469 0 1] 可以通过蓝图修改曲线
                  (bind (_direction _f _v) (Timeline|TL_缩放 PlayFromStart)
                    (:Update
                      (Variables|状态|Set受击alphaV _v)
                      (Variables|状态|Set受击alphaF _f)
                      (反馈动画|F障碍物受击缩放))))
                (:else
                  (Timeline|TL_缩放 PlayFromStart))))
            (:then_1
              (bind _变色time (Timeline|TL_闪烁 PlayFromStart)
                (:Update
                  (更新属性|F障碍物受击闪烁 _变色time))))))))
    (:then_1
      (Utilities|FlowControl|Delay (Variables|默认|反馈动画|Get受击反馈间隔时间))
      (goto _label Reset))))

(event Custom|CE_死亡
  (params (障碍物 :type BP%20障碍物%20Base%20Object%20Reference) (死因 :type String))
  (Utilities|FlowControl|DoOnce false
    (:Completed
      (Default|CallED-障碍物被打破时 self 死因)
      (Transformation|DetachFromActor "KeepWorld" "KeepWorld" "KeepWorld")
      (Variables|状态|Set已死亡 true)
      (激活特效|F激活死亡特效)
      (Actor|SetLifeSpan 5.0)
      (Collision|SetActorEnableCollision false)
      (Default|F文本渐隐 (Variables|状态|GetAs%20UMG%20文本) 1.0)
      ;[0.5234 1 0] 缩放隐藏模型
      (bind _新建轨道_0 (Timeline|TL_消失 PlayFromStart)
        (:Update
          (Transformation|SetRelativeScale3D (Variables|Default|GetRoot_障碍物模型) (Math|Conversions|ToVector(Float) (Math|Float|Lerp 1.0 0.01 _新建轨道_0))))
        (:Finished
          (Development|SetHiddeninGame (Variables|状态|GetMeshComps) true false))))))

(event EventBeginPlay
  (Variables|状态|Set障碍物生命值_Max (Variables|默认|生命值|Get障碍物生命值_Cur))
  (Variables|状态|SetWidget初始缩放 (CallFunction|向量转浮点(平均值) (Variables|/Script/Engine.SceneComponent|GetRelativeScale3D (Variables|Default|GetWidget_文本))))
  (初始化|F初始化文本)
  (初始化|F记录网格体组件)
  (Variables|状态|SetWidget初始相对位置 (Variables|/Script/Engine.SceneComponent|GetRelativeLocation (Variables|Default|GetWidget_文本))))

(event EventTick
  (params (DeltaSeconds :type Float%20%28single-precision%29))
  ;[0 0.08594 1] 默认禁用
)

(fn ConstructionScript)

(fn F障碍物受击缩放
  (bind _受击时widget偏移程度 (Variables|默认|反馈动画|Get受击时widget偏移程度))
  (bind _widget初始相对位置 (Variables|状态|GetWidget初始相对位置))
  (Variables|默认|反馈动画|Get覆盖缩放曲线
    (:then
      (Transformation|SetRelativeScale3D (Variables|Default|GetRoot_障碍物模型) (Variables|状态|Get受击alphaV)))
    (:else
      (Transformation|SetRelativeScale3D (Variables|Default|GetRoot_障碍物模型) (Math|Conversions|ToVector(Float) (Math|Float|Lerp 1.0 (Variables|默认|反馈动画|Get受击时widget缩放大小) (Variables|状态|Get受击alphaF))))))
  (Transformation|SetRelativeScale3D (Variables|Default|GetRoot_widget) (Math|Conversions|ToVector(Float) (Math|Float|Lerp 1.0 (Variables|默认|反馈动画|Get受击时widget缩放大小) (Variables|状态|Get受击alphaF))))
  (if (!= _受击时widget偏移程度 0.0)
    (Transformation|SetRelativeLocation (Variables|Default|GetWidget_文本) (Math|Vector|Lerp(Vector) _widget初始相对位置 (+ _widget初始相对位置 (Math|Vector|MakeVector _受击时widget偏移程度 0.0 0.0)) (Variables|状态|Get受击alphaF)) false false)))

(fn F初始化文本
  (bind _widget_文本 (Variables|Default|GetWidget_文本))
  (bind _asumg_文本 (Utilities|Casting|CastToUMG_文本 (UserInterface|GetWidget _widget_文本))
    (:then
      (Variables|状态|SetAs%20UMG%20文本 _asumg_文本))
    (:CastFailed
      _))
  (Rendering|SetCastShadow _widget_文本 false)
  (更新属性|F修改UMG文本数字 (Variables|状态|GetAs%20UMG%20文本) (Variables|默认|生命值|Get障碍物生命值_Cur) false))

(fn F记录网格体组件
  ;[0 0.4609 1] 记录网格体组件
  (bind _网格体组件 (CallFunction|F获取所有网格体组件 self true true false))
  (Variables|状态|SetMeshComps _网格体组件))

(fn F激活死亡特效
  (bind _output_get (LocalVariables|Set死亡特效 (Components|GetChildrenComponents (Variables|Default|GetVFX_死亡特效) true)))
  (for _array_element _output_get
    (Components|Activation|Activate _array_element true)))

(fn F修改UMG文本数字
  (params (As%20UMG%20文本 :type UMG%20文本%20Object%20Reference) (Number :type Float%20%28double-precision%29) (反转符号 :type Boolean))
  (Default|F修改文本内容Float As%20UMG%20文本 (Math|Float|Max(Float) Number 0.0) "ToPositiveInfinity" false 反转符号 false 0 true))

(fn F障碍物受击闪烁
  (params (Alpha :type Float%20%28single-precision%29))
  (Rendering|Material|SetScalarParameterValueonMaterials (Variables|状态|GetMeshComps) "SH_闪烁Alpha" Alpha))

(fn F伤害计算
  (params (伤害值 :type Float%20%28double-precision%29))
  (bind _每次受到伤害值 (Variables|默认|生命值|Get每次受到伤害值))
  (LocalVariables|Set基础伤害 (select (!= _每次受到伤害值 0.0) _每次受到伤害值 (* 伤害值 (Variables|默认|生命值|Get受到伤害百分比))))
  (LocalVariables|Set计算后的生命值 (- (Variables|默认|生命值|Get障碍物生命值_Cur) (LocalVariables|Get基础伤害)))
  (return (LocalVariables|Get计算后的生命值)))

(fn F更换受击缩放曲线
  (params (NewVectorCurve :type Curve%20Vector%20Object%20Reference))
  (Utilities|IsValid NewVectorCurve
    (:Is%20Valid
      (Class|TimelineComponent|SetVectorCurve (Variables|Default|GetTL_缩放) NewVectorCurve "V"))))

(fn BPI-发起交互
  (params (发起者 :type Actor%20Object%20Reference) (交互类型 :type String))
  (return false ""))

(fn BPI-应用伤害-SH
  (params (伤害值 :type Float%20%28double-precision%29) (Instigator :type Pawn%20Object%20Reference) (DamageCauser :type Actor%20Object%20Reference) (伤害类型 :type String) (物理冲击 :type Vector :default "0, 0, 0") (命中结果 :type Hit%20Result%20Structure))
  (Variables|状态|SetDamage%20Causer%20Last DamageCauser)
  (CallFunction|CE障碍物受击 伤害值)
  (return true 0.0))

(fn BPI-获取当前速度
  (return false "0, 0, 0"))

(fn BPI-获取所属阵营
  (return 0))

(fn BPI-获取是否死亡
  (return false 0))