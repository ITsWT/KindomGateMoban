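; Base Blueprint for SH template firearms, handling what happens to the gun on its weapon-death event.
; On first death it either destroys itself or, with 不直接死亡 set, physics-simulates its meshes, colliding with the world and thrown by the owner's last damage impulse.
; When the owner's corpse starts sinking, the meshes ignore all collision.
; The owner's OnDestroyed handler calls DestroyActor on that destroyed owner, not on the weapon.
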(event Custom|CEED-尸体下沉时
  ;[1 0.8203 0] 尸体下沉时
  (for _array_element (Variables|Default|Get所有网格体组件)
    (Collision|SetCollisionResponsetoAllChannels _array_element "ECR_Ignore")))

(event Custom|CEED-角色销毁时
  (params (DestroyedActor :type Actor%20Object%20Reference))
  ;[0 0.6484 1] 角色销毁时
  (Actor|DestroyActor DestroyedActor))

(event EventBeginPlay
  (|CallParentFunction))

(event EventCE-武器死亡
  (bind _ref拥有者角色 (Variables|Default|GetRef拥有者角色))
  (bind _最后受到的伤害冲量 (Variables|/Game/蓝图功能库/蓝图模板/SH_Template/角色/BP_SH角色_Base.BP_SH角色_Base_C|Get最后受到的伤害冲量 _ref拥有者角色))
  (|CallParentFunction)
  (Utilities|FlowControl|DoOnce false
    (:Completed
      (if (Variables|Default|Get不直接死亡)
        ;[0 0.6953 1] 获取网格体
        (bind _网格体组件 (CallFunction|F获取所有网格体组件 self true true false))
        (Variables|Default|Set所有网格体组件 _网格体组件)
        ;[1 0.8203 0] 尸体下沉时
        (EventDispatchers|BindEventtoED-尸体开始下沉 (Variables|Default|GetRef拥有者角色) (delegate Custom|CEED-尸体下沉时))
        ;[0 0.6484 1] 角色销毁时
        (Game|AssignOnDestroyed (Variables|Default|GetRef拥有者角色) (delegate Custom|CEED-角色销毁时))
        ;[1 0.7969 0] 设置碰撞通道
        (for _array_element (Variables|Default|Get所有网格体组件)
          (Collision|SetCollisionResponsetoChannel _array_element "ECC_PhysicsBody" "ECR_Ignore")
          (Collision|SetCollisionResponsetoChannel _array_element "ECC_Pawn" "ECR_Ignore")
          (Collision|SetCollisionResponsetoChannel _array_element "ECC_Vehicle" "ECR_Ignore")
          (Collision|SetCollisionResponsetoChannel _array_element "ECC_Destructible" "ECR_Ignore")
          (Collision|SetCollisionResponsetoChannel _array_element "ECC_WorldStatic" "ECR_Block")
          (Collision|SetCollisionResponsetoChannel _array_element "ECC_WorldDynamic" "ECR_Block")
          ;[1 1 1] 设置物理速度
          (CallFunction|一键模拟物理 _array_element "PhysicsOnly" "ECC_PhysicsBody" true)
          (Physics|SetPhysicsLinearVelocity _array_element (* _最后受到的伤害冲量 0.35) false "None")
          (Class|PrimitiveComponent|SetPhysicsAngularVelocityinDegrees _array_element (* (Math|Vector|RotateVector _最后受到的伤害冲量 (Math|Rotator|MakeRotator 0.0 0.0 (CallFunction|绝对值范围内随机浮点 15.0))) 0.1) false "None"))
        (else
          (Actor|DestroyActor))))))

(event EventTick
  (params (DeltaSeconds :type Float%20%28single-precision%29))
  (|CallParentFunction DeltaSeconds) ; 此节点被禁用，将不会被调用。\n从引脚连出引线来编译功能。
)

(fn ConstructionScript
  (|CallParentFunction))