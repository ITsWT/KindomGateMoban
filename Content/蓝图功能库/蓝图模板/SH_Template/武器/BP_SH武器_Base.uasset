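; Base weapon actor for SH characters that handles firing and owner interaction, leaving most projectile behavior to the spawned class.
; Tick or interaction calls trigger an overridable attack gated by cooldown, playing montage and effects, then spawning timed bursts of multi-trajectory projectiles.
; Aim follows a selectable direction source with precise/fuzzy angle assist, using a seeded stream for spread and offsets.
; It inherits the owner's faction and shuts down when the owner dies.
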(event Custom|CE-开始生成发射物
  ;[1 0.9844 0] 开火
  (私有函数|F激活开火特效)
  ;;[0.2656 1 0] 连发
  (if (> (Variables|参数|连发设置|Get连发数量_Max) 1)
    (Utilities|ForLoopPeriodicwithDelay 0 (- (Variables|参数|连发设置|Get连发数量_Max) 1) (Variables|参数|连发设置|Get连发数量_PerDuration) (Variables|参数|连发设置|Get连发数量_PerNum) ; 连发loop
      (:Loop%20Body
        _)))
  ;;[0.3594 1 0] 多重弹道
  (if (> (Variables|参数|多弹道设置|Get弹道_数量) 1)
    (for _index (range 0 (- (Variables|参数|多弹道设置|Get弹道_数量) 1)) ; 弹道loop
      (私有函数|F生成发射物 _index))
    (else
      ;;[0.1719 0 1] 单发
      (私有函数|F生成发射物))))

(event Custom|CE_尝试开火一次
  ;[1 0.9844 0] 开火
  (if (属性获取|F武器能否开火)
    (CallFunction|CE攻击执行)
    (CallFunction|CE-使武器进入冷却)))

(event Custom|CE_开火一次%28无视条件%29
  ;[1 0.9844 0] 开火
  (CallFunction|CE攻击执行)
  (CallFunction|CE-使武器进入冷却))

(event Custom|CE_攻击执行
  ;[1 0.9844 0] 开火
  (CallFunction|F播放攻击动画蒙太奇)
  (Default|CallED-成功开火时 self)
  (Utilities|DelayNotZero (Variables|参数|发射物参数|Get发射物_生成延迟)
    (:false
      (私有函数|F激活开火特效)
      (CallFunction|CE-开始生成发射物))))

(event Custom|CE-武器死亡
  ;[0 1 0.9063] CEED-拥有者角色死亡时
  (Utilities|FlowControl|DoOnce false
    (:Completed
      (Variables|状态|Set武器能够开火 false)
      (Variables|状态|Set武器已死亡 true)
      (Components|DestroyComponent (Variables|Default|GetP_开火特效)))))

(event Custom|CE-使武器进入冷却
  ;[1 0.9844 0] 开火
  (Variables|状态|Set武器正在冷却 true)
  (Utilities|FlowControl|RetriggerableDelay (Variables|参数|基础设置|Get开火间隔时间))
  (if (not (Variables|状态|Get武器正在初始冷却)) ; 初始冷却时不能正常解除冷却
    (Variables|状态|Set武器正在冷却 false)))

(event Custom|CEED-拥有者角色死亡时
  (params (死亡的角色 :type BP%20SH角色%20Base%20Object%20Reference))
  ;[0 1 0.9063] CEED-拥有者角色死亡时
  (EventDispatchers|BindEventtoED-材质变化时 (Variables|状态|GetRef拥有者角色) (EventDispatchers|CreateEvent :!event FED-角色材质变化时)) ; 角色材质变化时
  (CallFunction|CE-武器死亡))

(event Custom|CE-刷新初始冷却
  ;[1 0.7969 0] 刷新初始冷却
  (Variables|状态|Set武器正在冷却 true)
  (Variables|状态|Set武器正在初始冷却 true)
  ;[1 1 1] 获取网格体组件
  (bind _网格体组件 (CallFunction|F获取所有网格体组件 self true true false))
  (Variables|状态|Set有效网格体组件 _网格体组件)
  ;[1 0 0.3984] 初始冷却状态
  (Utilities|DelayNotZero (+ (Variables|参数|基础设置|Get初始冷却时长) (CallFunction|流送中绝对值范围内随机浮点 (Variables|参数|基础设置|Get初始冷却时长_Offset) (Variables|状态|Get武器seed)))
    (:false
      (Variables|状态|Set武器正在冷却 false)
      (Variables|状态|Set武器正在初始冷却 false))))

(event EventBeginPlay
  ;[1 0.2109 0] BeignPlay
  (Development|SetHiddeninGame (Variables|Default|GetArrow_武器朝向) true false)
  ;;[0 1 0.6953] 初始寻找拥有者角色
  (Utilities|IsValid (Variables|状态|GetRef拥有者角色)
    (:Is%20Valid
      _)
    (:Is%20Not%20Valid
      (bind _asbp_sh角色_base (Utilities|Casting|CastToBP_SH角色_Base (Actor|GetAttachParentActor))
        (:then
          (CallFunction|F设置武器拥有者 _asbp_sh角色_base))
        (:CastFailed
          _))))
  ;[1 0.7969 0] 刷新初始冷却
  (Variables|状态|Set武器正在冷却 true)
  (Variables|状态|Set武器正在初始冷却 true)
  ;[1 1 1] 获取网格体组件
  (bind _网格体组件 (CallFunction|F获取所有网格体组件 self true true false))
  (Variables|状态|Set有效网格体组件 _网格体组件)
  ;[1 0 0.3984] 初始冷却状态
  (Utilities|DelayNotZero (+ (Variables|参数|基础设置|Get初始冷却时长) (CallFunction|流送中绝对值范围内随机浮点 (Variables|参数|基础设置|Get初始冷却时长_Offset) (Variables|状态|Get武器seed)))
    (:false
      (Variables|状态|Set武器正在冷却 false)
      (Variables|状态|Set武器正在初始冷却 false))))

(event EventTick
  (params (DeltaSeconds :type Float%20%28single-precision%29))
  ;[1 0.9844 0] 开火
  (|CallParentFunction DeltaSeconds)
  (私有函数|F同步拥有者隐藏)
  (if (or (Variables|参数|基础设置|Get按下扳机) (Variables|参数|其他设置|Get武器独立扳机))
    (CallFunction|CE尝试开火一次)))

(fn ConstructionScript)

(fn F计算弹道基础朝向
  (bind _returnvalue (Components|GetOwner))
  (bind _ref拥有者角色 (Variables|状态|GetRef拥有者角色))
  (bind _角色期望朝向 (Variables|/Game/蓝图功能库/蓝图模板/SH_Template/角色/BP_SH角色_Base.BP_SH角色_Base_C|Get角色期望朝向 _ref拥有者角色))
  (Utilities|FlowControl|Sequence
    (:then_0
      ;[0.007812 0 1] 基础朝向归类
      (switch Utilities|FlowControl|Switch|SwitchonE武器瞄准方向 (Variables|参数|射击方向|GetE武器瞄准方向)
        (:NewEnumerator6
          ;;[0.9922 1 0] 朝向角色当前的攻击目标角色
          (Utilities|IsValid (Variables|状态|GetRef拥有者角色)
            (:Is%20Valid
              (Utilities|IsValid (Variables|/Game/蓝图功能库/蓝图模板/SH_Template/角色/BP_SH角色_Base.BP_SH角色_Base_C|Get当前攻击目标角色 (Variables|状态|GetRef拥有者角色))
                (:Is%20Valid
                  (Variables|状态|Set射击期望方向 (Math|Rotator|FindLookatRotation (Transformation|GetWorldLocation (Variables|Default|GetArrow_武器朝向)) (Transformation|GetActorLocation (Variables|/Game/蓝图功能库/蓝图模板/SH_Template/角色/BP_SH角色_Base.BP_SH角色_Base_C|Get当前攻击目标角色 (Variables|状态|GetRef拥有者角色))))))
                (:Is%20Not%20Valid
                  (CallFunction|F-DebugMSG " 计算基础朝向失败" "(R=1.000000,G=0.613698,B=0.000000,A=1.000000)" 2.0 :!label _label))))
            (:Is%20Not%20Valid
              (goto _label))))
        (:NewEnumerator2
          ;;[0.6172 1 0] 朝向角色的期望朝向
          (Utilities|IsValid _ref拥有者角色
            (:Is%20Valid
              (if (Utilities|Operators|NotEqual(!=) _角色期望朝向 "-1.000000,-1.000000,-1.000000" 0.0)
                (Variables|状态|Set射击期望方向 _角色期望朝向)
                (else
                  (CallFunction|F-DebugMSG " 计算基础朝向失败" "(R=1.000000,G=0.613698,B=0.000000,A=1.000000)" 2.0 :!label _label_2))))
            (:Is%20Not%20Valid
              (goto _label_2))))
        (:NewEnumerator0
          ;;[0.4766 1 0] 使用拥有者的朝向
          (Utilities|IsValid _returnvalue
            (:Is%20Valid
              (Variables|状态|Set射击期望方向 (Transformation|GetActorRotation _returnvalue)))
            (:Is%20Not%20Valid
              (CallFunction|F-DebugMSG " 计算基础朝向失败" "(R=1.000000,G=0.613698,B=0.000000,A=1.000000)" 2.0))))
        (:NewEnumerator5
          ;;[0 1 0.8359] 使用自身的朝向
          (Variables|状态|Set射击期望方向 (Transformation|GetWorldRotation (Variables|Default|GetArrow_武器朝向))))
        (:NewEnumerator8
          ;;[1 0 0.9844] 使用武器期望朝向
          (if (Utilities|Operators|NotEqual(!=) (Variables|状态|Get射击期望方向) "-1.000000,-1.000000,-1.000000" 0.0)
            (Variables|状态|Set射击期望方向 (Variables|状态|Get射击期望方向))
            (else
              (CallFunction|F-DebugMSG " 计算基础朝向失败" "(R=1.000000,G=0.613698,B=0.000000,A=1.000000)" 2.0))))))
    (:then_1
      (LocalVariables|Setlp_Rotation (私有函数|F计算精确射击朝向 (Variables|状态|Get射击期望方向)))
      (if (Variables|参数|射击方向|Get解锁武器Yaw旋转)
        (return (LocalVariables|Getlp_Rotation))
        (else
          (return (.OnlyZ%28Yaw%29 (CallFunction|旋转体Z轴 (LocalVariables|Getlp_Rotation)))))))))

(fn F计算弹道方向偏移
  (params (Index :type Integer) (基础朝向 :type Rotator))
  (bind _弹道_间隔角度 (Variables|参数|多弹道设置|Get弹道_间隔角度))
  (return (Math|Rotator|CombineRotators 基础朝向 (Math|Rotator|MakeRotator 0.0 0.0 (+ (+ (* Index _弹道_间隔角度) (* _弹道_间隔角度 (- (Variables|参数|多弹道设置|Get弹道_数量) 1) -0.5)) (CallFunction|流送中绝对值范围内随机浮点 (Variables|参数|其他设置|Get弹道随机扩散角度) (Variables|状态|Get武器seed)))))))

(fn F计算弹道位置偏移
  (return (* (Math|Vector|GetRightVector (Variables|Default|GetArrow_武器朝向)) (* (- (Variables|参数|多弹道设置|Get弹道_数量) 1) (Variables|参数|多弹道设置|Get弹道_间隔距离) -0.5))))

(fn F计算发射物生成位置
  (params (Index :type Integer))
  (return (+ (Transformation|GetWorldLocation (Variables|Default|GetRoot_开火特效)) (+ (* (Math|Vector|GetForwardVector (Variables|Default|GetArrow_武器朝向)) (+ (Variables|参数|发射物参数|Get发射物_生成位置向前偏移) (CallFunction|流送中绝对值范围内随机浮点 (Variables|参数|发射物参数|Get发射物_生成位置向前偏移_Offset) (Variables|状态|Get武器seed)))) (* (Math|Vector|GetRightVector (Variables|Default|GetArrow_武器朝向)) (CallFunction|流送中绝对值范围内随机浮点 (Variables|参数|发射物参数|Get发射物_生成位置向右偏移_Offset) (Variables|状态|Get武器seed)))) (+ (* Index (Variables|参数|多弹道设置|Get弹道_间隔距离) (Class|KismetMathLibrary|VectorNormal2D (Math|Vector|GetRightVector (Variables|Default|GetArrow_武器朝向)) 0.0001)) (私有函数|F计算弹道位置偏移)))))

(fn F计算精确射击朝向
  (params (基础朝向 :type Rotator))
  (if (or (>= (Variables|参数|射击方向|Get精确射击角度) 0.0) (>= (Variables|参数|射击方向|Get模糊射击角度) 0.0))
    ;[0 1 0.7422] 是否满足精确射击角度
    (bind (_夹角度数 _已瞄准) (CallFunction|F判断是否成功瞄准 (Math|Rotator|GetRotationXVector (Transformation|GetWorldRotation (Variables|Default|GetArrow_武器朝向))) (Math|Rotator|GetRotationXVector (Variables|状态|Get射击期望方向)) (not (Variables|参数|射击方向|Get解锁武器Yaw旋转)) (Variables|参数|射击方向|Get精确射击角度)))
    (LocalVariables|Set当前夹角 _夹角度数)
    (if _已瞄准
      ;[1 0 0.3984] 直接进行精确射击
      (return (Variables|状态|Get射击期望方向))
      (else
        _)))
  ;[0.6875 1 0] 是否满足模糊射击？
  (if (< (LocalVariables|Get当前夹角) (Variables|参数|射击方向|Get模糊射击角度))
    ;[0.5469 1 0] 模糊射击
    (return (Math|Rotator|Lerp(Rotator) (Variables|状态|Get射击期望方向) (Transformation|GetWorldRotation (Variables|Default|GetArrow_武器朝向)) (Math|Float|Power (Math|Float|MapRangeClamped (LocalVariables|Get当前夹角) 0.0 (Variables|参数|射击方向|Get模糊射击角度) 0.0 1.0) 2.5) true))
    (else
      ;[0.3828 0 1] 条件不满足，使用基础朝向
      (return 基础朝向))))

(fn F生成发射物
  (params (Index :type Integer))
  (if (Utilities|IsValidClass (Variables|参数|基础设置|Get发射物类型))
    ;[1 0.3984 0] 原始的基础朝向，基于此方向进行偏移计算
    (LocalVariables|Setlp_基础朝向 (私有函数|F计算弹道基础朝向))
    (bind _returnvalue (Game|SpawnActorfromClass (Variables|参数|基础设置|Get发射物类型) (Math|Transform|MakeTransform (+ (私有函数|F计算发射物生成位置 Index) "") (私有函数|F计算弹道方向偏移 Index (LocalVariables|Getlp_基础朝向)) (Math|Conversions|ToVector(Float) (Variables|参数|发射物参数|Get发射物_缩放倍率))) "AlwaysSpawn" "MultiplyWithRoot" self (Variables|状态|Get武器所属阵营) (CallFunction|流送中的随机流送 (Variables|状态|Get武器seed)) (Variables|状态|Get覆盖发射物速度) (Variables|参数|发射物参数|Get发射物_速度倍率) (Variables|参数|发射物参数|Get发射物_伤害值_Overload) (Variables|参数|发射物参数|Get发射物_生命周期%20Override) (Variables|状态|Get射击期望位置) (Variables|参数|发射物参数|Get发射物_溅射范围%20Override) (Variables|Actor|GetInstigator)))
    (LocalVariables|Setlp_生成的发射物 _returnvalue)
    (Utilities|IsValid (LocalVariables|Getlp_生成的发射物)
      (:Is%20Valid
        (Default|CallED-生成发射物时 self (LocalVariables|Getlp_生成的发射物))
        (return (LocalVariables|Getlp_生成的发射物)))
      (:Is%20Not%20Valid
        (return 0)))
    (else
      (return 0))))

(fn F激活开火特效
  (bind _开火特效时间膨胀 (Variables|参数|其他设置|Get开火特效时间膨胀))
  ;[0 1 0.6953] 获取附加的组件
  (bind _output_get (LocalVariables|SetchildComs (Components|GetChildrenComponents (Variables|Default|GetRoot_开火特效) true)))
  (for _array_element _output_get
    ;[0.3594 1 0] Cast 粒子
    (bind _asniagara_particle_system_component (Utilities|Casting|CastToNiagaraComponent _array_element)
      (:then
        ;[0.5469 1 0] 更新时间膨胀
        (Class|NiagaraComponent|SetCustomTimeDilation _asniagara_particle_system_component _开火特效时间膨胀))
      (:CastFailed
        (bind _ascascade_particle_system_component (Utilities|Casting|CastToParticleSystemComponent _array_element))
        (Variables|/Script/Engine.ParticleSystemComponent|SetCustomTimeDilation _ascascade_particle_system_component _开火特效时间膨胀)))
    ;[0 0.1562 1] 激活
    (Components|Activation|Activate _array_element true)))

(fn F设置武器拥有者
  (params (武器拥有者 :type BP%20SH角色%20Base%20Object%20Reference))
  (Utilities|IsValid 武器拥有者
    (:Is%20Valid
      (bind _output_get (Variables|状态|SetRef拥有者角色 武器拥有者))
      (CallFunction|F装备到角色并附加 _output_get)
      (Actor|SetOwner (Variables|状态|GetRef拥有者角色))
      (bind _阵营 (Default|BPI-获取所属阵营 (Variables|状态|GetRef拥有者角色)))
      (Variables|状态|Set武器所属阵营 _阵营)
      (EventDispatchers|BindEventtoED-角色死亡时 (Variables|状态|GetRef拥有者角色) (EventDispatchers|CreateEvent :!event Custom|CEED-拥有者角色死亡时)) ; 角色死亡后禁用武器
      (return true))
    (:Is%20Not%20Valid
      (return false))))

(fn F装备到角色并附加
  (params (角色 :type BP%20SH角色%20Base%20Object%20Reference))
  (Utilities|IsValid (Variables|状态|GetRef拥有者角色)
    (:Is%20Valid
      (EventDispatchers|BindEventtoED-角色死亡时 (Variables|状态|GetRef拥有者角色) (EventDispatchers|CreateEvent :!event Custom|CEED-拥有者角色死亡时)) ; 角色死亡后禁用武器
      (Utilities|Array|AddUnique (Variables|/Game/蓝图功能库/蓝图模板/SH_Template/角色/BP_SH角色_Base.BP_SH角色_Base_C|Get已装备的武器 (Variables|状态|GetRef拥有者角色)) self :!label _label)
      (Transformation|AttachActorToActor self (Variables|状态|GetRef拥有者角色) "RightHandSocket" "KeepWorld" "KeepWorld" "KeepWorld" true))
    (:Is%20Not%20Valid
      (bind _设置成功 (CallFunction|F设置武器拥有者 角色))
      (if _设置成功
        (goto _label)))))

(fn F修改弹道设置
  (params (弹道_数量 :type Integer) (弹道_间隔距离 :type Float%20%28double-precision%29) (弹道_间隔角度 :type Float%20%28double-precision%29))
  (Variables|参数|多弹道设置|Set弹道_数量 弹道_数量)
  (Variables|参数|多弹道设置|Set弹道_间隔距离 弹道_间隔距离)
  (Variables|参数|多弹道设置|Set弹道_间隔角度 弹道_间隔角度))

(fn F修改连发设置
  (params (连发数量_Max :type Integer) (连发数量_PerNum :type Integer) (连发数量_PerDuration :type Float%20%28double-precision%29))
  (Variables|参数|连发设置|Set连发数量_Max 连发数量_Max)
  (Variables|参数|连发设置|Set连发数量_PerNum 连发数量_PerNum)
  (Variables|参数|连发设置|Set连发数量_PerDuration 连发数量_PerDuration))

(fn F修改开火特效
  (params (粒子特效 :type F粒子特效%20Structure) (NewTransform :type Transform%20%28by%20ref%29))
  (bind (_niagara _cascade) (Utilities|Struct|BreakF粒子特效 粒子特效))
  (bind _n_开火特效 (Variables|Default|GetN_开火特效))
  (bind _p_开火特效 (Variables|Default|GetP_开火特效))
  (Utilities|FlowControl|Sequence
    (:then_0
      (Class|NiagaraComponent|SetAsset _n_开火特效 _niagara true)
      (Transformation|SetRelativeTransform _n_开火特效 NewTransform false false))
    (:then_1
      (Effects|Components|ParticleSystem|SetTemplate _p_开火特效 _cascade)
      (Transformation|SetRelativeTransform _p_开火特效 NewTransform false false))))

(fn F武器能否开火
  (return (Math|Boolean|ANDBoolean (Variables|状态|Get武器能够开火) (not (Variables|状态|Get武器正在冷却)) (not (Variables|状态|Get武器已死亡)) (or (not (Variables|Rendering|GetbHidden)) (Variables|参数|其他设置|Get武器隐藏时能够开火)))))

(fn F武器去色
  (bind _网格体组件 (CallFunction|F获取所有网格体组件 self true true false))
  (for _array_element _网格体组件
    (Rendering|Material|SetOverlayMaterial _array_element 0 :!class /Script/Engine.MeshComponent)))

(fn F获取子弹属性
  (bind _发射物类型 (Variables|参数|基础设置|Get发射物类型))
  (bind (_发射物伤害值 _发射物伤害值偏移百分比 _发射物飞行速度 _范围检测类型 _范围伤害时生成额外特效 _发射物生命周期) (Utilities|GetClassDefaults _发射物类型))
  (if (Utilities|IsValidClass _发射物类型)
    (return _发射物伤害值 _发射物飞行速度 _发射物生命周期)
    (else
      (return -1.0 -1.0 -1.0))))

(fn FED-角色材质变化时
  (params (ParameterName :type Name) (ParmeterValue :type Float%20%28double-precision%29) (TimelineAlpha :type Float%20%28double-precision%29))
  (Rendering|Material|SetScalarParameterValueonMaterials (Variables|状态|Get有效网格体组件) ParameterName ParmeterValue))

(fn F显示瞄准线
  (params (show :type Boolean))
  (bind (_发射物伤害值 _发射物飞行速度 _发射物生命周期) (属性获取|F获取子弹属性))
  (bind _output_get (Variables|状态|Set显示瞄准线 show))
  (if _output_get
    (Development|SetHiddeninGame (Variables|Default|GetArrow_瞄准线) (not (Variables|状态|Get显示瞄准线)) false)
    (Variables|/Script/Engine.ArrowComponent|SetArrowLength (Variables|Default|GetArrow_瞄准线) (/ (* _发射物飞行速度 _发射物生命周期) (Variables|/Script/Engine.ArrowComponent|GetArrowSize (Variables|Default|GetArrow_瞄准线))))))

(fn F同步拥有者隐藏
  (bind _ref拥有者角色 (Variables|状态|GetRef拥有者角色))
  (if (Variables|参数|其他设置|Get同步拥有者隐藏)
    (Utilities|IsValid _ref拥有者角色
      (:Is%20Valid
        (Rendering|SetActorHiddenInGame (Variables|/Script/Engine.Actor|GetbHidden _ref拥有者角色))))))

(fn F播放攻击动画蒙太奇
  (if (Variables|参数|其他设置|Get开火时播放蒙太奇)
    (if (Utilities|Array|IsNotEmpty (Variables|参数|其他设置|Get攻击动画蒙太奇))
      (Variables|状态|GetRef拥有者角色
        (:then
          (Animation|PlayAnimMontage (Variables|状态|GetRef拥有者角色) (.OutItem (Utilities|Array|RandomFromStream (Variables|参数|其他设置|Get攻击动画蒙太奇) (Variables|状态|Get武器seed))) 1.0 "None"))
        (:else)))))

(fn F直接附加
  (bind _附加到插槽name (Variables|参数|其他设置|Get附加到插槽Name))
  (bind _asbp_sh角色_base (Utilities|Casting|CastToBP_SH角色_Base (Actor|GetAttachParentActor)))
  (if (Transformation|DoesSocketExist (Variables|/Script/Engine.Character|GetMesh _asbp_sh角色_base) _附加到插槽name)
    (Transformation|AttachComponentToComponent (Variables|/Script/Engine.Character|GetMesh _asbp_sh角色_base) _附加到插槽name "SnapToTarget" "SnapToTarget" "SnapToTarget" true)))

(fn F-DebugMSG
  (params (内容 :type String) (TextColor :type Linear%20Color%20Structure :default "(R=0.000000,G=0.357402,B=1.000000,A=1.000000)") (Duration :type Float%20%28single-precision%29))
  (Development|PrintString (Utilities|String|Append (Utilities|GetDisplayName self) 内容) true true TextColor Duration (Utilities|String|StringToName 内容)))

(fn BPI-发起交互
  (params (发起者 :type Actor%20Object%20Reference) (交互类型 :type String))
  (switch string 交互类型
    (:Default
      (return false "无效交互"))
    (:开火
      (CallFunction|CE尝试开火一次))
    (:无冷却开火
      (CallFunction|CE开火一次(无视条件))))
  (return true "开火成功"))

(fn BPI-应用伤害-SH
  (params (伤害值 :type Float%20%28double-precision%29) (Instigator :type Pawn%20Object%20Reference) (DamageCauser :type Actor%20Object%20Reference) (伤害类型 :type String) (物理冲击 :type Vector :default "0, 0, 0") (命中结果 :type Hit%20Result%20Structure))
  (return false 0.0))

(fn BPI-获取当前速度
  (bind _returnvalue (Components|GetOwner))
  (Utilities|IsValid _returnvalue
    (:Is%20Valid
      (bind (_获取成功 _runtimevelocity) (Class|BPISH交互接口|BPI-获取当前速度(Message) _returnvalue))
      (return _获取成功 _runtimevelocity))
    (:Is%20Not%20Valid
      (return false "0, 0, 0"))))

(fn BPI-获取所属阵营
  (return (Variables|状态|Get武器所属阵营)))

(fn BPI-获取是否死亡
  (return false 0))