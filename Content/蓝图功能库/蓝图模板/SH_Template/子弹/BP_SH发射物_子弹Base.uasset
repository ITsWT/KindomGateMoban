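; Base bullet projectile Blueprint that plays a firing sound through the BP_音效控制 actor on BeginPlay and customizes hit-effect spawning.
; When enabled for weapon-fired hits on characters, F生成命中特效 applies scalar material parameters from a map to the character's meshes.
; It places particles at the struck bone, pushed toward the weapon by capsule radius at bullet height to avoid clipping.
; Otherwise, particles spawn at the supplied location with random yaw.
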(event EventBeginPlay
  (|CallParentFunction)
  ;[0.15 0.15 0.15 0.5] 使用音效控制播放音效
  (bind _returnvalue (Actor|GetActorOfClass "/Game/蓝图功能库/蓝图模板/SH_Template/角色/玩家控制器/BP_音效控制.BP_音效控制_C"))
  (Variables|Default|SetBP_音效控制 _returnvalue)
  (Default|CE生成发射物 (Variables|Default|GetBP_音效控制) (Variables|Default|GetEunm_开枪音效选择)))

(event Collision|EventActorBeginOverlap
  (params (OtherActor :type Actor%20Object%20Reference)))

(event EventDestroyed)

(fn ConstructionScript
  (|CallParentFunction))

(fn F生成命中特效
  (params (粒子 :type F粒子特效%20Structure) (Spawn%20Location :type Vector :default "0, 0, 0") (Spawn%20Scale :type Float%20%28double-precision%29) (附加到组件 :type Primitive%20Component%20Object%20Reference%20%28by%20ref%29) (附加的插槽 :type Name :default "None") (附加类型 :type EAttachLocation%20Enum :default "KeepRelativeOffset") (自定义时间膨胀 :type Float%20%28single-precision%29))
  (LocalVariables|Set网格体_lp 附加到组件)
  (LocalVariables|Set附加_lp 附加的插槽)
  ;[0 0.7891 1] 是否为武器发射
  (Utilities|IsValid (Variables|Default|GetAs%20BP%20SH武器%20Base)
    (:Is%20Valid
      (if (Variables|参数|命中特效|Get命中角色后附加特效)
        ;[0.1016 0 1] 命中了角色？
        (bind _asbp_sh角色_base (Utilities|Casting|CastToBP_SH角色_Base (Variables|Default|Get最后伤害的Actor))
          (:then
            (bind _output_get (LocalVariables|Set角色 _asbp_sh角色_base))
            (CallFunction|F修改角色材质参数F _output_get)
            ;[1 0.7969 0] 获取网格体和插槽
            (LocalVariables|Set网格体_lp (Variables|/Script/Engine.Character|GetMesh (LocalVariables|Get角色)))
            (bind _validsoket (CallFunction|F插槽在网格体中有效 (Variables|/Script/Engine.Character|GetMesh (LocalVariables|Get角色)) (Variables|/Game/蓝图功能库/蓝图模板/SH_Template/角色/BP_SH角色_Base.BP_SH角色_Base_C|Get被冲击的骨骼 (LocalVariables|Get角色))))
            (LocalVariables|Set附加_lp _validsoket)
            ;[0.4062 0 1] 生成粒子并附加到角色
            (bind (_returnniagara _returncascade) (CallFunction|F生成粒子特效 (Math|Transform|MakeTransform (CallFunction|向量合并XYZ轴 (+ (* (CallFunction|单元方向2D (Transformation|GetSocketLocation (LocalVariables|Get网格体_lp) (LocalVariables|Get附加_lp)) (Transformation|GetWorldLocation (Variables|/Game/蓝图功能库/蓝图模板/SH_Template/武器/BP_SH武器_Base.BP_SH武器_Base_C|GetArrow_武器朝向 (Variables|Default|GetAs%20BP%20SH武器%20Base)))) (Components|Capsule|GetScaledCapsuleRadius (Variables|/Script/Engine.Character|GetCapsuleComponent (LocalVariables|Get角色)))) (Transformation|GetSocketLocation (LocalVariables|Get网格体_lp) (LocalVariables|Get附加_lp))) (Transformation|GetActorLocation)) "0, 0, 0" (Math|Conversions|ToVector(Float) Spawn%20Scale)) 粒子 0 (LocalVariables|Get附加_lp) 附加类型 true true false))
            (return _returnniagara _returncascade))
          (:CastFailed
            _))))
    (:Is%20Not%20Valid
      _))
  ;[0 0.2969 1] 普通生成
  (bind (_returnniagara_2 _returncascade_2) (CallFunction|F生成粒子特效 (Math|Transform|MakeTransform Spawn%20Location (.OnlyZ%28Yaw%29 (CallFunction|旋转体Z轴 (Math|Random|RandomRotator false))) (Math|Conversions|ToVector(Float) Spawn%20Scale)) 粒子 (LocalVariables|Get网格体_lp) (LocalVariables|Get附加_lp) 附加类型 true true false))
  (return _returnniagara_2 _returncascade_2))

(fn F修改角色材质参数F
  (params (角色 :type BP%20SH角色%20Base%20Object%20Reference))
  (Utilities|IsValid 角色
    (:Is%20Valid
      (bind _网格体组件 (CallFunction|F获取所有网格体组件 角色 true true false))
      (LocalVariables|Setmesh _网格体组件)
      (bind _keys (Utilities|Map|Keys (Variables|参数|额外参数|Get修改角色材质参数F)))
      (for _array_element _keys
        (if (.ReturnValue (Utilities|Map|Find (Variables|参数|额外参数|Get修改角色材质参数F) _array_element))
          (Rendering|Material|SetScalarParameterValueonMaterials (LocalVariables|Getmesh) _array_element (.Value (Utilities|Map|Find (Variables|参数|额外参数|Get修改角色材质参数F) _array_element))))))))