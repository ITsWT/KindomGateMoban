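; Soldier character for the parkour shooter template that is recruited into a squad gathered around a rally point (集中点).
; On BeginPlay it spawns a BP_物理移动 actor to take over movement, registering with the rally point if already joined.
; Unjoined soldiers move toward the point and join on capsule contact with a joined soldier.
; Joined soldiers turn toward the focus-fire position or point's facing, holding the weapon trigger once aligned.
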(event OnComponentHit(CapsuleComponent)
  (params (HitComponent :type Primitive%20Component%20Object%20Reference) (OtherActor :type Actor%20Object%20Reference) (OtherComp :type Primitive%20Component%20Object%20Reference) (NormalImpulse :type Vector :default "0, 0, 0") (Hit :type Hit%20Result%20Structure%20%28by%20ref%29))
  (bind _ref集中点 (Variables|Default|GetRef集中点))
  ;[0.8984 0 1] 加入集中点
  (bind _asbp_sh角色_士兵_孤勇者 (Utilities|Casting|CastToBP_SH角色_士兵_孤勇者 OtherActor))
  (if (and (Variables|Default|Get已加入集中点 _asbp_sh角色_士兵_孤勇者) (not (Variables|Default|Get已加入集中点)))
    (Utilities|IsValid _ref集中点
      (:Is%20Valid
        (Utilities|FlowControl|DoOnce false
          (:Completed
            (Default|F成功加入角色 _ref集中点 self)
            (Utilities|FlowControl|Delay 0.033333)
            (Variables|Default|Set已加入集中点 true)))))))

(event EventBeginPlay
  (bind _capsulecomponent (Variables|Default|GetCapsuleComponent))
  (bind (_outradius _outhalfheight) (Class|CapsuleComponent|GetUnscaledCapsuleSize _capsulecomponent))
  (|CallParentFunction)
  ;[1 0 0.9844] 脱离附加，防bug
  (Transformation|DetachFromActor "KeepWorld" "KeepWorld" "KeepWorld")
  ;[1 0.8906 0] 生成物理移动来接管角色移动
  (bind _returnvalue (Game|SpawnActorfromClass :Class "/Game/蓝图功能库/蓝图模板/SH_Template/角色/集中点/BP_物理移动.BP_物理移动_C" :SpawnTransform (Transformation|GetActorTransform) :CollisionHandlingOverride "AlwaysSpawn" :TransformScaleMethod "MultiplyWithRoot" :胶囊体_半径 _outradius :胶囊体_半高 _outhalfheight :Ref集中点 0 :Ref附加者角色 self :约束模式 "Default" :聚拢速度 (Variables|/Script/Engine.CharacterMovementComponent|GetMaxWalkSpeed (Variables|Character|GetCharacterMovement)) :初始线性阻尼 4.0 :Instigator 0))
  (Variables|Default|SetRef物理移动 _returnvalue)
  ;[1 0.2344 0] 初始已加入集中点？
  (Utilities|IsValid (Variables|Default|GetRef集中点)
    (:Is%20Valid
      (if (Variables|Default|Get已加入集中点)
        (CallFunction|F尝试切换主武器 (Variables|/Game/蓝图功能库/蓝图模板/SH_Template/角色/集中点/BP_集中点.BP_集中点_C|Get当前武器 (Variables|Default|GetRef集中点)) true)
        (Variables|/Game/蓝图功能库/蓝图模板/SH_Template/角色/集中点/BP_物理移动.BP_物理移动_C|SetRef集中点 (Variables|Default|GetRef物理移动) (Variables|Default|GetRef集中点))
        (Utilities|Array|Add (Variables|/Game/蓝图功能库/蓝图模板/SH_Template/角色/集中点/BP_集中点.BP_集中点_C|Get集中的Actor数组 (Variables|Default|GetRef集中点)) (Variables|Default|GetRef物理移动))
        (bind _output_get (Variables|Default|Set无敌状态 false))
        (Default|CallED-无敌状态变更时 _output_get)
        (Utilities|Array|Add (Variables|/Game/蓝图功能库/蓝图模板/SH_Template/角色/集中点/BP_集中点.BP_集中点_C|Get集中的角色数组 (Variables|Default|GetRef集中点)) self)
        (Variables|Default|Set已加入集中点 true)))))

(event EventTick
  (params (DeltaSeconds :type Float%20%28single-precision%29))
  (bind _returnvalue (Transformation|GetActorLocation))
  (bind _已装备的武器 (Variables|Default|Get已装备的武器))
  (bind _ref集中点 (Variables|Default|GetRef集中点))
  (bind _ref集中点_2 (Variables|Default|GetRef集中点))
  (bind _returnvalue_2 (Transformation|GetActorLocation _ref集中点_2))
  (bind _output (Utilities|Array|Get(acopy) _已装备的武器))
  (bind _方向 (CallFunction|单元方向2D _returnvalue _returnvalue_2))
  ;[1 0.9375 0] tick
  (|CallParentFunction DeltaSeconds)
  ;[0.007812 1 0] 朝向前方旋转 或 移动
  (Utilities|IsValid (Variables|Default|GetRef集中点)
    (:Is%20Valid
      (if (Variables|Default|Get已加入集中点)
        (bind _output_get (Variables|状态|实时计算速度|Set当前目标旋转 (select (Variables|/Game/蓝图功能库/蓝图模板/SH_Template/角色/集中点/BP_集中点.BP_集中点_C|Get启用集火模式 (Variables|Default|GetRef集中点)) (.OnlyZ%28Yaw%29 (CallFunction|旋转体Z轴 (Math|Rotator|FindLookatRotation (Transformation|GetActorLocation) (Variables|/Game/蓝图功能库/蓝图模板/SH_Template/角色/集中点/BP_集中点.BP_集中点_C|Get当前集火位置 _ref集中点)))) (Transformation|GetActorRotation _ref集中点))))
        (CallFunction|F将Actor转向目标偏移 self 0 (.yaw (Variables|/Script/Engine.CharacterMovementComponent|GetRotationRate (Variables|Character|GetCharacterMovement))) (Transformation|GetActorRotation) _output_get)
        ;[0 1 1] 控制武器扳机
        (Utilities|IsValid _output
          (:Is%20Valid
            (Variables|/Game/蓝图功能库/蓝图模板/SH_Template/武器/BP_SH武器_Base.BP_SH武器_Base_C|Set按下扳机 _output (<= (Math|Float|Absolute(Float) (.yaw (Math|Rotator|Delta(Rotator) (Variables|状态|实时计算速度|Get当前目标旋转) (Transformation|GetActorRotation)))) 5.0))))
        (else
          ;[0 1 0.25] 向集中点移动 并朝向集中点
          (Pawn|Input|AddMovementInput _方向 1.0 false)
          (CallFunction|F将Actor转向目标插值 self 0 1e+01 (Transformation|GetActorRotation) (Math|Conversions|RotationFromXVector _方向) false))))))

(fn ConstructionScript
  (|CallParentFunction))

(fn F切换主武器Override
  (params (新的主武器 :type String))
  (switch string 新的主武器))