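; Child Blueprint of a hat-wearing male soldier character that overrides main-weapon switching.
; Each supported weapon (AK47, StarCraft-style Gatling, pistol) is created and equipped immediately.
; AK47 and Gatling also resize the capsule through the physics-movement component and scale its gather, rotation and spawn-force ranges by the radius ratio.
; Both then launch the character away from the gather point, with speed clamped from the group's size.
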(event EventBeginPlay
  (|CallParentFunction) ; This node is disabled and will not be called.\nDrag off pins to build functionality.
)

(event Collision|EventActorBeginOverlap
  (params (OtherActor :type Actor%20Object%20Reference)))

(event EventTick
  (params (DeltaSeconds :type Float%20%28single-precision%29))
  (|CallParentFunction DeltaSeconds) ; This node is disabled and will not be called.\nDrag off pins to build functionality.
)

(fn ConstructionScript
  (|CallParentFunction))

(fn F切换主武器Override
  (params (新的主武器 :type String))
  (bind _returnvalue (/ 6e+01 34.0))
  (bind _returnvalue_2 (/ 34.0 34.0))
  (bind _ref物理移动 (Variables|Default|GetRef物理移动))
  (bind _ref物理移动_2 (Variables|Default|GetRef物理移动))
  (bind _ref物理移动_3 (Variables|Default|GetRef物理移动))
  (bind _ref物理移动_4 (Variables|Default|GetRef物理移动))
  (bind _ref物理移动_5 (Variables|Default|GetRef物理移动))
  (switch string 新的主武器
    (:AK47
      ;[1 0 0 0.8] 帽子男：AK47
      (CallFunction|F创建武器并装备 "/Game/蓝图功能库/蓝图模板/SH_Template/角色/丧尸角色/新/BP_SH武器_枪械_AK47_新.BP_SH武器_枪械_AK47_新_C" true "None")
      (Default|F修改胶囊体半径 (Variables|Default|GetRef物理移动) 34.0)
      (Default|CE播放胶囊体缩放 (Variables|Default|GetRef物理移动))
      (Variables|/Game/蓝图功能库/蓝图模板/SH_Template/角色/集中点/BP_物理移动.BP_物理移动_C|Set聚拢衰减距离 _ref物理移动 (* (Variables|/Game/蓝图功能库/蓝图模板/SH_Template/角色/集中点/BP_物理移动.BP_物理移动_C|Get聚拢衰减距离 _ref物理移动) _returnvalue_2 1.0))
      (Variables|/Game/蓝图功能库/蓝图模板/SH_Template/角色/集中点/BP_物理移动.BP_物理移动_C|Set旋转衰减距离 _ref物理移动 (* (Variables|/Game/蓝图功能库/蓝图模板/SH_Template/角色/集中点/BP_物理移动.BP_物理移动_C|Get旋转衰减距离 _ref物理移动) _returnvalue_2 2.0))
      (Variables|/Game/蓝图功能库/蓝图模板/SH_Template/角色/集中点/BP_物理移动.BP_物理移动_C|Set生成力范围 _ref物理移动_3 (* (Variables|/Game/蓝图功能库/蓝图模板/SH_Template/角色/集中点/BP_物理移动.BP_物理移动_C|Get生成力范围 _ref物理移动_3) _returnvalue_2 2.0))
      ;[0.08691 0.15 0.03577 0.5] 切换武器时向周围弹射
      (Default|F弹射物理移动 (Variables|Default|GetRef物理移动) (* (Math|Vector|Normalize (- (Transformation|GetActorLocation) (Transformation|GetActorLocation (Variables|Default|GetRef集中点)))) (Math|Float|Clamp(Float) (* (Utilities|Array|Length (Variables|/Game/蓝图功能库/蓝图模板/SH_Template/角色/集中点/BP_集中点.BP_集中点_C|Get集中的角色数组 (Variables|Default|GetRef集中点))) 200) (.x (Variables|/Game/蓝图功能库/蓝图模板/SH_Template/角色/集中点/BP_物理移动.BP_物理移动_C|Get生成力范围 (Variables|Default|GetRef物理移动))) (.y (Variables|/Game/蓝图功能库/蓝图模板/SH_Template/角色/集中点/BP_物理移动.BP_物理移动_C|Get生成力范围 (Variables|Default|GetRef物理移动))))) true :!label _label))
    (:星际战士加特林
      ;[1 0.2109 0 0.8] 星际战士加特林
      (CallFunction|F创建武器并装备 "/Game/蓝图功能库/蓝图模板/SH_Template/角色/丧尸角色/新/BP_SH武器_枪械_加特林JF_新.BP_SH武器_枪械_加特林JF_新_C" true "None")
      (Default|F修改胶囊体半径 _ref物理移动_2 6e+01)
      (Default|CE播放胶囊体缩放 _ref物理移动_2)
      (Variables|/Game/蓝图功能库/蓝图模板/SH_Template/角色/集中点/BP_物理移动.BP_物理移动_C|Set聚拢衰减距离 _ref物理移动_4 (* (Variables|/Game/蓝图功能库/蓝图模板/SH_Template/角色/集中点/BP_物理移动.BP_物理移动_C|Get聚拢衰减距离 _ref物理移动_4) _returnvalue 1.0))
      (Variables|/Game/蓝图功能库/蓝图模板/SH_Template/角色/集中点/BP_物理移动.BP_物理移动_C|Set旋转衰减距离 _ref物理移动_4 (* (Variables|/Game/蓝图功能库/蓝图模板/SH_Template/角色/集中点/BP_物理移动.BP_物理移动_C|Get旋转衰减距离 _ref物理移动_4) _returnvalue 2.0))
      (Variables|/Game/蓝图功能库/蓝图模板/SH_Template/角色/集中点/BP_物理移动.BP_物理移动_C|Set生成力范围 _ref物理移动_5 (* (Variables|/Game/蓝图功能库/蓝图模板/SH_Template/角色/集中点/BP_物理移动.BP_物理移动_C|Get生成力范围 _ref物理移动_5) _returnvalue 0.6))
      (goto _label))
    (:手枪
      ;[0.15 0.1206 0.002851 0.5] 手枪
      (CallFunction|F创建武器并装备 "/Game/蓝图功能库/蓝图模板/SH_Template/角色/丧尸角色/新/BP_SH武器_枪械_战锤手枪_新.BP_SH武器_枪械_战锤手枪_新_C" true "None"))))