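; Base zombie character Blueprint for the SH template.
; Its construction script picks a random skeletal mesh from the zombie mesh array using the character's seeded stream, then resets the mesh offset.
; A collision function deals "角色撞击" damage equal to its max health to both the struck SH character and itself, with seeded knockback impulses, its own rotated 180 degrees.
; Interaction requests always fail.
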(event EventBeginPlay
  (|CallParentFunction))

(event EventTick
  (params (DeltaSeconds :type Float%20%28single-precision%29))
  (|CallParentFunction DeltaSeconds) ; 此节点被禁用，将不会被调用。\n从引脚连出引线来编译功能。
)

(fn ConstructionScript
  (bind _丧尸骨骼网格体 (Variables|角色参数|生成时|Get丧尸骨骼网格体))
  (|CallParentFunction)
  (if (Utilities|Array|IsNotEmpty _丧尸骨骼网格体)
    (CallFunction|F更换骨骼网格体 (Variables|Character|GetMesh) (.OutItem (Utilities|Array|RandomFromStream _丧尸骨骼网格体 (Variables|Default|GetSH角色Seed)))))
  (CallFunction|F重置网格体偏移))

(fn BPI-发起交互
  (params (发起者 :type Actor%20Object%20Reference) (交互类型 :type String))
  (return false ""))

(fn F碰撞敌人造成伤害
  (params (OtherActor :type Actor%20Object%20Reference) (HitResult :type Hit%20Result%20Structure%20%28by%20ref%29))
  (bind _self self)
  (bind _角色生命值_max (Variables|Default|Get角色生命值_Max))
  (bind _asbp_sh角色_base (Utilities|Casting|CastToBP_SH角色_Base OtherActor))
  (Default|BPI-应用伤害-SH _asbp_sh角色_base _角色生命值_max _self _self "角色撞击" (CallFunction|流送中范围内复合冲量 (Transformation|GetActorLocation) (Transformation|GetActorLocation _asbp_sh角色_base) "(X=800.000000,Y=1000.000000)" "(X=800.000000,Y=1000.000000)" 0.0 (Variables|Default|GetSH角色Seed)) HitResult)
  (CallFunction|BPI-应用伤害-SH _角色生命值_max _asbp_sh角色_base _asbp_sh角色_base "角色撞击" (Math|Vector|RotateVector (CallFunction|流送中范围内复合冲量 (Transformation|GetActorLocation) (Transformation|GetActorLocation _asbp_sh角色_base) "(X=800.000000,Y=1000.000000)" "(X=800.000000,Y=1000.000000)" 0.0 (Variables|Default|GetSH角色Seed)) "0.000000,180.000000,0.000000")) ; 对自己也造成等额伤害
)