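; Zombie base character that chases the BP_集中点 actor along a spline and rams SH characters.
; Construction picks a seeded random mesh; BeginPlay applies mesh, animation and materials from DT_敌人角色资产, then randomizes play rate and starts the chase.
; On collision, it deals its max health as damage to both the character and itself, with seeded, rotated knockback impulses.
; Interaction requests always fail.
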(event EventBeginPlay
  (|CallParentFunction)
  (CallFunction|F敌人通过表初始化资源)
  (CallFunction|F修改角色移动速度 451.0 false)
  (Variables|Default|Set追击目标改为AiMoveTo false)
  (bind _returnvalue (Actor|GetActorOfClass "/Game/蓝图功能库/蓝图模板/SH_Template/角色/集中点/BP_集中点.BP_集中点_C"))
  (CallFunction|CE-沿样条线追击目标 0 _returnvalue 1.2e+03)
  (Components|Timeline|SetPlayRate (Variables|Character|GetMesh) (Math|Random|RandomFloatinRange 0.8 1.2))
  (Variables|Default|Set到达停止距离 0.0))

(event EventTick
  (params (DeltaSeconds :type Float%20%28single-precision%29))
  (|CallParentFunction DeltaSeconds) ; 此节点被禁用，将不会被调用。\n从引脚连出引线来编译功能。
)

(fn ConstructionScript
  (bind _丧尸骨骼网格体 (Variables|角色参数|生成时|Get丧尸骨骼网格体))
  (|CallParentFunction)
  (if (Utilities|Array|IsNotEmpty _丧尸骨骼网格体)
    (CallFunction|F更换骨骼网格体 (Variables|Character|GetMesh) (.OutItem (Utilities|Array|RandomFromStream _丧尸骨骼网格体 (Variables|Default|GetSH角色Seed)))))
  (CallFunction|F重置网格体偏移))

(fn BPI-发起交互
  (params (发起者 :type Actor%20Object%20Reference) (交互类型 :type String))
  (return false ""))

(fn F碰撞敌人造成伤害
  (params (OtherActor :type Actor%20Object%20Reference) (HitResult :type Hit%20Result%20Structure%20%28by%20ref%29))
  (bind _self self)
  (bind _角色生命值_max (Variables|Default|Get角色生命值_Max))
  (bind _asbp_sh角色_base (Utilities|Casting|CastToBP_SH角色_Base OtherActor))
  (Default|BPI-应用伤害-SH _asbp_sh角色_base _角色生命值_max _self _self "角色撞击" (CallFunction|流送中范围内复合冲量 (Transformation|GetActorLocation) (Transformation|GetActorLocation _asbp_sh角色_base) "(X=800.000000,Y=1000.000000)" "(X=800.000000,Y=1000.000000)" 0.0 (Variables|Default|GetSH角色Seed)) HitResult)
  (CallFunction|BPI-应用伤害-SH _角色生命值_max _asbp_sh角色_base _asbp_sh角色_base "角色撞击" (Math|Vector|RotateVector (CallFunction|流送中范围内复合冲量 (Transformation|GetActorLocation) (Transformation|GetActorLocation _asbp_sh角色_base) "(X=800.000000,Y=1000.000000)" "(X=800.000000,Y=1000.000000)" 0.0 (Variables|Default|GetSH角色Seed)) "0.000000,180.000000,0.000000")) ; 对自己也造成等额伤害
)

(fn F敌人通过表初始化资源
  (bind _returnvalue (Utilities|GetDataTableRow "/Game/蓝图功能库/蓝图模板/SH_Template/角色/表资产/DT_敌人角色资产.DT_敌人角色资产" (Variables|Default|Get角色选择))
    (:then
      (Components|SkeletalMesh|SetSkeletalMeshAsset (Variables|Character|GetMesh) (.骨骼网格体 (Utilities|Struct|BreakST_敌人角色资产 _returnvalue)))
      (Components|Animation|SetAnimation (Variables|Character|GetMesh) (.动画资产 (Utilities|Struct|BreakST_敌人角色资产 _returnvalue)))
      (Audio|Components|Audio|Play (Variables|Character|GetMesh) true)
      (for (_array_element _array_index) (.材质 (Utilities|Struct|BreakST_敌人角色资产 _returnvalue))
        (Rendering|Material|SetMaterial (Variables|Character|GetMesh) _array_index _array_element))
      (return))))