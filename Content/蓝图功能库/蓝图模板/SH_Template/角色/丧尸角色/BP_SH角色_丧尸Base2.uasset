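; Base zombie character, seeded with a random skeletal mesh, that chases BP_集中点 (gather point) along a spline.
; On arrival it attacks, kills the gathered characters with launch forces, and swaps BGM for a sound sting.
; Hit-flash material changes mirror onto bound external actors, falling back to the attach parent.
; Tick broadcasts health changes and optionally kills it when hidden; its collision function deals its max health to both parties.
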(event Custom|CEED-材质变化时
  (params (ParameterName :type Name) (ParmeterValue :type Float%20%28double-precision%29) (TimelineAlpha :type Float%20%28double-precision%29))
  ;[1 0 0.6562] 绑定外部的受击闪烁到自己身上
  ;;[1 0.9609 0] 修改材质
  (for _array_element (Variables|Default|Get外部MeshComps)
    (Rendering|Material|SetVectorParameterValueonMaterials _array_element "SH_闪烁Color" (Math|Conversions|ToVector(LinearColor) (Variables|Default|Get受击颜色))) ; 将颜色配置到网格体中
    (Rendering|Material|SetScalarParameterValueonMaterials _array_element ParameterName ParmeterValue)))

(event Custom|CE_绑定事件
  (bind _returnvalue (Actor|GetAttachParentActor))
  ;[1 0 0.6562] 绑定外部的受击闪烁到自己身上
  (if (Utilities|Array|IsValidIndex (Variables|Default|Get绑定外部Actor))
    (EventDispatchers|BindEventtoED-材质变化时 (delegate Custom|CEED-材质变化时))
    (for _array_element (Variables|Default|Get绑定外部Actor)
      (bind _网格体组件 (CallFunction|F获取所有网格体组件 _array_element true true false))
      (Utilities|Array|AppendArray (Variables|Default|Get外部MeshComps) _网格体组件)
      (Rendering|Material|SetVectorParameterValueonMaterials _网格体组件 "SH_闪烁Color" (Math|Conversions|ToVector(LinearColor) (Variables|Default|Get受击颜色))) ; 将颜色配置到网格体中
    )
    (else
      ;;[0.07812 1 0 0.8] 如果没有绑定外部Actor，尝试绑定到附加父级
      (Utilities|IsValid _returnvalue
        (:Is%20Valid
          (Utilities|Array|Add (Variables|Default|Get绑定外部Actor) _returnvalue)
          (CallFunction|CE绑定事件))))))

(event EventBeginPlay
  (|CallParentFunction)
  (bind _returnvalue (Actor|GetActorOfClass "/Game/蓝图功能库/蓝图模板/SH_Template/角色/集中点/BP_集中点.BP_集中点_C"))
  (CallFunction|CE-沿样条线追击目标 0 _returnvalue 2.2e+03)
  (CallFunction|F修改角色移动速度 4.4e+02 false)
  (CallFunction|CE绑定事件))

(event EventTick
  (params (DeltaSeconds :type Float%20%28single-precision%29))
  (|CallParentFunction DeltaSeconds)
  (Utilities|FlowControl|Sequence
    (:then_0
      (if (!= (Variables|Default|Get角色生命值_Current) (Variables|Default|Get角色生命值%20Last))
        (bind _output_get (Variables|Default|Set角色生命值%20Last (Variables|Default|Get角色生命值_Current)))
        (Default|CallED-生命值变化时 _output_get)))
    (:then_1
      (if (Variables|Default|Get显隐变更时死亡)
        (if (!= (Variables|Default|GetbHidden) (Variables|Default|GetActor在游戏中隐藏_Last))
          (bind _output_get_2 (Variables|Default|SetActor在游戏中隐藏_Last (Variables|Default|GetbHidden)))
          (if _output_get_2
            (bind _output_get_3 (Variables|Default|Set角色生命值_Current 0.0))
            (Variables|Default|Set角色生命值%20Last _output_get_3)
            (CallFunction|CE角色死亡(强制) "0, 0, 0" 0.0)))))))

(event EventCE到达目标
  ;[0.08294 0.15 0.04282 0.5] CE_到达目标
  (Variables|Default|Set攻击 true)
  (Variables|/Script/Engine.CharacterMovementComponent|SetMaxWalkSpeed (Variables|Character|GetCharacterMovement) 0.0)
  (Utilities|FlowControl|Delay 0.5)
  (CallFunction|震屏 "/Game/蓝图功能库/相机振动/CS_轮胎撞人.CS_轮胎撞人_C")
  (bind _returnvalue (Actor|GetActorOfClass "/Game/蓝图功能库/蓝图模板/SH_Template/角色/集中点/BP_集中点_C.BP_集中点_C_C"))
  (Default|F杀死一批 _returnvalue (Utilities|Array|Length (Variables|/Game/蓝图功能库/蓝图模板/SH_Template/角色/集中点/BP_集中点.BP_集中点_C|Get集中的角色数组 _returnvalue)) "(X=26400.000000,Y=29040.000000)" "(X=25196.700375,Y=28724.238428)")
  (Niagara|SpawnSystematLocation "/Game/分类/爆炸/niagara/P_Attack03.P_Attack03" (Transformation|GetActorLocation _returnvalue) "0, 0, 0" "0.800000,0.800000,0.800000")
  (Variables|/Game/Assets/Maps/Level_Bp/BP_XiangJiMoban.BP_XiangJiMoban_C|Set停下否？ (Variables|Default|GetBP_XiangJiMoban) false)
  (bind _returnvalue_2 (Actor|GetActorOfClass "/Game/蓝图功能库/蓝图模板/SH_Template/角色/玩家控制器/BP_音效控制.BP_音效控制_C"))
  (Audio|Components|Audio|Stop (Variables|/Game/蓝图功能库/蓝图模板/SH_Template/角色/玩家控制器/BP_音效控制.BP_音效控制_C|GetBGM _returnvalue_2))
  (Audio|PlaySound2D "/Game/Runnning/Audios/糗大了.糗大了" 1.0 1.0 0.2 0 0))

(fn ConstructionScript
  (bind _丧尸骨骼网格体 (Variables|生成时|Get丧尸骨骼网格体))
  (|CallParentFunction)
  (if (Utilities|Array|IsNotEmpty _丧尸骨骼网格体)
    (CallFunction|F更换骨骼网格体 (Variables|Character|GetMesh) (.OutItem (Utilities|Array|RandomFromStream _丧尸骨骼网格体 (Variables|Default|GetSH角色Seed)))))
  (CallFunction|F重置网格体偏移))

(fn BPI-发起交互
  (params (发起者 :type Actor%20Object%20Reference) (交互类型 :type String))
  (return false ""))

(fn F碰撞敌人造成伤害
  (params (OtherActor :type Actor%20Object%20Reference) (HitResult :type Hit%20Result%20Structure%20%28by%20ref%29))
  (bind _self self)
  (bind _角色生命值_max (Variables|Default|Get角色生命值_Max))
  (bind _asbp_sh角色_base (Utilities|Casting|CastToBP_SH角色_Base OtherActor))
  (Default|BPI-应用伤害-SH _asbp_sh角色_base _角色生命值_max _self _self "角色撞击" (CallFunction|流送中范围内复合冲量 (Transformation|GetActorLocation) (Transformation|GetActorLocation _asbp_sh角色_base) "(X=800.000000,Y=1000.000000)" "(X=800.000000,Y=1000.000000)" 0.0 (Variables|Default|GetSH角色Seed)) HitResult)
  (CallFunction|BPI-应用伤害-SH _角色生命值_max _asbp_sh角色_base _asbp_sh角色_base "角色撞击" (Math|Vector|RotateVector (CallFunction|流送中范围内复合冲量 (Transformation|GetActorLocation) (Transformation|GetActorLocation _asbp_sh角色_base) "(X=800.000000,Y=1000.000000)" "(X=800.000000,Y=1000.000000)" 0.0 (Variables|Default|GetSH角色Seed)) "0.000000,180.000000,0.000000")) ; 对自己也造成等额伤害
)