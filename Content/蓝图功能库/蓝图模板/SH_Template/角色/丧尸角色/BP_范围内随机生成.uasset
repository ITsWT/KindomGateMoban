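; A zombie spawner actor that scatters BP_SH角色_丧尸Base1 characters at random positions within its Box component.
; On BeginPlay it spawns 生成总数 (total count) zombies in a loop, randomizing X and Y inside the box while keeping the spawner's Z and rotation.
; Spawns adjust for collisions but always succeed, and the spawner destroys itself once the loop finishes.
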(event EventBeginPlay
  (bind _box (Variables|Default|GetBox))
  (bind _returnvalue (Transformation|GetWorldLocation _box))
  (bind _boxextent (Variables|/Script/Engine.BoxComponent|GetBoxExtent _box))
  (bind _returnvalue_2 (Math|Random|RandomPointinBoundingBox _returnvalue _boxextent))
  (for _index (range 0 (- (Variables|生成|Get生成总数) 1))
    (Game|SpawnActorfromClass :Class "/Game/蓝图功能库/蓝图模板/SH_Template/角色/丧尸角色/BP_SH角色_丧尸Base1.BP_SH角色_丧尸Base1_C" :SpawnTransform (Math|Transform|MakeTransform (Math|Vector|MakeVector (.x _returnvalue_2) (.y _returnvalue_2) (.z (Transformation|GetActorLocation))) (Transformation|GetActorRotation) "1.000000,1.000000,1.000000") :CollisionHandlingOverride "AdjustIfPossibleButAlwaysSpawn" :TransformScaleMethod "MultiplyWithRoot" :Ref集中点 0 :Instigator 0))
  (Actor|DestroyActor))

(fn ConstructionScript)