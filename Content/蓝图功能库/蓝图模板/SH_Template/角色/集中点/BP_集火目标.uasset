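; BP_集火目标 is a focus-fire target that gives each shooter in a group its own attack point around a Sphere component.
; F计算攻击方向 takes the shooter's 2D offset from the group center, scales it by sphere radius over group radius, and applies it to the sphere's location, mirroring the formation onto the target.
; DebugMode reveals the Sphere and Billboard and draws an arrow from each firing position to its computed point.
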(fn ConstructionScript
  (Development|SetHiddeninGame (Variables|Default|GetSphere) (not (Variables|Default|GetDebugMode)) false))

(fn F计算攻击方向
  (params (开火位置 :type Vector) (群体中心位置 :type Vector) (群集半径 :type Float%20%28double-precision%29))
  (LocalVariables|Set所在半径 (Math|Vector|Distance2D(Vector) 开火位置 群体中心位置))
  (LocalVariables|Set所在方向 (CallFunction|单元方向2D 群体中心位置 开火位置))
  (LocalVariables|Set半径倍率 (/ (Components|Sphere|GetScaledSphereRadius (Variables|Default|GetSphere)) 群集半径))
  (LocalVariables|Set最终攻击位置 (+ (Transformation|GetWorldLocation (Variables|Default|GetSphere)) (* (LocalVariables|Get所在方向) (* (LocalVariables|Get所在半径) (LocalVariables|Get半径倍率)))))
  (Utilities|FlowControl|Sequence
    (:then_0
      (if (Variables|Default|GetDebugMode)
        (Rendering|Debug|DrawDebugArrow 开火位置 (LocalVariables|Get最终攻击位置) 5e+02 "(R=0.000000,G=1.000000,B=0.788188,A=1.000000)" 0.0 2.0)))
    (:then_1
      (return (LocalVariables|Get最终攻击位置)))))