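; BP_集中点 is a crowd gathering point that collects same-faction SH characters and drives them as one group.
; Absorb overlaps register candidates, the core sphere admits them, and a chase sphere sends enemies spline-chasing it.
; Tick pseudo-attaches members' physics-movement actors by adding its movement delta, then syncs firing and untested focus-fire aim.
; Functions spawn members using a seeded stream and apply group-wide weapon, level, mesh, effect, invincibility, knockback and kill operations.
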(event OnComponentBeginOverlap(Sphere_核心)
  (params (OverlappedComponent :type Primitive%20Component%20Object%20Reference) (OtherActor :type Actor%20Object%20Reference) (OtherComp :type Primitive%20Component%20Object%20Reference) (OtherBodyIndex :type Integer) (bFromSweep :type Boolean) (SweepResult :type Hit%20Result%20Structure%20%28by%20ref%29))
  ;[0.3594 1 0] 抵达核心区域的角色 直接加入
  (bind _asbp_sh角色_base (Utilities|Casting|CastToBP_SH角色_Base OtherActor))
  (if (== (Variables|/Game/蓝图功能库/蓝图模板/SH_Template/角色/BP_SH角色_Base.BP_SH角色_Base_C|Get角色所属阵营 _asbp_sh角色_base) (Variables|默认|参数|Get所属阵营))
    (CallFunction|F尝试加入角色 _asbp_sh角色_base)
    (CallFunction|F成功加入角色 _asbp_sh角色_base)
    (Variables|/Game/蓝图功能库/蓝图模板/SH_Template/角色/BP_SH角色_Base.BP_SH角色_Base_C|Set已加入集中点 _asbp_sh角色_base true)))

(event OnComponentBeginOverlap(Sphere_激活追击)
  (params (OverlappedComponent :type Primitive%20Component%20Object%20Reference) (OtherActor :type Actor%20Object%20Reference) (OtherComp :type Primitive%20Component%20Object%20Reference) (OtherBodyIndex :type Integer) (bFromSweep :type Boolean) (SweepResult :type Hit%20Result%20Structure%20%28by%20ref%29))
  ;[0.3125 0 1] 重叠时启用追击
  (if (Variables|默认|追击|Get追击_启用)
    (bind _asbp_sh角色_base (Utilities|Casting|CastToBP_SH角色_Base OtherActor))
    (if (CallFunction|F判断SH角色有效且敌对 _asbp_sh角色_base (Variables|默认|参数|Get所属阵营))
      ;;[0 1 0.8594 0.8] 移速调整
      (if (>= (Variables|默认|追击|Get追击_覆盖移速) 0.0)
        (Default|F修改角色移动速度 _asbp_sh角色_base (Variables|默认|追击|Get追击_覆盖移速) true)
        (elif (Variables|默认|追击|Get追击_保持当前速度)
          (Default|F修改角色移动速度 _asbp_sh角色_base (Variables|/Game/蓝图功能库/蓝图模板/SH_Template/角色/BP_SH角色_Base.BP_SH角色_Base_C|Get角色移速_Current _asbp_sh角色_base) true)
          (else
            (Default|F修改角色移动速度 _asbp_sh角色_base (Variables|/Game/蓝图功能库/蓝图模板/SH_Template/角色/BP_SH角色_Base.BP_SH角色_Base_C|Get角色移速_期望 _asbp_sh角色_base) true))))
      (Default|CE-沿样条线追击目标 _asbp_sh角色_base 0 self (Components|Sphere|GetScaledSphereRadius (Variables|Default|GetSphere_激活追击)))
      (if (Utilities|Enum|NotEqual(Enum) (Variables|/Script/Engine.CharacterMovementComponent|GetMovementMode (Variables|/Script/Engine.Character|GetCharacterMovement _asbp_sh角色_base)) "MOVE_None")
        (Transformation|DetachFromActor _asbp_sh角色_base "KeepWorld" "KeepWorld" "KeepWorld")))))

(event OnComponentBeginOverlap(Sphere_吸收角色)
  (params (OverlappedComponent :type Primitive%20Component%20Object%20Reference) (OtherActor :type Actor%20Object%20Reference) (OtherComp :type Primitive%20Component%20Object%20Reference) (OtherBodyIndex :type Integer) (bFromSweep :type Boolean) (SweepResult :type Hit%20Result%20Structure%20%28by%20ref%29))
  ;[0 1 0.5547] 重叠时吸收角色
  (bind _asbp_sh角色_base (Utilities|Casting|CastToBP_SH角色_Base OtherActor))
  (if (== (Variables|/Game/蓝图功能库/蓝图模板/SH_Template/角色/BP_SH角色_Base.BP_SH角色_Base_C|Get角色所属阵营 _asbp_sh角色_base) (Variables|默认|参数|Get所属阵营))
    (CallFunction|F尝试加入角色 _asbp_sh角色_base)))

(event OnComponentBeginOverlap(Box_吸收角色)
  (params (OverlappedComponent :type Primitive%20Component%20Object%20Reference) (OtherActor :type Actor%20Object%20Reference) (OtherComp :type Primitive%20Component%20Object%20Reference) (OtherBodyIndex :type Integer) (bFromSweep :type Boolean) (SweepResult :type Hit%20Result%20Structure%20%28by%20ref%29))
  ;[0 1 0.5547] 重叠时吸收角色
  (bind _asbp_sh角色_base (Utilities|Casting|CastToBP_SH角色_Base OtherActor))
  (if (== (Variables|/Game/蓝图功能库/蓝图模板/SH_Template/角色/BP_SH角色_Base.BP_SH角色_Base_C|Get角色所属阵营 _asbp_sh角色_base) (Variables|默认|参数|Get所属阵营))
    (CallFunction|F尝试加入角色 _asbp_sh角色_base)))

(event Custom|CEED-角色死亡时
  (params (死亡的角色 :type BP%20SH角色%20Base%20Object%20Reference))
  (Utilities|Array|RemoveItem (Variables|状态|Get集中的角色数组) 死亡的角色))

(event EventTick
  (params (DeltaSeconds :type Float%20%28single-precision%29))
  ;[1 0.07031 0] Tick：同步位置（伪附加）
  (CallFunction|F计算实时速度)
  (if (Utilities|Array|IsNotEmpty (Variables|状态|Get集中的Actor数组))
    (for _array_element (Variables|状态|Get集中的Actor数组)
      (Utilities|IsValid _array_element
        (:Is%20Valid
          (Transformation|AddActorWorldOffset _array_element (* (Variables|状态|Get当前实时速度cm/F) (Variables|默认|参数|Get同步程度百分比))))
        (:Is%20Not%20Valid
          (Utilities|Array|RemoveItem (Variables|状态|Get集中的Actor数组) _array_element))))
    (CallFunction|F统一开火 (Variables|默认|参数|Get统一武器能够开火))
    (CallFunction|F获取集火模式状态)))

(event EventBeginPlay
  ;[0 0.4141 1] 初始化：记录变量，启用重叠
  (Variables|状态|Set上一帧所在位置 (Transformation|GetActorLocation))
  (Collision|SetCollisionEnabled (Variables|Default|GetSphere_激活追击) "QueryOnly")
  (Variables|状态|Set角色等级 "NewEnumerator0"))

(fn ConstructionScript)

(fn F计算实时速度
  (Variables|状态|Set当前实时速度cm/F (- (Transformation|GetActorLocation) (Variables|状态|Get上一帧所在位置)))
  (Variables|状态|Set上一帧所在位置 (Transformation|GetActorLocation)))

(fn F全体更换武器
  (params (主武器 :type String))
  (Variables|默认|参数|Set当前武器 主武器)
  (for _array_element (Variables|状态|Get集中的角色数组)
    (Utilities|IsValid _array_element
      (:Is%20Valid
        (Default|F尝试切换主武器 _array_element (Variables|默认|参数|Get当前武器) true)))))

(fn F全体闪烁
  (params (颜色 :type Linear%20Color%20Structure :default "(R=1.000000,G=1.000000,B=1.000000,A=1.000000)") (覆盖菲涅尔 :type Float%20%28double-precision%29))
  (for _array_element (Variables|状态|Get集中的角色数组)
    (Utilities|IsValid _array_element
      (:Is%20Valid
        (Default|CE-播放闪烁 _array_element false 颜色 覆盖菲涅尔 true 0.3)))))

(fn F全体弹开
  (params (强度 :type Float%20%28double-precision%29))
  (bind _集中的actor数组 (Variables|状态|Get集中的Actor数组))
  (bind _boxextent (Collision|GetActorArrayBounds _集中的actor数组))
  (for _array_element _集中的actor数组
    (bind _asbp_物理移动 (Utilities|Casting|CastToBP_物理移动 _array_element))
    (Default|F弹射物理移动 _asbp_物理移动 (* (CallFunction|单元方向Actor self _asbp_物理移动 true) 强度 (Math|Float|MapRangeUnclamped (Transformation|GetHorizontalDistanceTo _asbp_物理移动) 0.0 (+ (.x _boxextent) (.y _boxextent)) 0.1 1.0)) true)))

(fn F尝试加入角色
  (params (加入角色 :type BP%20SH角色%20Base%20Object%20Reference))
  ;[1 0 0.375] 加入条件
  (if (and (not (Variables|/Game/蓝图功能库/蓝图模板/SH_Template/角色/BP_SH角色_Base.BP_SH角色_Base_C|Get已加入集中点 加入角色)) (not (Variables|/Game/蓝图功能库/蓝图模板/SH_Template/角色/BP_SH角色_Base.BP_SH角色_Base_C|Get角色已死亡 加入角色)))
    ;[0.8984 1 0] 记录变量
    (Variables|/Game/蓝图功能库/蓝图模板/SH_Template/角色/BP_SH角色_Base.BP_SH角色_Base_C|SetRef集中点 加入角色 self)
    ;[1 0.6094 0] 尝试加入期间，暂停旋转
    (Utilities|IsValid (Variables|/Game/蓝图功能库/蓝图模板/SH_Template/角色/BP_SH角色_Base.BP_SH角色_Base_C|GetRef物理移动 加入角色)
      (:Is%20Valid
        (Variables|/Game/蓝图功能库/蓝图模板/SH_Template/角色/集中点/BP_物理移动.BP_物理移动_C|Set旋转强度缩放 (Variables|/Game/蓝图功能库/蓝图模板/SH_Template/角色/BP_SH角色_Base.BP_SH角色_Base_C|GetRef物理移动 加入角色) 0.0)))))

(fn F成功加入角色
  (params (加入角色 :type BP%20SH角色%20Base%20Object%20Reference))
  (bind _ref物理移动 (Variables|/Game/蓝图功能库/蓝图模板/SH_Template/角色/BP_SH角色_Base.BP_SH角色_Base_C|GetRef物理移动 加入角色))
  (bind _mesh (Variables|/Script/Engine.Character|GetMesh 加入角色))
  (Utilities|IsValid 加入角色
    (:Is%20Valid
      (if (not (Variables|/Game/蓝图功能库/蓝图模板/SH_Template/角色/BP_SH角色_Base.BP_SH角色_Base_C|Get已加入集中点 加入角色))
        (Utilities|Array|Add (Variables|状态|Get集中的角色数组) 加入角色)
        (Utilities|FlowControl|Sequence
          (:then_0
            ;[0.6641 0 1] 解除无敌
            (bind _output_get (Variables|/Game/蓝图功能库/蓝图模板/SH_Template/角色/BP_SH角色_Base.BP_SH角色_Base_C|Set无敌状态 加入角色 false))
            (Default|CallED-无敌状态变更时 加入角色 _output_get 加入角色)
            ;[0 0.9531 1] 加入成功后更换武器
            (Default|F尝试切换主武器 加入角色 (Variables|默认|参数|Get当前武器) true)
            ;[1 1 1] 绑定死亡
            (EventDispatchers|BindEventtoED-角色死亡时 加入角色 (EventDispatchers|CreateEvent :!event Custom|CEED-角色死亡时)))
          (:then_1
            ;[0.2656 0 1] 加入数组方便管理
            (Utilities|IsValid (Variables|/Game/蓝图功能库/蓝图模板/SH_Template/角色/BP_SH角色_Base.BP_SH角色_Base_C|GetRef物理移动 加入角色)
              (:Is%20Valid
                (Utilities|Array|AddUnique (Variables|状态|Get集中的Actor数组) (Variables|/Game/蓝图功能库/蓝图模板/SH_Template/角色/BP_SH角色_Base.BP_SH角色_Base_C|GetRef物理移动 加入角色))
                (Variables|/Game/蓝图功能库/蓝图模板/SH_Template/角色/集中点/BP_物理移动.BP_物理移动_C|SetRef集中点 _ref物理移动 self)
                ;;[0.9922 0 1] 启用旋转
                (Variables|/Game/蓝图功能库/蓝图模板/SH_Template/角色/集中点/BP_物理移动.BP_物理移动_C|Set旋转强度缩放 _ref物理移动 1.0))))
          (:then_2
            ;[1 1 1] 加入时播放特效
            (if (Variables|默认|加入|Get加入特效_启用)
              (CallFunction|F生成粒子特效 (Math|Transform|MakeTransform (+ (Transformation|GetWorldLocation _mesh) (Variables|默认|加入|Get加入特效_位置偏移)) "0, 0, 0" (Math|Conversions|ToVector(Float) (Variables|默认|加入|Get加入特效_缩放))) (Variables|默认|加入|Get加入特效_类型) _mesh "None" "KeepWorldPosition" true true false)))
          (:then_3
            (if true
              (Default|CE-播放闪烁 加入角色 false (Variables|默认|加入|Get加入闪烁_颜色) -1.0 true 0.3))))))))

(fn F获取集火模式状态
  (Utilities|IsValid (Variables|默认|参数|Get集火目标Ref)
    (:Is%20Valid
      (if (and (Variables|状态|Get启用集火模式) (Variables|默认|参数|Get统一武器能够开火))
        ;[1 1 1] 整合集火目标，未实验
        (LocalVariables|Setcenter (Transformation|GetWorldLocation (Variables|Default|GetSphere_核心)))
        (for _array_element (Variables|状态|Get集中的角色数组)
          (bind _终点 (Default|F计算攻击方向 (Variables|默认|参数|Get集火目标Ref) (Transformation|GetActorLocation _array_element) (LocalVariables|Getcenter) (Components|Sphere|GetScaledSphereRadius (Variables|Default|GetSphere_核心))))
          (Variables|状态|Set当前集火位置 _终点))
        (else
          (Variables|状态|Set当前集火位置 "0, 0, 0" :!label _label))))
    (:Is%20Not%20Valid
      (goto _label))))

(fn F杀死一批
  (params (数量 :type Integer) (水平力度范围 :type Vector%202D%20Structure :default "(X=1500.000000,Y=2000.000000)") (垂直力度范围 :type Vector%202D%20Structure :default "(X=750.000000,Y=1500.000000)"))
  (if (Utilities|Array|IsNotEmpty (Variables|状态|Get集中的角色数组))
    (bind _sh角色数组 (CallFunction|CastActorArraytoSH角色Array (CallFunction|从Actor数组中获取随机子数组 (Variables|状态|Get集中的角色数组) 数量)))
    (for _array_element _sh角色数组
      (Utilities|IsValid _array_element
        (:Is%20Valid
          (Default|BPI-应用伤害-SH _array_element 9999.0 0 self "集中点减员" (CallFunction|流送中范围内复合冲量 (Transformation|GetActorForwardVector) (+ (Transformation|GetActorUpVector) (Math|Vector|NegateVector (Transformation|GetActorForwardVector))) 水平力度范围 垂直力度范围 0.0 (Variables|默认|参数|Get集中点Seed))))))))

(fn F统一开火
  (params (开火 :type Boolean))
  (Variables|默认|参数|Set统一武器能够开火 开火)
  (for _array_element (Variables|状态|Get集中的角色数组)
    (Utilities|IsValid _array_element
      (:Is%20Valid
        (for _array_element_2 (Variables|/Game/蓝图功能库/蓝图模板/SH_Template/角色/BP_SH角色_Base.BP_SH角色_Base_C|Get已装备的武器 _array_element)
          (Utilities|IsValid _array_element_2
            (:Is%20Valid
              (Variables|/Game/蓝图功能库/蓝图模板/SH_Template/武器/BP_SH武器_Base.BP_SH武器_Base_C|Set武器能够开火 _array_element_2 (Variables|默认|参数|Get统一武器能够开火)))))))))

(fn F筛选阵营角色
  (params (SH角色 :type Array%20of%20BP%20SH角色%20Base%20Object%20References) (阵营 :type Integer))
  (for _array_element SH角色
    (if (and (== (Variables|/Game/蓝图功能库/蓝图模板/SH_Template/角色/BP_SH角色_Base.BP_SH角色_Base_C|Get角色所属阵营 _array_element) 阵营) (not (Variables|/Game/蓝图功能库/蓝图模板/SH_Template/角色/BP_SH角色_Base.BP_SH角色_Base_C|Get角色已死亡 _array_element)))
      (Utilities|Array|Add (LocalVariables|Getlp阵营角色) _array_element)))
  (return (LocalVariables|Getlp阵营角色)))

(fn F全体缩放
  (params (缩放耗时 :type Float%20%28single-precision%29) (缩放曲线 :type Curve%20Vector%20Object%20Reference))
  (for _array_element (Variables|状态|Get集中的角色数组)
    (Utilities|IsValid _array_element
      (:Is%20Valid
        (Default|CE播放网格体缩放 _array_element 缩放耗时 缩放曲线 0.0)))))

(fn F全体特效
  (params (粒子类型 :type F粒子特效%20Structure) (粒子偏移 :type Vector :default "0.000000,0.000000,10.000000") (粒子附加 :type Boolean) (粒子缩放 :type Float%20%28double-precision%29))
  (for _array_element (Variables|状态|Get集中的角色数组)
    (Utilities|IsValid _array_element
      (:Is%20Valid
        (CallFunction|F生成粒子特效 (Math|Transform|MakeTransform (+ (Transformation|GetWorldLocation (Variables|/Script/Engine.Character|GetMesh _array_element)) (* 粒子偏移 (.z (Transformation|GetActorScale3D _array_element)))) "0, 0, 0" (Math|Conversions|ToVector(Float) 粒子缩放)) 粒子类型 (select 粒子附加 (Variables|/Script/Engine.Character|GetMesh _array_element) 0) "None" "KeepWorldPosition" true true false)))))

(fn F全体武器冷却
  (for _array_element (Variables|状态|Get集中的角色数组)
    (for _array_element_2 (Variables|/Game/蓝图功能库/蓝图模板/SH_Template/角色/BP_SH角色_Base.BP_SH角色_Base_C|Get已装备的武器 _array_element)
      (if (Variables|默认|加入|Get需要刷新初始冷却)
        (Default|CE-刷新初始冷却 _array_element_2)
        (else
          (Default|CE-使武器进入冷却 _array_element_2))))))

(fn F增加人数-外围
  (params (数量 :type Integer) (生成间距 :type Float%20%28double-precision%29) (检测长度 :type Float%20%28double-precision%29) (生成类型 :type BP%20SH角色%20Base%20Class%20Reference) (生成缩放 :type Vector :default "1.000000,1.000000,1.000000"))
  (LocalVariables|Set初始角 (Class|KismetMathLibrary|VectorNormal2D (Math|Random|RandomUnitVectorfromStream (Variables|默认|参数|Get集中点Seed)) 0.0001))
  (for _index (range 0 (- 数量 1))
    (LocalVariables|Setlp_角度 (* (/ 3.6e+02 (Math|Conversions|ToFloat(Integer) 数量)) _index))
    (bind (_outhits _returnvalue) (Collision|MultiSphereTraceForObjects (+ (Transformation|GetActorLocation) (* (Math|Vector|RotateVector (LocalVariables|Get初始角) (Math|Rotator|MakeRotator 0.0 0.0 (LocalVariables|Getlp_角度))) 检测长度)) (Transformation|GetActorLocation) 2.0 (Utilities|Array|MakeArray "ObjectTypeQuery3") false 0 "None"))
    (LocalVariables|Setlp_命中结果 _outhits)
    (if _returnvalue
      (bind _命中的actor (CallFunction|命中结果中的Actor _outhits))
      (bind _sh角色数组 (CallFunction|CastActorArraytoSH角色Array _命中的actor))
      (bind _阵营角色 (CallFunction|F筛选阵营角色 _sh角色数组 (Variables|默认|参数|Get所属阵营)))
      (LocalVariables|Setlp_生成位置 (+ (.Location (Collision|BreakHitResult (Utilities|Array|Get(acopy) (LocalVariables|Getlp_命中结果) (Utilities|Array|FindItem _命中的actor (.最远Actor (CallFunction|最远的Actor _阵营角色 (Transformation|GetActorLocation) true)))))) (Math|Vector|RotateVector (Math|Vector|MakeVector 生成间距 0.0 0.0) (Math|Rotator|MakeRotator 0.0 0.0 (LocalVariables|Getlp_角度)))))
      (Rendering|Debug|DrawDebugSphere (LocalVariables|Getlp_生成位置) 8e+01 0 "(R=1.000000,G=0.048397,B=0.000000,A=1.000000)" 0.0)
      (else
        (LocalVariables|Setlp_生成位置 (Transformation|GetWorldLocation (Variables|Default|GetSphere_核心)))))
    (bind _returnvalue_2 (Game|SpawnActorfromClass 生成类型 (Math|Transform|MakeTransform (LocalVariables|Getlp_生成位置) (Transformation|GetActorRotation) 生成缩放) "AlwaysSpawn" "MultiplyWithRoot" 0 (CallFunction|流送中的随机流送 (Variables|默认|参数|Get集中点Seed)) (Variables|默认|参数|Get所属阵营) self -1.0 0))
    (Utilities|IsValid _returnvalue_2
      (:Is%20Valid
        (Utilities|Array|Add (LocalVariables|Getlp_生成角色arr) _returnvalue_2)
        (CallFunction|F生成角色后 _returnvalue_2))
      (:Is%20Not%20Valid
        (Development|PrintString "集中点生成角色失败" true true "(R=1.000000,G=0.111111,B=0.000000,A=1.000000)"))))
  (return (LocalVariables|Getlp_生成角色arr)))

(fn F全体无敌
  (params (无敌时长 :type Float%20%28double-precision%29))
  (for _array_element (Variables|状态|Get集中的角色数组)
    (if (not (Variables|/Game/蓝图功能库/蓝图模板/SH_Template/角色/BP_SH角色_Base.BP_SH角色_Base_C|Get无敌状态 _array_element))
      (Default|CE-设置角色无敌 _array_element true 无敌时长))))

(fn F增加人数-中心
  (params (数量 :type Integer) (生成范围 :type Float%20%28double-precision%29) (生成类型 :type BP%20SH角色%20Base%20Class%20Reference) (生成缩放 :type Vector :default "1.000000,1.000000,1.000000"))
  (for _index (range 0 (- 数量 1))
    (bind _output_get (LocalVariables|Setlp_生成位置 (CallFunction|流送中圆形边随机点 (Transformation|GetWorldLocation (Variables|Default|GetSphere_核心)) 生成范围 (Variables|默认|参数|Get集中点Seed))))
    (Rendering|Debug|DrawDebugSphere _output_get 34.0 0 "(R=0.401460,G=2.000000,B=0.000000,A=1.000000)" 0.0)
    (bind _returnvalue (Game|SpawnActorfromClass 生成类型 (Math|Transform|MakeTransform (LocalVariables|Getlp_生成位置) (Transformation|GetActorRotation) 生成缩放) "AdjustIfPossibleButAlwaysSpawn" "MultiplyWithRoot" 0 (CallFunction|流送中的随机流送 (Variables|默认|参数|Get集中点Seed)) (Variables|默认|参数|Get所属阵营) self -1.0 0))
    (Utilities|IsValid _returnvalue
      (:Is%20Valid
        (Utilities|Array|Add (LocalVariables|Getlp_生成的角色) _returnvalue)
        (CallFunction|F生成角色后 _returnvalue))
      (:Is%20Not%20Valid
        (Development|PrintString "集中点生成角色失败" true true "(R=1.000000,G=0.111111,B=0.000000,A=1.000000)"))))
  (return (LocalVariables|Getlp_生成的角色)))

(fn F增加人数-位置
  (params (数量 :type Integer) (生成范围 :type Float%20%28double-precision%29) (生成类型 :type BP%20SH角色%20Base%20Class%20Reference) (生成缩放 :type Vector :default "1.000000,1.000000,1.000000") (位置 :type Vector))
  (for _index (range 0 (- 数量 1))
    (bind _output_get (LocalVariables|Setlp_生成位置 (CallFunction|流送中圆形边随机点 位置 生成范围 (Variables|默认|参数|Get集中点Seed))))
    (Rendering|Debug|DrawDebugSphere _output_get 34.0 0 "(R=1.000000,G=0.048397,B=0.000000,A=1.000000)" 0.0 2.0)
    (bind _returnvalue (Game|SpawnActorfromClass 生成类型 (Math|Transform|MakeTransform (LocalVariables|Getlp_生成位置) (Transformation|GetActorRotation) 生成缩放) "AlwaysSpawn" "MultiplyWithRoot" 0 (CallFunction|流送中的随机流送 (Variables|默认|参数|Get集中点Seed)) (Variables|默认|参数|Get所属阵营) self -1.0 0))
    (Utilities|IsValid _returnvalue
      (:Is%20Valid
        (Utilities|Array|Add (LocalVariables|Getlp_生成的角色) _returnvalue)
        (CallFunction|F生成角色后 _returnvalue))
      (:Is%20Not%20Valid
        (Development|PrintString "集中点生成角色失败" true true "(R=1.000000,G=0.111111,B=0.000000,A=1.000000)"))))
  (return (LocalVariables|Getlp_生成的角色)))

(fn F生成角色后
  (params (新角色 :type BP%20SH角色%20Base%20Object%20Reference))
  (CallFunction|F尝试加入角色 新角色)
  (CallFunction|F成功加入角色 新角色)
  (Variables|/Game/蓝图功能库/蓝图模板/SH_Template/角色/BP_SH角色_Base.BP_SH角色_Base_C|Set已加入集中点 新角色 true)
  (if (Variables|默认|加入|Get增加人数时刷新武器冷却)
    (全角色控制|F全体武器冷却)))

(fn F全体切换角色
  (params (新骨骼网格体 :type Skeletal%20Mesh%20Object%20Reference) (新动画蓝图 :type Object%20Class%20Reference) (新材质 :type Array%20of%20Material%20Interface%20Object%20References))
  (for _array_element (Variables|状态|Get集中的角色数组)
    (Utilities|IsValid _array_element
      (:Is%20Valid
        (Default|F角色替换网格体及动画蓝图 _array_element 新骨骼网格体 新动画蓝图 新材质 (Variables|状态|Get角色等级)))))
  ;[0.04085 0.15 0.01362 0.5] 每次升级后都标记一下，方便后续新生成的角色比配角色模型
  (Variables|状态|Set角色等级 (Utilities|Enum|ByteToEnum角色等级 (+ (Variables|状态|Get角色等级) 1)))
  (return))

(fn F全体修改等级
  (for _array_element (Variables|状态|Get集中的角色数组)
    (Utilities|IsValid _array_element
      (:Is%20Valid
        (Default|F修改角色等级 _array_element))))
  ;[0.04085 0.15 0.01362 0.5] 每次升级后都标记一下，方便后续新生成的角色比配角色模型
  (Variables|状态|Set角色等级 (Utilities|Enum|ByteToEnum角色等级 (+ (Variables|状态|Get角色等级) 1)))
  (return))