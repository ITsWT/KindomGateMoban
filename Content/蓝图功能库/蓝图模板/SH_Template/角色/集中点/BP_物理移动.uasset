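; BP_物理移动 is a physics-capsule proxy that moves an attached character, syncing its location every tick and destroying itself when that character dies.
; It sweeps toward a gathering point with distance-scaled pull and swirl, or feeds character input to a floating movement component without one.
; A spawn timeline grows the seeded-random capsule radius and scales the mesh.
; Extra downward impulse offsets linear damping, and a launch function sets physics velocity.
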(event Custom|CEED-角色死亡时
  (params (死亡的角色 :type BP%20SH角色%20Base%20Object%20Reference))
  ;[0.8516 0 1] BeginPlay
  ;;[0 1 0.3438] Bind角色
  (Actor|DestroyActor))

(event Custom|CE_播放胶囊体缩放
  ;[1 1 1] 缩放胶囊体
  (Variables|Default|SetRef附加者缩放 (Variables|/Script/Engine.SceneComponent|GetRelativeScale3D (Variables|/Script/Engine.Character|GetMesh (Variables|Default|GetRef附加者角色))))
  (Components|Timeline|SetPlayRate (Variables|Default|GetTL_出生缩放) (/ 1.0 (Variables|Default|Get胶囊体出生缩放耗时)))
  (bind (_direction _f _s) (Timeline|TL_出生缩放 PlayFromStart)
    (:Update
      (bind _output_get (Variables|状态|Set移动总控百分比 _f))
      (Components|Capsule|SetCapsuleRadius (Variables|Default|Get物理胶囊体) (Math|Float|Lerp 5.0 (Variables|Default|Get胶囊体_半径) _output_get) true)
      ;[0 0.15 0.002663 0.5] 缩放网格体
      (Transformation|SetRelativeScale3D (Variables|/Script/Engine.Character|GetMesh (Variables|Default|GetRef附加者角色)) (* (Variables|Default|GetRef附加者缩放) _s)))))

(event Custom|CEED-角色移速变化时
  (params (当前新移速 :type Float%20%28double-precision%29) (期望移速 :type Float%20%28double-precision%29))
  ;[0.8516 0 1] BeginPlay
  ;;[0 1 0.3438] Bind角色
  (Variables|/Script/Engine.FloatingPawnMovement|SetMaxSpeed (Variables|Default|Get浮动组件) 当前新移速))

(event EventTick
  (params (DeltaSeconds :type Float%20%28single-precision%29))
  (bind _ref附加者角色 (Variables|Default|GetRef附加者角色))
  (bind _物理胶囊体 (Variables|Default|Get物理胶囊体))
  ;[1 0.2344 0] Tick
  (Utilities|IsValid (Variables|Default|GetRef附加者角色)
    (:Is%20Valid
      ;;[1 0.2344 0] 将角色的位置同步过来
      (Variables|Default|Set角色移速_期望 (Variables|/Game/蓝图功能库/蓝图模板/SH_Template/角色/BP_SH角色_Base.BP_SH角色_Base_C|Get角色移速_期望 _ref附加者角色))
      (Transformation|SetActorLocation _ref附加者角色 (+ (Transformation|GetActorLocation) (Variables|Default|Get绑定位置偏移)) false false))
    (:Is%20Not%20Valid
      _))
  ;;[0.7812 0 1] 施加额外的重力以对抗线性阻尼
  (Utilities|IsValid _物理胶囊体
    (:Is%20Valid
      (Physics|AddImpulse _物理胶囊体 (Math|Vector|MakeVector 0.0 0.0 (* (Class|PrimitiveComponent|GetLinearDamping (Variables|Default|Get物理胶囊体)) -9.8e+02 (Variables|Default|Get额外重力缩放))) "None" false)
      ;;[1 0.8203 0] 向集中点进行聚拢行为
      (Utilities|IsValid (Variables|Default|GetRef集中点)
        (:Is%20Valid
          (CallFunction|F向集中点聚拢))
        (:Is%20Not%20Valid
          ;;[1 0.6328 0] 绑定到移动输入
          (bind _ref附加者角色_2 (Variables|Default|GetRef附加者角色)
            (:then
              (Class|PawnMovementComponent|AddInputVector (Variables|Default|Get浮动组件) (Pawn|Components|PawnMovement|GetLastInputVector (Variables|/Script/Engine.Character|GetCharacterMovement _ref附加者角色_2)) false))
            (:else)))))))

(event EventBeginPlay
  ;[0.8516 0 1] BeginPlay
  ;;[0.6875 1 0] 初始设置移动速度和约束
  (Variables|/Script/Engine.FloatingPawnMovement|SetMaxSpeed (Variables|Default|Get浮动组件) (Variables|Default|Get聚拢速度))
  (Class|PrimitiveComponent|SetConstraintMode (Variables|Default|Get物理胶囊体) (Variables|Default|Get约束模式))
  (Utilities|FlowControl|Sequence
    (:then_0
      ;;[0 1 0.3438] Bind角色
      (Utilities|IsValid (Variables|Default|GetRef附加者角色)
        (:Is%20Valid
          (EventDispatchers|BindEventtoED-角色死亡时 (Variables|Default|GetRef附加者角色) (delegate Custom|CEED-角色死亡时))
          (EventDispatchers|AssignED-移速变化时 (Variables|Default|GetRef附加者角色) (delegate Custom|CEED-角色移速变化时)))))
    (:then_1
      ;;[0 1 0.5313] 加入集中点管理
      (Utilities|IsValid (Variables|Default|GetRef集中点)
        (:Is%20Valid
          (Utilities|Array|Add (Variables|/Game/蓝图功能库/蓝图模板/SH_Template/角色/集中点/BP_集中点.BP_集中点_C|Get集中的Actor数组 (Variables|Default|GetRef集中点)) self))))
    (:then_2
      (CallFunction|CE播放胶囊体缩放))))

(fn ConstructionScript
  (bind _物理胶囊体 (Variables|Default|Get物理胶囊体))
  (bind _物理胶囊体_2 (Variables|Default|Get物理胶囊体))
  (CallFunction|F修改胶囊体半径 (Variables|Default|Get胶囊体_半径))
  ;[0.4766 1 0] 设置碰撞胶囊体的半径和半高
  (Components|Capsule|SetCapsuleRadius _物理胶囊体 1.0 true) ; 初始没有，等待出生缩放
  (Components|Capsule|SetCapsuleHalfHeight _物理胶囊体 (Variables|Default|Get胶囊体_半高) true)
  ;[0.6406 0 1] 设置碰撞胶囊体的阻尼
  (Class|PrimitiveComponent|SetLinearDamping _物理胶囊体_2 (Variables|Default|Get初始线性阻尼))
  (Class|PrimitiveComponent|SetAngularDamping _物理胶囊体_2 (Variables|Default|Get初始角阻尼))
  (Class|PrimitiveComponent|SetConstraintMode (Variables|Default|Get物理胶囊体) (Variables|Default|Get约束模式))
  (Development|SetHiddeninGame (Variables|Default|Get物理胶囊体) (Variables|Default|Get隐藏碰撞体) false))

(fn F向集中点聚拢
  (bind _returnvalue (Transformation|GetActorLocation))
  (bind _旋转衰减距离 (Variables|Default|Get旋转衰减距离))
  (bind _聚拢衰减距离 (Variables|Default|Get聚拢衰减距离))
  (bind _ref集中点 (Variables|Default|GetRef集中点))
  (bind _returnvalue_2 (Transformation|GetActorLocation _ref集中点))
  ;[0 0.5781 1] 移动的方向和距离
  (LocalVariables|Setlp_聚拢方向 (CallFunction|单元方向2D _returnvalue _returnvalue_2))
  (bind _output_get (LocalVariables|Setlp_距离中心点的距离 (Math|Vector|Distance2D(Vector) _returnvalue _returnvalue_2)))
  (if (> _output_get 5.0)
    ;[0 1 0.1797] 计算最终方向
    (Development|PrintString (Utilities|String|ToString(Float) (LocalVariables|Getlp_距离中心点的距离)) true true "(R=0.000000,G=0.660000,B=1.000000,A=1.000000)" 0.01)
    (bind _output_get_2 (LocalVariables|Setlp_最终方向 (+ (* (LocalVariables|Getlp_聚拢方向) (Math|Float|MapRangeClamped (LocalVariables|Getlp_距离中心点的距离) (.x _聚拢衰减距离) (.y _聚拢衰减距离) 0.1 1.0) (Variables|/Game/蓝图功能库/蓝图模板/SH_Template/角色/集中点/BP_集中点.BP_集中点_C|Get集中点聚拢强度缩放 (Variables|Default|GetRef集中点)) (Variables|Default|Get聚拢强度缩放)) (Math|Vector|RotateVector (* (LocalVariables|Getlp_聚拢方向) (Math|Float|MapRangeClamped (LocalVariables|Getlp_距离中心点的距离) (.x _聚拢衰减距离) (.y _聚拢衰减距离) 0.1 1.0) (Variables|/Game/蓝图功能库/蓝图模板/SH_Template/角色/集中点/BP_集中点.BP_集中点_C|Get集中点聚拢强度缩放 (Variables|Default|GetRef集中点)) (Variables|Default|Get聚拢强度缩放)) (Math|Rotator|MakeRotator 0.0 0.0 (* (Variables|默认|Get旋转强度缩放) (Variables|/Game/蓝图功能库/蓝图模板/SH_Template/角色/集中点/BP_集中点.BP_集中点_C|Get集中点旋转强度缩放 (Variables|Default|GetRef集中点)) (* (Math|Float|MapRangeClamped (LocalVariables|Getlp_距离中心点的距离) 0.0 (.x _旋转衰减距离) 0.5 1.0) (Math|Float|MapRangeClamped (LocalVariables|Getlp_距离中心点的距离) 0.0 (* (.y _旋转衰减距离) 2.0) 1.0 0.1) (Variables|Default|Get旋转速度))))))))
    (Transformation|AddWorldOffset (Variables|Default|Get物理胶囊体) (* _output_get_2 (Variables|Default|Get角色移速_期望) (Utilities|Time|GetWorldDeltaSeconds) (Variables|状态|Get移动总控百分比)) true true)
    ;[0 0.3203 1] 绘制期望的移动方向
    (if (Variables|Default|Get绘制移动线条)
      (CallFunction|F绘制预测速度 5 (Variables|Default|Get聚拢速度) (LocalVariables|Getlp_最终方向) (Variables|状态|Get上一帧移动方向) (- (Transformation|GetActorLocation) (Math|Vector|MakeVector 0.0 0.0 (+ (Variables|Default|Get胶囊体_半高) -1.0))) "(R=0.000000,G=1.000000,B=0.279250,A=1.000000)")
      (Variables|状态|Set上一帧移动方向 (LocalVariables|Getlp_最终方向)))))

(fn F弹射物理移动
  (params (Velocity :type Vector) (bAddToCurrent :type Boolean))
  (Physics|SetPhysicsLinearVelocity (Variables|Default|Get物理胶囊体) Velocity bAddToCurrent "None"))

(fn F修改胶囊体半径
  (params (新半径 :type Float%20%28double-precision%29))
  (Variables|Default|Set胶囊体_半径 (* 新半径 (+ (CallFunction|流送中绝对值范围内随机浮点 (Variables|Default|Get胶囊体_随机半径百分比) (Variables|Default|Get物理移动_Seed)) 1.0))))