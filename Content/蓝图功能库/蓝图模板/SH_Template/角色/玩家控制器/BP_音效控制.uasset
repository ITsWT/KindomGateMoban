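; BP_音效控制 is the game's audio manager, starting looping or one-off background music on BeginPlay and playing 2D sound effects.
; Custom events, called by other Blueprints such as the base character and bullets, cover death, projectile firing by weapon type and bullet hits by surface (door or rolling log).
; Each effect passes through a short cooldown (冷却) to limit overlapping playback.
; Alternative music tracks remain as unconnected nodes.
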(event Custom|CE_生成发射物
  (params (Selection :type Eunm_开枪音效选择%20Enum :default "NewEnumerator0"))
  ;[0.15 0.15 0.15 0.5] CE_生成发射物（在各自子弹里面调用）
  (switch Utilities|FlowControl|Switch|SwitchonEunm_开枪音效选择 Selection
    (:NewEnumerator0
      (Utilities|冷却 0.1
        (:Completed
          (Audio|PlaySound2D "/Game/DoormdayTrain/Audios/手枪.手枪" 0.2 1.0 0.0 0 0))))
    (:NewEnumerator1
      (Utilities|冷却 0.1
        (:Completed
          (Audio|PlaySound2D "/Game/DoormdayTrain/Audios/AK47__2_.AK47__2_" 0.15 1.0 0.0 0 0))))
    (:NewEnumerator2
      (Utilities|冷却 0.05
        (:Completed
          (Audio|PlaySound2D "/Game/DoormdayTrain/Audios/加特林.加特林" 0.4 1.0 0.0 0 0))))))

(event Custom|CE_播放死亡
  ;[0.15 0.15 0.15 0.5] CE_播放死亡（BP_SH角色_Base里面调用）
  (Utilities|冷却 0.2
    (:Completed
      (Audio|PlaySound2D "/Game/DoormdayTrain/Audios/男人死亡.男人死亡" 0.2 1.0 0.0 0 0))))

(event Custom|CE_子弹击中
  (params (Selection :type Eunm_子弹击中音效选择%20Enum :default "NewEnumerator0"))
  ;[0.15 0.15 0.15 0.5] CE_子弹击中
  (switch Utilities|FlowControl|Switch|SwitchonEunm_子弹击中音效选择 Selection
    (:NewEnumerator1
      (Utilities|冷却 0.1
        (:Completed
          (Audio|PlaySound2D "/Game/Suika/Audios/ber2.ber2" 0.2 1.0 0.0 0 0))))
    (:NewEnumerator3
      (Utilities|冷却 0.1
        (:Completed
          (Audio|PlaySound2D "/Game/Runnning/Audios/子弹击中木头.子弹击中木头" 0.1 1.0 0.0 0 0))))))

(event EventBeginPlay
  (bind _returnvalue (Audio|SpawnSound2D "/Game/Runnning/Audios/Immediate_Music_-_Rockin__The_Boat.Immediate_Music_-_Rockin__The_Boat" 0.4 1.0 0.0 0))
  (Variables|Default|SetBGM _returnvalue))

(fn ConstructionScript)