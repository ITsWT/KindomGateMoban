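; Player controller for the parkour (跑酷) character template that sets up input and handles global hotkeys.
; BeginPlay adds the IMC_MyCharacter Enhanced Input mapping context to the local player.
; Hard-bound key events toggle game pause through a FlipFlop on Pause, quit the game on Escape, and reload the KindomDoors_Total_MoBan level by name on R.
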(event EventBeginPlay
  (Input|AddMappingContext (PlayerController|LocalPlayerSubsystems|GetEnhancedInputLocalPlayerSubsystem self) "/Game/Projects/Input/IMC_MyCharacter.IMC_MyCharacter" 0 "(bIgnoreAllPressedKeysUntilRelease=True,bForceImmediately=False,bNotifyUserSettings=False)"))

(event Input|KeyboardEvents|Escape
  (params (Key :type Key%20Structure))
  (:Pressed
    (Game|QuitGame 0 "Quit" false)))

(event Input|KeyboardEvents|Pause
  (params (Key :type Key%20Structure))
  (:Pressed
    (Utilities|FlowControl|FlipFlop
      (:A
        (Game|SetGamePaused true))
      (:B
        (Game|SetGamePaused false)))))

(event Input|KeyboardEvents|R
  (params (Key :type Key%20Structure))
  (:Pressed
    (Game|OpenLevel(byName) "KindomDoors_Total_MoBan")))

(fn ConstructionScript)