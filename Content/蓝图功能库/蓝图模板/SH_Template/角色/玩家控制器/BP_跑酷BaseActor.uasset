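; Parkour (跑酷) base actor that handles the player's sideways movement.
; The IA_MoveRight Enhanced Input action offsets the actor along its right vector, scaled by input value and Speed, without sweep or delta-time scaling.
; Tick is empty.
; Unconnected leftover logic prints game time and sphere-traces nearby light-gate obstacles to randomize their health and refresh their material and number text.
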(event Input|EnhancedActionEvents|EnhancedInputActionIA_MoveRight
  (params (ActionValue :type Float%20%28double-precision%29) (ElapsedSeconds :type Float%20%28double-precision%29) (TriggeredSeconds :type Float%20%28double-precision%29) (InputAction :type Input%20Action%20Object%20Reference :default "/Game/Projects/Input/IA_MoveRight.IA_MoveRight"))
  (Transformation|AddActorWorldOffset (* (Transformation|GetActorRightVector) (* ActionValue (Variables|Default|GetSpeed)))))

(event EventTick
  (params (DeltaSeconds :type Float%20%28single-precision%29)))

(fn ConstructionScript)