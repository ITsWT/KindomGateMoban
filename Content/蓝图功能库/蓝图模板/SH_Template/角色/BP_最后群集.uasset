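; BP_最后群集 (final swarm) is an enemy particle-swarm Blueprint for the parkour template, with a visual matching the selected character.
; On BeginPlay it copies 角色选择 (character selection) from the BP_跑酷BaseActor found in the level.
; It uses that value as the DT_敌人角色资产 row name and assigns the row's 粒子群集 asset to Move农民, resetting override parameters.
; A missing row leaves the component unchanged.
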(event EventBeginPlay
  ;[0.03585 0.15 0.01971 0.5] 初始化时候拿取源“角色选择”并设置
  (bind _returnvalue (Actor|GetActorOfClass "/Game/蓝图功能库/蓝图模板/SH_Template/角色/玩家控制器/BP_跑酷BaseActor.BP_跑酷BaseActor_C"))
  (Variables|Default|Set角色选择 (Variables|/Game/蓝图功能库/蓝图模板/SH_Template/角色/玩家控制器/BP_跑酷BaseActor.BP_跑酷BaseActor_C|Get角色选择 _returnvalue))
  (CallFunction|F敌人通过表初始化资源))

(fn ConstructionScript)

(fn F敌人通过表初始化资源
  (bind _returnvalue (Utilities|GetDataTableRow "/Game/蓝图功能库/蓝图模板/SH_Template/角色/表资产/DT_敌人角色资产.DT_敌人角色资产" (Variables|Default|Get角色选择))
    (:then
      (Class|NiagaraComponent|SetAsset (Variables|Default|GetMove_农民) (.粒子群集 (Utilities|Struct|BreakST_敌人角色资产 _returnvalue)) true)
      (return))))