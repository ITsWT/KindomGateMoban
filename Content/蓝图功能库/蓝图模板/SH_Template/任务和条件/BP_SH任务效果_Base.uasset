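; Base actor for task effects in the SH template, meant to be subclassed to run a conditional, optionally delayed task for an executor.
; F执行任务, called manually or on BeginPlay, constructs and checks condition objects, then starts the task or broadcasts failure and expires.
; Completion or abort fires once, broadcasts the result, sets a destroy lifespan and spawns follow-up task actors with their own delays, regardless of success.
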(event Custom|CE_执行任务
  (bind _任务_延迟 (Variables|Default|Get任务_延迟))
  (Utilities|DelayNotZero _任务_延迟
    (:false
      (Default|CallED-任务开始时 (Variables|Default|Get任务_执行者) _任务_延迟))))

(event Custom|CE_中止任务
  (params (原因 :type String))
  (CallFunction|CE任务完成 false 原因))

(event Custom|CE_任务完成
  (params (成功 :type Boolean) (原因 :type String))
  (bind _任务_新任务 (Variables|Default|Get任务_新任务))
  (Utilities|FlowControl|DoOnce false
    (:Completed
      (Variables|调试状态|Set任务_已完成执行 true)
      (Utilities|FlowControl|Sequence
        (:then_0
          (if (Variables|调试状态|GetDebugMode)
            (Development|PrintString (Utilities|String|Append (.RightS (Utilities|String|Split (Utilities|GetDisplayName self) "BP_SH任务效果_")) "  执行" (select 成功 "成功     " "失败     ") 原因 "     by" (Utilities|GetDisplayName (Variables|Default|Get任务_执行者))) true true (select 成功 "(R=0.053568,G=0.796875,B=0.000000,A=1.000000)" "(R=1.000000,G=0.000000,B=0.000000,A=1.000000)"))))
        (:then_1
          (Default|CallED-任务完成时 (Variables|Default|Get任务_执行者) 成功 原因)
          (Actor|SetLifeSpan (Variables|Default|Get任务_销毁延迟))
          ;[1 0 0.4687] 执行后续任务
          (if (Utilities|Map|IsNotEmpty _任务_新任务)
            (bind _keys (Utilities|Map|Keys _任务_新任务))
            (for _array_element _keys
              (bind _returnvalue (Game|SpawnActorfromClass _array_element (Transformation|GetActorTransform) "AlwaysSpawn" "MultiplyWithRoot" (Components|GetOwner) (Variables|Default|Get任务_执行者) 0 0 0 (.Value (Utilities|Map|Find _任务_新任务 _array_element)) 0.5 false (Variables|Actor|GetInstigator)))
              (CallFunction|F执行任务 _returnvalue))))))))

(event EventBeginPlay
  (if (Variables|Default|Get任务_自动执行)
    (CallFunction|F执行任务)))

(fn ConstructionScript)

(fn F是否满足条件
  (bind _任务_条件 (Variables|Default|Get任务_条件))
  (if (Utilities|Array|IsEmpty _任务_条件)
    (return true "无条件")
    (else
      (bind _array_element (Utilities|Array|ForEachLoopwithBreak _任务_条件 :!label _label)
        (:LoopBody
          (bind _returnvalue (Game|ConstructObjectfromClass (Components|GetOwner) _array_element (Variables|Default|Get任务_执行者)))
          (bind (_满足 _原因) (Default|F判断任务条件是否满足 _returnvalue))
          (if (not _满足)
            (goto _label Break)))
        (:Completed
          (return _满足 _原因))))))

(fn F执行任务
  ;[1 0.1875 0] 用于覆写
  (bind (_全部满足 _不满足的原因) (CallFunction|F是否满足条件))
  (if _全部满足
    (CallFunction|CE执行任务)
    (else
      (Default|CallED-任务完成时 (Variables|Default|Get任务_执行者) false _不满足的原因)
      (Actor|SetLifeSpan 1.0))))