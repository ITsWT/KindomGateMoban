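; Actor component that gives a BP_SH武器_Base weapon a pool of reusable projectiles.
; On BeginPlay it copies the owning weapon's projectile settings once, then pre-spawns projectiles of that type with those values and attaches them to the owner.
; SpawnFromPool moves the first idle projectile to the requested transform and activates it, printing a warning rather than growing when none is free.
; F清除所有 destroys and empties the pool.
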(event Custom|InitializePool
  (params (LastIndex :type Integer))
  (for _index (range (Utilities|Array|Length (Variables|缓存池|GetObjectPool)) LastIndex)
    (bind _returnvalue (Game|SpawnActorfromClass (Variables|发射物|Get发射物类型) (Math|Transform|MakeTransform (Transformation|GetActorLocation (Components|GetOwner)) "0, 0, 0" "1.000000,1.000000,1.000000") "AdjustIfPossibleButAlwaysSpawn" "MultiplyWithRoot" (Variables|发射物|GetBP_SH武器_Base) (Variables|发射物|Get武器所属阵营) (Variables|发射物|Get武器seed) (Variables|发射物|Get覆盖发射物速度) (Variables|发射物|Get发射物_速度倍率) (Variables|发射物|Get发射物_伤害值_Overload) (Variables|发射物|Get发射物_生命周期%20Override) (Variables|发射物|Get射击期望位置) (Variables|发射物|Get发射物_溅射范围%20Override) (Variables|发射物|GetInstigator)))
    (Utilities|Array|AddUnique (Variables|缓存池|GetObjectPool) _returnvalue)
    (Transformation|AttachActorToActor _returnvalue (Components|GetOwner) "None" "KeepWorld" "KeepWorld" "KeepRelative" true)))

(event EventBeginPlay
  (CallFunction|F获取基本属性)
  (CallFunction|InitializePool (Variables|缓存池|GetPoolSize)))

(fn FindFirstAvailableActor
  (for _array_element (Variables|缓存池|GetObjectPool)
    (Utilities|IsValid _array_element
      (:Is%20Valid
        (if (not (Variables|/Game/蓝图功能库/蓝图模板/SH_Template/子弹/BP_SH发射物_Base.BP_SH发射物_Base_C|Get是否正在使用 _array_element))
          (return _array_element))))))

(fn SpawnfromPool
  (params (Spawn%20Transform :type Transform))
  (bind _pooledactor (CallFunction|FindFirstAvailableActor))
  (Utilities|IsValid _pooledactor
    (:Is%20Valid
      (Transformation|SetActorTransform _pooledactor Spawn%20Transform)
      (Default|F设置状态 _pooledactor true)
      (return _pooledactor))
    (:Is%20Not%20Valid
      (Development|PrintString "不够用啦~" true true "(R=1.000000,G=0.000000,B=0.051567,A=1.000000)"))))

(fn F获取基本属性
  (bind _asbp_sh武器_base (Utilities|Casting|CastToBP_SH武器_Base (Components|GetOwner))
    (:then
      (Variables|发射物|Set发射物类型 (Variables|/Game/蓝图功能库/蓝图模板/SH_Template/武器/BP_SH武器_Base.BP_SH武器_Base_C|Get发射物类型 _asbp_sh武器_base))
      (Variables|发射物|SetBP_SH武器_Base _asbp_sh武器_base)
      (Variables|发射物|Set武器所属阵营 (Variables|/Game/蓝图功能库/蓝图模板/SH_Template/武器/BP_SH武器_Base.BP_SH武器_Base_C|Get武器所属阵营 _asbp_sh武器_base))
      (Variables|发射物|Set武器seed (Variables|/Game/蓝图功能库/蓝图模板/SH_Template/武器/BP_SH武器_Base.BP_SH武器_Base_C|Get武器seed _asbp_sh武器_base))
      (Variables|发射物|Set覆盖发射物速度 (Variables|/Game/蓝图功能库/蓝图模板/SH_Template/武器/BP_SH武器_Base.BP_SH武器_Base_C|Get覆盖发射物速度 _asbp_sh武器_base))
      (Variables|发射物|Set发射物_速度倍率 (Variables|/Game/蓝图功能库/蓝图模板/SH_Template/武器/BP_SH武器_Base.BP_SH武器_Base_C|Get发射物_速度倍率 _asbp_sh武器_base))
      (Variables|发射物|Set发射物_伤害值_Overload (Variables|/Game/蓝图功能库/蓝图模板/SH_Template/武器/BP_SH武器_Base.BP_SH武器_Base_C|Get发射物_伤害值_Overload _asbp_sh武器_base))
      (Variables|发射物|Set发射物_生命周期%20Override (Variables|/Game/蓝图功能库/蓝图模板/SH_Template/武器/BP_SH武器_Base.BP_SH武器_Base_C|Get发射物_生命周期%20Override _asbp_sh武器_base))
      (Variables|发射物|Set射击期望位置 (Variables|/Game/蓝图功能库/蓝图模板/SH_Template/武器/BP_SH武器_Base.BP_SH武器_Base_C|Get射击期望位置 _asbp_sh武器_base))
      (Variables|发射物|Set发射物_溅射范围%20Override (Variables|/Game/蓝图功能库/蓝图模板/SH_Template/武器/BP_SH武器_Base.BP_SH武器_Base_C|Get发射物_溅射范围%20Override _asbp_sh武器_base))
      (return))
    (:CastFailed
      (Development|PrintString "获取失败"))))

(fn F清除所有
  (for _array_element (Variables|缓存池|GetObjectPool)
    (Actor|DestroyActor _array_element))
  (Utilities|Array|Clear (Variables|缓存池|GetObjectPool))
  (Development|PrintString "Hello"))