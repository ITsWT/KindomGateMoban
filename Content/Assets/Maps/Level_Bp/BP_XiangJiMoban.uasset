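; BP_XiangJiMoban (camera template) is an actor that shifts sideways against its own world Y offset from a fixed reference, within a clamped range.
; Each tick records that inverted offset in a 15-slot ring buffer.
; While 停下否 is true, it sets relative Y to the offset, barely interpolated toward slot 0, and saves its transform; otherwise it reapplies the saved transform.
; The view-target switch is unconnected.
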(event EventBeginPlay)

(event EventTick
  (params (DeltaSeconds :type Float%20%28single-precision%29))
  (bind _returnvalue (Transformation|GetActorLocation))
  (bind _returnvalue_2 (- (.y _returnvalue) -1312.0))
  (bind _returnvalue_3 (Math|Float|Clamp(Float) _returnvalue_2 -1.5e+02 1.5e+02))
  (bind _returnvalue_4 (* _returnvalue_3 -1.0))
  (bind _result (Math|Integer|IncrementInt (Variables|Default|Get帧下标))
    (:%20%20
      (Utilities|Array|SetArrayElem (Variables|Default|Get帧对应偏移) (Math|Integer|%(Integer) _result 15) _returnvalue_4)
      (if (Variables|Default|Get停下否？)
        (Transformation|SetActorRelativeLocation (Math|Vector|MakeVector -1104.0 (Math|Interpolation|FInterptoConstant _returnvalue_4 (Utilities|Array|Get(acopy) (Variables|Default|Get帧对应偏移)) DeltaSeconds 0.01) 928.0))
        (Variables|Default|SetNewVar (Transformation|GetActorTransform))
        (else
          (Transformation|SetActorTransform (Variables|Default|GetNewVar)))))))

(fn ConstructionScript)